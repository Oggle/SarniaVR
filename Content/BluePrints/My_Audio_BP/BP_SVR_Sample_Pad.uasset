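; Sample pad Blueprint, apparently a drum pad, that plays a chosen sound when its trigger is hit or overlapped.
; Hits pass a GateMin check comparing frame delta seconds, rather than elapsed time, with the stored value.
; Accepted hits can briefly swap the trigger to an emissive material.
; The construction script applies scale, volume, sample selection, custom-primitive-data colour, optional material overrides and an optional text title.
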(event `self.myTrigger.OnComponentHit`
  (params (HitComponent :type "PrimitiveComponent Object Reference") (OtherActor :type "Actor Object Reference") (OtherComp :type "PrimitiveComponent Object Reference") (NormalImpulse :type "Vector Structure") (Hit :type "HitResult Structure (by ref)"))
  (`|ExecutionSequence` :!label _label
    (:`then_0`
      ;[1 0 0.01909] Open close gate variable
      (if (>= (- (`GameplayStatics.GetWorldDeltaSeconds`) (`self.oldGate`)) (/ (`self.gateMin`) 1000.0))
        (set `self.gateOpen` true)
        (set `self.goodHit` true)
        ;[1 0.03818 0] Play Sample On Trigger Hit
        (set `self.oldGate` (`GameplayStatics.GetWorldDeltaSeconds`))
        (`AudioComponent.Play` (`self.mySample`) 0.0)
        (set `self.gateOpen` false)
        (else
          (set `self.gateOpen` false))))
    (:`then_1`
      ;[1 0.1437 0.9059] Light Up material animation
      (if (`self.goodHit`)
        (set `self.goodHit` false)
        (`KismetSystemLibrary.PrintString` "Good Hit")
        (if (`self.lightUp`)
          (set `self.oldTriggerMatterial` (`|GetArrayItem` (`MeshComponent.GetMaterials` (`self.myTrigger`)) (`self.emissiveTriggerSlot`)))
          (`PrimitiveComponent.SetMaterial` (`self.myTrigger`) (`self.emissiveTriggerSlot`) (`self.emmisiveMaterial`))
          (`KismetSystemLibrary.Delay` (`self.animHitDelay`))
          (`PrimitiveComponent.SetMaterial` (`self.myTrigger`) (`self.emissiveTriggerSlot`) (`self.oldTriggerMatterial`)))))))

(event `self.myTrigger.OnComponentBeginOverlap`
  (params (OverlappedComponent :type "PrimitiveComponent Object Reference") (OtherActor :type "Actor Object Reference") (OtherComp :type "PrimitiveComponent Object Reference") (OtherBodyIndex :type Integer) (bFromSweep :type Boolean) (SweepResult :type "HitResult Structure (by ref)"))
  (goto _label))

(fn `UserConstructionScript`
  (locals (local_myTextRenderTitle :type "TextRenderComponent Object Reference"))
  (bind (_drumscale_location _drumscale_rotation _drumscale_scale) (`KismetMathLibrary.BreakTransform` (`self.drumScale`)))
  (bind _local_mytextrendertitle (`local.local_myTextRenderTitle`))
  (bind _mymesh (`self.myMesh`))
  (bind (_returnvalue_location _returnvalue_rotation _returnvalue_scale) (`KismetMathLibrary.BreakTransform` (`SceneComponent.GetRelativeTransform` (`self.myTrigger`))))
  (bind (_returnvalue_location_2 _returnvalue_rotation_2 _returnvalue_scale_2) (`KismetMathLibrary.BreakTransform` (`SceneComponent.GetRelativeTransform` (`self.myMesh`))))
  (bind (_r _g _b) (`KismetMathLibrary.BreakColor` (`self.primitiveColour`)))
  (bind _x (.x (+ _returnvalue_scale_2 _drumscale_scale)))
  (bind _x_2 (.x (+ _returnvalue_scale _drumscale_scale)))
  (`SceneComponent.K2_SetRelativeTransform` (`self.myMesh`) (`KismetMathLibrary.MakeTransform` _returnvalue_location_2 (struct) (`KismetMathLibrary.MakeVector` _x _x (.z (+ _returnvalue_scale_2 _drumscale_scale)))) false false)
  (`SceneComponent.K2_SetRelativeTransform` (`self.myTrigger`) (`KismetMathLibrary.MakeTransform` (0.0 0.0 0.0) (struct) (`KismetMathLibrary.MakeVector` _x_2 _x_2 (.z (+ _returnvalue_scale _drumscale_scale)))) false false)
  ;[0.04365 0.474 1] Set Pad Volume
  (`AudioComponent.SetVolumeMultiplier` (`self.mySample`) (`self.defVol`))
  ;[1 0.5344 0] Establish Primitive Colour  Connection
  (`PrimitiveComponent.SetCustomPrimitiveDataFloat` _mymesh 0 0.0)
  (`PrimitiveComponent.SetCustomPrimitiveDataVector3` _mymesh 0 (`KismetMathLibrary.MakeVector` _r _g _b))
  ;[0.1419 0 1] Load sound from table based on int
  (`AudioComponent.SetSound` (`self.mySample`) (`|GetArrayItem` (`self.padSoundSamples`) (`self.useSample`)))
  (set `self.triggerMeshTransform` (`SceneComponent.GetRelativeTransform` (`self.myTrigger`)))
  (`|ExecutionSequence`
    (:`then_0`
      ;[1 0 0.2223] Override Materials
      (if (`self.overrideMaterials`)
        (`|ExecutionSequence`
          (:`then_0`
            ;[1 0.1208 0.3216] Set mesh material
            (`PrimitiveComponent.SetMaterial` (`self.myMesh`) 0 (`|GetArrayItem` (`self.meshMaterial`) (`self.useMeshMaterial`))))
          (:`then_1`
            ;[1 0 0.4547] Visible Trigger if so use material
            (if (`self.triggerMeshVisible`)
              (`PrimitiveComponent.SetMaterial` (`self.myTrigger`) 0 (`|GetArrayItem` (`self.meshMaterial`) (`self.useTriggerMaterial`)))
              (else
                (`SceneComponent.SetVisibility` (`self.myTrigger`) false false)))))))
    (:`then_1`
      ;[0.4651 1 0.1096] Show Title Of Sample
      (if (`self.showTitle`)
        (bind _returnvalue (`AddComponent|NODE_AddTextRenderComponent-0`))
        (set `local.local_myTextRenderTitle` _returnvalue)
        (if (`KismetStringLibrary.NotEqual_StrStr` (`self.userDrumTitle`))
          (`TextRenderComponent.K2_SetText` _local_mytextrendertitle (`KismetTextLibrary.Conv_StringToText` (`self.userDrumTitle`)))
          (else
            (`TextRenderComponent.K2_SetText` _local_mytextrendertitle (`KismetTextLibrary.Conv_StringToText` (`KismetSystemLibrary.GetObjectName` (`|GetArrayItem` (`self.padSoundSamples`) (`self.useSample`)))))))
        (`SceneComponent.K2_SetRelativeTransform` (`local.local_myTextRenderTitle`) (`self.padTitleOffset`) false false)))))