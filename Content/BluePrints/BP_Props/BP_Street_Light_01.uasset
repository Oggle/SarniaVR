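; Configurable street light and power pole prop, set up entirely in the Construction Script.
; A transformer flag picks the pole mesh, and per-slot direction arrays choose which street lights, stop lights and walk lights appear, each type at an adjustable height.
; Unused street arms and spotlights are destroyed, while unused stop and walk lights are hidden.
; Spline-mesh wiring to the next pole is left disconnected, and DrawPowerLines is empty.
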(event `self.ReceiveBeginPlay`)

(fn `drawPowerLines`)

(fn `UserConstructionScript`
  (locals (local_splineMeshComponent :type "SplineMeshComponent Object Reference") (local_wire_connection :type "Vector Structure" :default (0.0 0.0 0.0)) (local_next_pole_wire_connect :type "Vector Structure" :default (0.0 0.0 0.0)))
  (bind _power_pole_type_1 (`self.Power_Pole_Type_1`))
  (bind _stoplightarray (`self.stopLightArray`))
  (bind _power_pole_type_2 (`self.Power_Pole_Type_2`))
  (bind _streetlightarray (`self.streetLightArray`))
  (bind _spotlightarray (`self.spotLightArray`))
  (bind _walklightarray (`self.walkLightArray`))
  (`KismetArrayLibrary.Array_Clear` (`self.streetLightArray`))
  (`KismetArrayLibrary.Array_Clear` (`self.walkLightArray`))
  (`KismetArrayLibrary.Array_Clear` (`self.stopLightArray`))
  (`KismetArrayLibrary.Array_Clear` (`self.spotLightArray`))
  ;[0.9533 0.1848 1] Setting Arrays
  ;;[0.6908 0.8319 1] Add Street Lights
  (`KismetArrayLibrary.Array_Add` _streetlightarray (`self.Street_Light_Arm_01`))
  (`KismetArrayLibrary.Array_Add` _streetlightarray (`self.Street_Light_Arm_02`))
  (`KismetArrayLibrary.Array_Add` _streetlightarray (`self.Street_Light_Arm_03`))
  (`KismetArrayLibrary.Array_Add` _streetlightarray (`self.Street_Light_Arm_04`))
  ;;[0.6908 0.8319 1] Add Stop Lights
  (`KismetArrayLibrary.Array_Add` _stoplightarray (`self.StLight_Tlight_Mount_01`))
  (`KismetArrayLibrary.Array_Add` _stoplightarray (`self.StLight_Tlight_Mount_02`))
  (`KismetArrayLibrary.Array_Add` _stoplightarray (`self.StLight_Tlight_Mount_03`))
  (`KismetArrayLibrary.Array_Add` _stoplightarray (`self.StLight_Tlight_Mount_04`))
  ;;[0.6908 0.8319 1] Add Spotlights
  (`KismetArrayLibrary.Array_Add` _spotlightarray (`self.sl_spotlight_01`))
  (`KismetArrayLibrary.Array_Add` _spotlightarray (`self.sl_spotlight_02`))
  (`KismetArrayLibrary.Array_Add` _spotlightarray (`self.sl_spotlight_03`))
  (`KismetArrayLibrary.Array_Add` _spotlightarray (`self.sl_spotlight_04`))
  ;;[0.6908 0.8319 1] Add Walklights
  (`KismetArrayLibrary.Array_Add` _walklightarray (`self.StLight_WalkLight_01`))
  (`KismetArrayLibrary.Array_Add` _walklightarray (`self.StLight_WalkLight_02`))
  ;[0.3395 0.5822 1] Power Pole Type
  (if (`self.hasTransformer`)
    (`SceneComponent.SetVisibility` _power_pole_type_2 false true)
    (`SceneComponent.SetVisibility` _power_pole_type_1 true true)
    (else
      (`SceneComponent.SetVisibility` _power_pole_type_1 false true)
      (`SceneComponent.SetVisibility` _power_pole_type_2 true true)))
  ;[1 0.8688 0] Street Light
  (for (_array_element _array_index) (`self.lightDir`)
    (if _array_element
      (bind _output (`|GetArrayItem` (`self.streetLightArray`) _array_index))
      (`SceneComponent.SetVisibility` _output true true)
      (bind _output_2 (`|GetArrayItem` (`self.spotLightArray`) _array_index))
      ;;[0.2611 1 0.7352] HandleSpot Light
      (`SceneComponent.SetHiddenInGame` _output_2 false false)
      (`SceneComponent.SetVisibility` _output_2 true true)
      (else
        ;;[1 0.3596 0.2397] Destroy Components
        (`ActorComponent.K2_DestroyComponent` _output)
        (`ActorComponent.K2_DestroyComponent` (`|GetArrayItem` (`self.spotLightArray`) _array_index))))
    (`SceneComponent.K2_SetRelativeLocation` _output (`KismetMathLibrary.MakeVector` 0.0 0.0 (`self.lightHeight`)) false false))
  ;[1 0.2911 0.0904] Stop Lights
  (for (_array_element_2 _array_index_2) (`self.stopLightDir`)
    (if _array_element_2
      (bind _output_3 (`|GetArrayItem` (`self.stopLightArray`) _array_index_2))
      (`SceneComponent.SetVisibility` _output_3 true true)
      (else
        (`SceneComponent.SetVisibility` _output_3 false true)))
    (`SceneComponent.K2_SetRelativeLocation` _output_3 (`KismetMathLibrary.MakeVector` 0.0 0.0 (`self.stopLightHeight`)) false false))
  ;[1 0 0.5541] Walk Lights
  (for (_array_element_3 _array_index_3) (`self.walkLightDir`)
    (if _array_element_3
      (bind _output_4 (`|GetArrayItem` (`self.walkLightArray`) _array_index_3))
      (`SceneComponent.SetVisibility` _output_4 true true)
      (else
        (`SceneComponent.SetVisibility` _output_4 false true)))
    (`SceneComponent.K2_SetRelativeLocation` _output_4 (`KismetMathLibrary.MakeVector` 0.0 0.0 (`self.walkLightHeight`)) false false)))