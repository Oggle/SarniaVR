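; Multitrack player actor that builds a row of push buttons, acting as either a step sequencer or a linked-track panel.
; Construction script gathers sample pads by kit ID or resolves master/slave tracks by GroupID, then spawns spaced, labelled child-actor buttons.
; At BeginPlay, a three-second delay loop toggles step buttons while PlaySeq is set.
; Unfinished: LinkedTrackBP is cleared before its length check, and the button array is cleared on every spawn.
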(event `self.ReceiveBeginPlay`
  (if (`self.playSeq`) :!label _label
    (`/Game/BluePrints/BP_Buttons_Switches/BP_Push_Button.toggleButton` (`|GetArrayItem` (`self.stepSeqButtonArray`) (`self.atStep`)))
    (bind _result (`/Engine/EditorBlueprintResources/StandardMacros.IncrementInt` (`self.atStep`))
      (:`  `
        (if (< _result (`self.stepSize`))
          (set `self.atStep` 0))
        (`KismetSystemLibrary.Delay` 3.0)
        (goto _label)))))

(fn `UserConstructionScript`
  (locals (local_buttonIndex :type Integer) (local_CreatedPushButton :type "/Game/BluePrints/BP_Buttons_Switches/BP_Push_Button Object Reference") (local_pushButtonClassIndex :type Integer) (loca_GroupID :type Integer :default 0) (local_bpOfClassElement :type "/Game/BluePrints/BP_Buttons_Switches/BP_Push_Button Object Reference"))
  (bind (_quickoffset_x _quickoffset_y _quickoffset_z) (`KismetMathLibrary.BreakVector` (`self.quickOffset`)))
  (bind _local_createdpushbutton (`local.local_CreatedPushButton`))
  (bind _local_bpofclasselement (`local.local_bpOfClassElement`))
  (bind (_quickspacer_x _quickspacer_y) (`KismetMathLibrary.BreakVector` (`self.quickSpacer`)))
  (bind _local_buttonindex (`local.local_buttonIndex`))
  (bind _returnvalue (`KismetArrayLibrary.Array_Length` (`self.linkedTrackBP`)))
  (bind _output (`|GetArrayItem` (`self.buttonLabelTextArray`) (`local.local_buttonIndex`)))
  (bind _output_2 (`|GetArrayItem` (`self.linkedTrackBP`)))
  ;[1 0 0] Reset Arrays
  (`KismetArrayLibrary.Array_Clear` (`self.BP Push Button`))
  (`KismetArrayLibrary.Array_Clear` (`self.linkedDrumKit`))
  (`KismetArrayLibrary.Array_Clear` (`self.linkedTrackBP`))
  (`|ExecutionSequence`
    (:`then_0`
      ;[0.5172 0.1539 1] Crude Base Modifier
      (`SceneComponent.K2_SetRelativeTransform` (`self.mt_Base`) (`self.baseMeshTransform`) false false))
    (:`then_1`
      ;[1 0 0] STEPSEQUENCER DRUMPAD SETUP
      (if (`self.modeSeq`)
        (bind _outactors (`GameplayStatics.GetAllActorsOfClass` "/Game/BluePrints/My_Audio_BP/DrumPad/BP_SVR_Sample_Pad_V2.BP_SVR_Sample_Pad_V2_C"))
        (for _array_element _outactors
          (if (== (`self.stepSeqKitID`) (`/Game/BluePrints/My_Audio_BP/DrumPad/BP_SVR_Sample_Pad_V2.myKit` _array_element))
            (`KismetArrayLibrary.Array_Add` (`self.linkedDrumKit`) _array_element)))
        ;;[0.5473 1 0.1145] UpdateButton Count
        (set `self.buttonCount` (`self.stepSize`))
        (else
          ;[0.02728 0.2423 1] Check for linked Master track and get
          (if (> _returnvalue 0)
            (set `self.buttonCount` _returnvalue)
            ;[1 0 0.02628] If the first selected is a salve then get it's master, maybe issue ID
            (if (`/Game/BluePrints/BP_Buttons_Switches/BP_Push_Button.linkSlave` _output_2)
              ;;[1 0 0.2691] Use what this is linked to
              (set `self.linkedMasterLooper` (`/Game/BluePrints/BP_Buttons_Switches/BP_Push_Button.linked_tmpAudio` _output_2))
              (else
                ;;[1 0.7339 0.02011] Not a Slave Use Index 0 as Parent
                (set `self.linkedMasterLooper` (`/Game/BluePrints/BP_Buttons_Switches/BP_Push_Button.tmpAudio` _output_2))
                ;;[1 0.02329 0] Capture Master BP_PushButton Component
                (set `self.linkedMasterPushButtonComponent` _output_2)
                ;[0.4238 1 0.006914] Get all actors for group track
                (bind _outactors_2 (`GameplayStatics.GetAllActorsOfClass` "/Game/BluePrints/BP_Buttons_Switches/BP_Push_Button.BP_Push_Button_C"))
                (for (_array_element_2 _array_index) _outactors_2
                  (set `local.local_bpOfClassElement` _array_element_2)
                  (set `local.local_pushButtonClassIndex` _array_index)
                  (bind _output_get (set `local.loca_GroupID` (`/Game/BluePrints/BP_Buttons_Switches/BP_Push_Button.groupID` (`local.local_bpOfClassElement`))))
                  ;;[1 0 0.4244 1 14] Filter for PushButton with group ID
                  (if (== _output_get (`/Game/BluePrints/BP_Buttons_Switches/BP_Push_Button.groupID` (`self.linkedMasterPushButtonComponent`)))
                    ;;[1 0.4488 0 1 14] Check for slave boolean
                    (if (`/Game/BluePrints/BP_Buttons_Switches/BP_Push_Button.linkSlave` (`self.linkedMasterPushButtonComponent`))
                      ;;[0.4167 0 0] Add slaves past 1 and add master to slot 0
                      (`KismetArrayLibrary.Array_Set` (`self.linkedTrackBP`) (+ (`KismetArrayLibrary.Array_Length` (`self.linkedTrackBP`)) 1) _local_bpofclasselement true)
                      (else
                        (`KismetArrayLibrary.Array_Set` (`self.linkedTrackBP`) 0 _local_bpofclasselement true)))))))))))
    (:`then_2`
      ;[0.1936 0.9203 1] Loop through neede button int
      (for _index (range (`self.buttonCount`))
        (set `local.local_buttonIndex` _index)
        ;[1 0.04724 0] Brute Spacer, not dynamic
        (`KismetArrayLibrary.Array_Clear` (`self.stepSeqButtonArray`))
        (bind _returnvalue_2 (`AddComponent|NODE_AddChildActorComponent-0` :`RelativeTransform` (`KismetMathLibrary.MakeTransform` (`KismetMathLibrary.MakeVector` (+ _quickoffset_x (* _local_buttonindex _quickspacer_x)) (+ (* _local_buttonindex _quickspacer_y) _quickoffset_y) _quickoffset_z))))
        (bind _childactor (`ChildActorComponent.ChildActor` _returnvalue_2))
        ;;[0.4554 1 0] Just Making Sure Lol
        (if (== (`GameplayStatics.GetObjectClass` _childactor) "/Game/BluePrints/BP_Buttons_Switches/BP_Push_Button.BP_Push_Button_C")
          (bind _asbp_push_button (cast `/Game/BluePrints/BP_Buttons_Switches/BP_Push_Button` _childactor))
          ;;[0 0.2162 1] Create a local instance
          (bind _output_get_2 (set `local.local_CreatedPushButton` _asbp_push_button))
          (`KismetArrayLibrary.Array_Add` (`self.stepSeqButtonArray`) _output_get_2)
          (`StaticMeshComponent.SetStaticMesh` (`/Game/BluePrints/BP_Buttons_Switches/BP_Push_Button.Button` _output_get_2) (`self.stepSeqButtonMesh`))
          ;;[1 0 0.09783] Show Player Button Labels
          (set `/Game/BluePrints/BP_Buttons_Switches/BP_Push_Button.showLabel` (`self.showButtonLabels`) (`local.local_CreatedPushButton`))
          ;;[1 0.2453 0.575] If So then set those from the Player Label Array
          (set `/Game/BluePrints/BP_Buttons_Switches/BP_Push_Button.labelOff` _output _local_createdpushbutton)
          (set `/Game/BluePrints/BP_Buttons_Switches/BP_Push_Button.labelOn` _output _local_createdpushbutton))))))