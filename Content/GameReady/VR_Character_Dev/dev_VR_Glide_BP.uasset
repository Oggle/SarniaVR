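; Development VR glide locomotion Blueprint that moves the player pawn along the camera's forward direction.
; The MoveForward axis event, without reading the axis value, stores camera location and a trace end GlideSpped units ahead.
; It plays a timeline at RateOfPlay, lerping between those points by curve and feeding only X and Y into SetActorLocation.
; The line trace's hit result is never checked, so it only supplies the endpoint.
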(event `InputAxis|MoveForward`
  (params (AxisValue :type "Float (single-precision)"))
  (bind _returnvalue (`GameplayStatics.GetPlayerCameraManager` 0))
  (bind _returnvalue_2 (`self.K2_GetActorLocation` _returnvalue))
  (bind _outhit (`KismetSystemLibrary.LineTraceSingle` _returnvalue_2 (+ _returnvalue_2 (* (`self.GetActorForwardVector` _returnvalue) (`self.glideSpped`))) "TraceTypeQuery1"))
  (set `self.endTrace` (`.TraceEnd` (`GameplayStatics.BreakHitResult` _outhit)))
  (set `self.startTrace` (`self.K2_GetActorLocation` (`GameplayStatics.GetPlayerCameraManager` 0)))
  ;[1 0.02357 0] Animation Curve
  (`TimelineComponent.SetPlayRate` (`self.glideTimeline`) (/ (`self.rateOfPlay`) 1.0))
  (bind (_direction _glidetrack) (`Timeline|glideTimeline`)
    (:`Update`
      (`self.K2_SetActorLocation` (`GameplayStatics.GetPlayerPawn` 0) (`KismetMathLibrary.MakeVector` (.x (`KismetMathLibrary.VLerp` (`self.startTrace`) (`self.endTrace`) _glidetrack)) (.y (`KismetMathLibrary.VLerp` (`self.startTrace`) (`self.endTrace`) _glidetrack))) false false))))

(fn `UserConstructionScript`)