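; VR bow actor that nocks a BP_Arrow touching its string and lets the player draw and release it.
; The string is spline meshes along a spline; while nocked, Tick pulls the middle point to the arrow and aims it at the handle.
; Distance from handle to arrow feeds the arrow's BowCharge.
; The arrow's release event switches bow state, snapping the string to its stored default and playing handling audio.
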(event `self.ReceiveBeginPlay`
  ;[1 0 0.1519] Start Loaded
)

(event `self.ReceiveTick`
  (params (DeltaSeconds :type "Float (single-precision)"))
  (bind _returnvalue (`SceneComponent.K2_GetComponentLocation` (`self.Bow_Handle`)))
  (bind _returnvalue_2 (`self.K2_GetActorLocation` (`self.asMyBPArrowUser`)))
  (bind _returnvalue_3 (`self.K2_GetActorLocation` (`self.asMyBPArrowUser`)))
  ;[1 0 0.3023] Animate and redraw bow string
  (if (`self.bowReady`)
    (set `self.Delta Seconds` DeltaSeconds)
    ;;[1 0.7915 0] Do We Have An Arrow
    (if (`self.arrow_onString`)
      (bind _asmybparrowuser (`self.asMyBPArrowUser`)
        (:`then`
          (if (`|EnumEquality` (`/Game/BluePrints/BP_Weapons/Bow_Arrow/BP_Arrow.arrowState` _asmybparrowuser) "NewEnumerator2")
            (`SplineComponent.SetLocationAtSplinePoint` (`self.stringSpline`) 1 _returnvalue_2 "World" true)
            (`self.K2_SetActorRotation` (`self.asMyBPArrowUser`) (`KismetMathLibrary.FindLookAtRotation` _returnvalue_3 _returnvalue) false)
            ;;[1 0 0.1271] Feed Bow charge to arrow
            (set `/Game/BluePrints/BP_Weapons/Bow_Arrow/BP_Arrow.bowCharge` (* (`KismetMathLibrary.Vector_Distance` _returnvalue_3 _returnvalue) (`self.bowChargeMulti`)) (`self.asMyBPArrowUser`))
            (`KismetSystemLibrary.PrintString` (`KismetStringLibrary.Conv_VectorToString` _returnvalue_2) false)
            (`self.drawBowStringLive` 2)))
        (:`else`
          (`KismetSystemLibrary.PrintString` "Invalid Arrow" false)
          (set `self.arrow_onString` false))))))

(event `getShootHand`
  ;[1 0 0.1322] From Tutorial
  (add `/Game/VRTemplate/Blueprints/GrabComponent.OnGrabbed` (`self.GrabComponent`) (delegate `getShootHand`)))

(event `beginCharge`
  ;[1 0 0.1322] From Tutorial
  (`self.myArrow`
    (:`then`
      (`Timeline|chargeTimeLine` :!label _label))
    (:`else`)))

(event `endCharge`
  ;[1 0 0.1322] From Tutorial
  (`self.myArrow`
    (:`then`
      (goto _label :!via `Reverse`))
    (:`else`)))

(event `stopCharge`
  ;[1 0 0.1322] From Tutorial
  (`|ExecutionSequence`
    (:`then_0`
      (goto _label :!via `Stop`))
    (:`then_1`
      (goto _label :!via `SetNewTime`))))

(event `self.stringSplineMeshComp.OnComponentBeginOverlap`
  (params (OverlappedComponent :type "PrimitiveComponent Object Reference") (OtherActor :type "Actor Object Reference") (OtherComp :type "PrimitiveComponent Object Reference") (OtherBodyIndex :type Integer) (bFromSweep :type Boolean) (SweepResult :type "HitResult Structure (by ref)"))
  ;[0.699 0.2785 1] Arrow On String Overlap
  (if (`self.bowReady`)
    ;;[1 0.1242 0.5164] Is It an Arrow
    (if (== (`GameplayStatics.GetObjectClass` OtherActor) "/Game/BluePrints/BP_Weapons/Bow_Arrow/BP_Arrow.BP_Arrow_C")
      (bind _asbp_arrow (cast `/Game/BluePrints/BP_Weapons/Bow_Arrow/BP_Arrow` OtherActor))
      (`/Game/VRTemplate/Blueprints/GrabComponent.HapticHit` (`self.GrabComponent`) "/Game/GameReady/Haptics/ArrowGrabHaptic.ArrowGrabHaptic")
      (if (`|EnumEquality` (`/Game/BluePrints/BP_Weapons/Bow_Arrow/BP_Arrow.arrowState` _asbp_arrow) "NewEnumerator1")
        (set `self.asMyBPArrowUser` _asbp_arrow)
        (set `self.arrow_onString` true)
        ;;[0.783 0.02122 1 1 14] Arrow Rec. It Is in a bow
        (`/Game/BluePrints/BP_Weapons/Bow_Arrow/BP_Arrow.setArrowState` (`self.asMyBPArrowUser`) "NewEnumerator2")
        (`self.setBowState` "NewEnumerator2")
        (add `/Game/BluePrints/BP_Weapons/Bow_Arrow/BP_Arrow.arrowReleasedDisp` (`self.asMyBPArrowUser`) (delegate `arrowDropped`))
        (`KismetSystemLibrary.PrintString` "Arrow In Bow")
        (else
          (`KismetSystemLibrary.PrintString` "Arrow is Busy"))))
    (else
      (`KismetSystemLibrary.PrintString` "Bow not ready") ; NOT READY
    )))

(event `reloadBow`
  ;[1 0 0.1322] From Tutorial
  (bind _returnvalue (`|SpawnActorFromClass` "/Game/BluePrints/BP_Weapons/Bow_Arrow/BP_Arrow.BP_Arrow_C" (`KismetMathLibrary.MakeTransform` (0.0 0.0 0.0)) "Undefined" "OverrideRootScale" null "NewEnumerator0" null))
  (set `self.myArrow` _returnvalue))

(event `arrowDropped`
  ;[0.699 0.2785 1] Arrow On String Overlap
  (`self.setBowState` "NewEnumerator3"))

(event `self.stringSpline.OnComponentEndOverlap`
  (params (OverlappedComponent :type "PrimitiveComponent Object Reference") (OtherActor :type "Actor Object Reference") (OtherComp :type "PrimitiveComponent Object Reference") (OtherBodyIndex :type Integer))
  ;[1 0.867 0.1864] End overlap string
)

(event `gateKeeper`
  ;[1 0.08141 0.05157] Simple Bow Ready Delay Gatekeeper
  (`KismetSystemLibrary.Delay` (`self.bowReadDelay`))
  (set `self.bowReady` true))

(fn `beginBowState`
  (params (newState :type "/Game/BluePrints/BP_Weapons/Bow_Arrow/EBowState Enum" :default "NewEnumerator0"))
  (bind _stringspline (`self.stringSpline`))
  (bind _sc_bowhandling (`self.SC_BowHandling`))
  (bind _bowstringcenterpointindex (`self.bowStringCenterPointIndex`))
  (bind (_output_location _output_rotation _output_scale) (`KismetMathLibrary.BreakTransform` (`|GetArrayItem` (`self.defPointPositions`) _bowstringcenterpointindex)))
  (switch `/Game/BluePrints/BP_Weapons/Bow_Arrow/EBowState` newState
    (:`NewEnumerator3`
      (`AudioComponent.SetIntParameter` _sc_bowhandling "bowActivity" 1)
      (`AudioComponent.Play` _sc_bowhandling 0.0)
      (`SplineComponent.SetLocationAtSplinePoint` _stringspline _bowstringcenterpointindex _output_location "Local" true)
      (`SplineComponent.SetTangentAtSplinePoint` _stringspline _bowstringcenterpointindex _output_scale "Local" true)
      (`self.drawBowStringLive` 0))))

(fn `drawBowString`
  (bind _stringspline (`self.stringSpline`))
  (for _index (range (+ (- (`SplineComponent.GetNumberOfSplinePoints` (`self.stringSpline`)) 2) 1))
    (bind _returnvalue (`AddComponent|NODE_AddSplineMeshComponent-2`))
    (`KismetArrayLibrary.Array_Add` (`self.stringSplineMeshCompArray`) _returnvalue)
    (bind _output_get (set `self.stringSplineMeshComp` _returnvalue))
    (bind (_location _tangent) (`SplineComponent.GetLocationAndTangentAtSplinePoint` _stringspline _index "Local"))
    (`KismetArrayLibrary.Array_Add` (`self.defPointPositions`) (`KismetMathLibrary.MakeTransform` _location (struct) _tangent))
    (bind (_location_2 _tangent_2) (`SplineComponent.GetLocationAndTangentAtSplinePoint` _stringspline (+ _index 1) "Local"))
    (`SplineMeshComponent.SetStartAndEnd` _output_get _location _tangent _location_2 _tangent_2 true)
    (`SceneComponent.K2_AttachToComponent` (`self.stringSplineMeshComp`) null "None" "KeepRelative" "KeepRelative" "KeepRelative" true)))

(fn `drawBowStringLive`
  (params (indexStartAdjust :type Integer))
  (bind _stringspline (`self.stringSpline`))
  (for _index (range (+ (- (`SplineComponent.GetNumberOfSplinePoints` (`self.stringSpline`)) (`local.indexStartAdjust`)) 1))
    (bind _output (`|GetArrayItem` (`self.stringSplineMeshCompArray`) _index))
    (`/Engine/EditorBlueprintResources/StandardMacros.IsValid` _output
      (:`Is Valid`
        (bind (_location _tangent) (`SplineComponent.GetLocationAndTangentAtSplinePoint` _stringspline _index "Local"))
        (bind (_location_2 _tangent_2) (`SplineComponent.GetLocationAndTangentAtSplinePoint` _stringspline (+ _index 1) "Local"))
        (`SplineMeshComponent.SetStartAndEnd` _output _location _tangent _location_2 _tangent_2 true))
      (:`Is Not Valid`
        (`KismetSystemLibrary.PrintString` "Invalid Spline Mesh")))))

(fn `endBowState`
  (params (oldState :type "/Game/BluePrints/BP_Weapons/Bow_Arrow/EBowState Enum" :default "NewEnumerator0")))

(fn `fireProjectile`
  (locals (projectile_BP_Arrow :type "/Game/BluePrints/BP_Weapons/Bow_Arrow/BP_Arrow Object Reference"))
  (bind _returnvalue (`|SpawnActorFromClass` "/Game/BluePrints/BP_Weapons/Bow_Arrow/BP_Arrow.BP_Arrow_C" (`SceneComponent.K2_GetComponentToWorld` (`/Game/BluePrints/BP_Weapons/Bow_Arrow/BP_Arrow.Arrow` (`self.asMyBPArrowUser`))) "AlwaysSpawn" "OverrideRootScale" null "NewEnumerator0" null))
  (bind _output_get (set `local.projectile_BP_Arrow` _returnvalue))
  (bind _returnvalue_2 (`AddComponent|NODE_AddProjectileMovementComponent-1` :`self` _output_get))
  (set `ProjectileMovementComponent.InitialSpeed` (`self.projectileSpeed`) _returnvalue_2)
  (`ActorComponent.SetActive` _returnvalue_2 true false)
  (`KismetSystemLibrary.PrintString` "arrowFired"))

(fn `reloadBowArrow`
  (bind _returnvalue (`|SpawnActorFromClass` "/Game/BluePrints/BP_Weapons/Bow_Arrow/BP_Arrow.BP_Arrow_C" (`KismetMathLibrary.MakeTransform` (0.0 0.0 0.0)) "AlwaysSpawn" "OverrideRootScale" null "NewEnumerator0" null))
  (bind _output_get (set `self.myArrow` _returnvalue))
  (`SceneComponent.K2_SetRelativeLocation` (`/Game/BluePrints/BP_Weapons/Bow_Arrow/BP_Arrow.Arrow` _output_get) (`SplineComponent.GetLocationAtSplinePoint` (`self.stringSpline`) 1 "World") false false)
  (`self.K2_AttachToComponent` (`self.myArrow`) (`self.Bow`) (`self.myArrowSocket`) "SnapToTarget" "SnapToTarget" "KeepWorld" false)
  (`KismetSystemLibrary.PrintString` "Reloaded Arrow Function"))

(fn `setBowState`
  (params (newState :type "/Game/BluePrints/BP_Weapons/Bow_Arrow/EBowState Enum" :default "NewEnumerator0"))
  (bind _bowstate (`self.bowState`))
  (bind _sc_bowhandling (`self.SC_BowHandling`))
  (bind _sc_bowhandling_2 (`self.SC_BowHandling`))
  (if (`|EnumInequality` newState _bowstate)
    (`self.endBowState` _bowstate)
    (bind _output_get (set `self.bowState` (`local.newState`)))
    (`self.beginBowState` _output_get)
    (`AudioComponent.SetIntParameter` _sc_bowhandling "bowActivity" 1)
    (`AudioComponent.Play` _sc_bowhandling 0.0)
    (else
      (`AudioComponent.SetIntParameter` _sc_bowhandling_2 "bowActivity" 0)
      (`AudioComponent.Play` _sc_bowhandling_2 0.0))))

(fn `UserConstructionScript`
  (`|ExecutionSequence`
    (:`then_0`
      ;[0.1338 1 0.9502] Set arrow to our pull spline point index
      (`SceneComponent.K2_SetRelativeLocation` (`self.arrowMock`) (`SplineComponent.GetLocationAtSplinePoint` (`self.stringSpline`) 1 "Local") false false))
    (:`then_1`
      ;[0.8651 1 0] Clear spline point default storage arrays
      (`KismetArrayLibrary.Array_Clear` (`self.stringSplineMeshCompArray`))
      (`KismetArrayLibrary.Array_Clear` (`self.defPointPositions`))
      ;[1 0 0.007892 1 14] Set Enum State and draw the bow string the first time.
      (set `self.bowState` "NewEnumerator1")
      (`self.drawBowString`))))