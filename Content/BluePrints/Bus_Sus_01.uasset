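; Bus actor that cycles through the locations of all BP_BusStop actors, with heavy debug printing.
; BeginPlay gathers the stops; overlapping any actor not yet in its history records it and advances the destination index, wrapping at the end.
; Tick spins four tire components by TopSpeed and delta time, computing a look-at rotation that never steers.
; A dot product of rotators built from location coordinates only prints a left/right guess.
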(event `self.ReceiveActorBeginOverlap`
  (params (OtherActor :type "Actor Object Reference"))
  (`KismetSystemLibrary.PrintString` "Hit Something")
  (if (not (`self.routeHistoryBeen` OtherActor))
    (`self.nextStop` OtherActor)))

(event `self.ReceiveBeginPlay`
  (`self.getStops`)
  (`self.nextStop` null)
  (set `self.canDrive` true))

(event `self.ReceiveTick`
  (params (DeltaSeconds :type "Float (single-precision)"))
  (bind _mydeltadrive (`self.myDeltaDrive`))
  (set `self.atLocation` (`self.K2_GetActorLocation`))
  (set `self.myDeltaSeconds` DeltaSeconds)
  (set `self.turnZ` (`KismetMathLibrary.FindLookAtRotation` (`self.atLocation`) (`self.destLocation`)))
  (if (`self.canDrive`)
    (set `self.myDeltaDrive` (* (`self.myDeltaSeconds`) (* (`self.topSpeed`) -1.0)))
    ;[0.3445 1 0.0904] 4 Wheel Drive Forward
    (bind _result (`/Engine/EditorBlueprintResources/StandardMacros.NegateFloat` _mydeltadrive)
      (:`  `
        (`SceneComponent.K2_AddWorldRotation` (`self.Sarnia_Bus_Tire_FL`) (`KismetMathLibrary.MakeRotator` 0.0 _mydeltadrive) false false)
        (`SceneComponent.K2_AddWorldRotation` (`self.Sarnia_Bus_Tire_FR`) (`KismetMathLibrary.MakeRotator` 0.0 _result) false false)
        (`SceneComponent.K2_AddWorldRotation` (`self.Sarnia_Bus_Tire_BL`) (`KismetMathLibrary.MakeRotator` 0.0 _mydeltadrive) false false)
        (`SceneComponent.K2_AddWorldRotation` (`self.Sarnia_Bus_Tire_BR`) (`KismetMathLibrary.MakeRotator` 0.0 _result) false false)))))

(fn `getLeftRightDegree`
  (params (vectorA :type "Vector Structure") (vectorB :type "Vector Structure"))
  (returns (myRadians :type "Float (double-precision)"))
  (return (`KismetMathLibrary.Dot_VectorVector` (`KismetMathLibrary.GetForwardVector` (`KismetMathLibrary.MakeRotator` (.x vectorA) (.y vectorA))) (`KismetMathLibrary.GetForwardVector` (`KismetMathLibrary.MakeRotator` (.x vectorB) (.y vectorB))))))

(fn `getStops`
  (bind _returnvalue (`KismetArrayLibrary.Array_Length` (`self.allBusStops`)))
  (bind _outactors (`GameplayStatics.GetAllActorsOfClass` "/Game/BluePrints/BP_BusStop.BP_BusStop_C"))
  (bind _output_get (set `self.allBusStops` _outactors))
  (if (> _returnvalue 0)
    (bind _output_get_2 (set `self.outDiagString` (`KismetStringLibrary.Concat_StrStr` (`KismetStringLibrary.Conv_IntToString` _returnvalue) " Stops Found")))
    (`KismetSystemLibrary.PrintString` _output_get_2)
    (for (_array_element _array_index) _output_get
      (`KismetArrayLibrary.Array_Insert` (`self.destArrays`) (`self.K2_GetActorLocation` _array_element) _array_index))
    (`KismetSystemLibrary.PrintString` "Bus Got Routes")
    (else
      (`KismetSystemLibrary.PrintString` "No Stops"))))

(fn `nextStop`
  (params (newStopActor :type "Actor Object Reference"))
  (bind _returnvalue (`KismetMathLibrary.Dot_VectorVector` (`KismetMathLibrary.GetForwardVector` (`KismetMathLibrary.MakeRotator` (.x (`self.atLocation`)) (.y (`self.atLocation`)))) (`KismetMathLibrary.GetForwardVector` (`KismetMathLibrary.MakeRotator` (.x (`self.destLocation`)) (.y (`self.destLocation`))))))
  (`self.routeHistoryAdd` newStopActor)
  (bind _result (`/Engine/EditorBlueprintResources/StandardMacros.IncrementInt` (`self.atLocArray`))
    (:`  `
      (set `self.atLocation` (`self.K2_GetActorLocation`))
      (if (>= _result (`KismetArrayLibrary.Array_Length` (`self.destArrays`)))
        (set `self.atLocArray` 0))
      (set `self.destLocation` (`|GetArrayItem` (`self.destArrays`) (`self.atLocArray`)))
      (`KismetSystemLibrary.PrintString` (`KismetStringLibrary.Concat_StrStr` "Goingt To Stop " (`KismetStringLibrary.Conv_IntToString` (`self.atLocArray`))) true true (struct :`G` 0.66 :`B` 1.0 :`A` 1.0) 5.0)
      (`KismetSystemLibrary.PrintString` (`KismetStringLibrary.Concat_StrStr` (`KismetStringLibrary.Conv_DoubleToString` _returnvalue) "Dot") true true (struct :`R` 1.0 :`G` 0.109751 :`B` 0.050025 :`A` 1.0) 15.0)
      (if (> _returnvalue 0.0)
        (`KismetSystemLibrary.PrintString` "Stop To Our Right")
        (else
          (`KismetSystemLibrary.PrintString` "Stop To Our Left")))
      (`KismetSystemLibrary.PrintString` (`KismetStringLibrary.Conv_DoubleToString` (`KismetMathLibrary.RadiansToDegrees` _returnvalue)) true true (struct :`R` 0.614583 :`B` 0.565375 :`A` 1.0) 15.0))))

(fn `routeHistoryAdd`
  (params (stopActor :type "Actor Object Reference"))
  (bind _returnvalue (`KismetArrayLibrary.Array_Add` (`self.stopAtors`) stopActor))
  (`KismetSystemLibrary.PrintString` (`KismetStringLibrary.Concat_StrStr` (`KismetStringLibrary.Concat_StrStr` "Added Stop" (`KismetStringLibrary.Conv_IntToString` _returnvalue)) (`KismetStringLibrary.Concat_StrStr` "History Length" (`KismetStringLibrary.Conv_IntToString` (`KismetArrayLibrary.Array_Length` (`self.stopAtors`)))))))

(fn `routeHistoryBeen`
  (params (thisStop :type "Actor Object Reference"))
  (returns (haveBeen :type Boolean))
  (return (`KismetArrayLibrary.Array_Contains` (`self.stopAtors`) thisStop)))

(fn `UserConstructionScript`)