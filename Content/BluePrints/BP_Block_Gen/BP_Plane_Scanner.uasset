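; BP_Plane_Scanner is an unfinished Blueprint for scanning a plane primitive.
; Its scanPlane event fires a single complex Visibility trace straight down through the component's bounds center, spanning UpFromPlaneZ above and below, with one-frame debug drawing.
; The hit result is not used, PlaneScanResolution is not wired in, and the StartNow check on BeginPlay leads nowhere.
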(event `self.ReceiveBeginPlay`
  (if (`self.startNow`)
    _))

(event `scanPlane`
  (bind _planeprimitive (`self.planePrimitive`)
    (:`then`
      (bind _origin (`KismetSystemLibrary.GetComponentBounds` _planeprimitive))
      (`KismetSystemLibrary.LineTraceSingle` :`Start` (`KismetMathLibrary.MakeVector` (.x _origin) (.y _origin) (+ (.z _origin) (`self.upFromPlaneZ`))) :`End` (`KismetMathLibrary.MakeVector` (.x _origin) (.y _origin) (- (.z _origin) (`self.upFromPlaneZ`))) :`TraceChannel` "TraceTypeQuery1" :`bTraceComplex` true :`DrawDebugType` "ForOneFrame"))
    (:`else`)))

(fn `UserConstructionScript`)