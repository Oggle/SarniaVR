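; BP_Metronome_Helper is an actor that runs a Quartz-clocked music loop with a blinking metronome light.
; BeginPlay creates the clock, loads sound sets into track components and queues them on bar boundaries, resuming the clock once queued.
; Quantization events toggle the light material, print debug info and, every LengthOfMusicInBars, alternately replay two banks filled with the same components.
; An older playback-percent transition method remains unused.
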(event `StartMusicSequencer`
  ;[0.2724 1 0.09082] Start Music init from tutorial 1 with the playback hack
)

(event `self.ReceiveBeginPlay`
  ;[1 0.06181 0] Begin Play
  (bind _assarnia_vrthird_person (cast `/Game/GameReady/SarniaVRThirdPerson` (`GameplayStatics.GetPlayerPawn` 0)))
  (set `self.firstPersonRef` _assarnia_vrthird_person)
  (`self.StartQuartz`)
  (`KismetSystemLibrary.PrintString` "Hello"))

(event `StartQuartz`
  ;[1 0.06253 0] Tutorial 2 Quart Based with musical timing
  ;;[1 0.06871 0.9013] Quartz initialize and settings
  (bind _returnvalue (`QuartzSubsystem.CreateNewClock` (subsystem `QuartzSubsystem`) (`self.bpmClock`) (make `QuartzClockSettings` (make `QuartzTimeSignature` (`self.qTSBeats`) (`self.QTSBeatType`))) false true))
  (bind _output_get (set `self.musicClockRef` _returnvalue))
  ;;[1 0.1706 0.52] Set beats per minute and insert sound
  (`QuartzClockHandle.SetBeatsPerMinute` :`self` _output_get :`BeatsPerMinute` (`self.beatsPerMinute`))
  (`self.setSounds`)
  (`AudioComponent.PlayQuantized` (`self.storedSounds1`) (`self.musicClockRef`) (make `QuartzQuantizationBoundary` "Bar" 1.0 "TransportRelative") (`|CreateDelegate` :!event `queStatus`) 0.0 0.0 (`self.musicVolumeLevel`) "Linear")
  ;;[1 0 0.6873] One Off Sounds
  (`self.setSounds`)
  (`AudioComponent.PlayQuantized` :`self` (`self.storedOneOffSounds`) :`InClockHandle` (`self.musicClockRef`) :`InQuantizationBoundary` (make `QuartzQuantizationBoundary` "Bar" 1.0 "TransportRelative") :`InFadeVolumeLevel` (`self.musicVolumeLevel`))
  (`KismetSystemLibrary.PrintString` "Hello")
  (`QuartzClockHandle.SubscribeToQuantizationEvent` (`self.musicClockRef`) (`self.subscribeToQBeat`) (`|CreateDelegate` :!event `playSounds`)))

(event `queStatus`
  (params (EventType :type "EQuartzCommandDelegateSubType Enum" :default "CommandOnFailedToQueue") (Name :type Name))
  ;[1 0.06253 0] Tutorial 2 Quart Based with musical timing
  ;;[0.4098 0.5521 0.0123] Que Status Deligate supporting quartz events
  (switch `EQuartzCommandDelegateSubType` EventType
    (:`CommandOnQueued`
      (`QuartzClockHandle.ResumeClock` (`self.musicClockRef`)))))

(event `self.ReceiveTick`
  (params (DeltaSeconds :type "Float (single-precision)")))

(event `playSounds`
  (params (ClockName :type Name) (QuantizationType :type "EQuartzCommandQuantization Enum" :default "Bar") (NumBars :type Integer) (Beat :type Integer) (BeatFraction :type "Float (double-precision)"))
  (bind _quartzquantizationboundary (make `QuartzQuantizationBoundary` "Bar" 1.0 "TransportRelative"))
  (bind _musicvolumelevel (`self.musicVolumeLevel`))
  (bind _returnvalue (mod (`self.currentBar`) (`self.lengthOfMusicInBars`)))
  ;[0.955 0 1] Comment
  (`self.blinkMe` false)
  (set `self.currentBar` NumBars)
  (set `self.currentBeat` Beat)
  (`|ExecutionSequence`
    (:`then_0`
      (`/Engine/EditorBlueprintResources/StandardMacros.Gate` true :!label _label
        (:`Exit`
          (`/Engine/EditorBlueprintResources/StandardMacros.DoOnce` false :!label _label_2
            (:`Completed`
              (`KismetSystemLibrary.PrintString` "++++Next Section++++" (`self.showDebug`))
              (`/Engine/EditorBlueprintResources/StandardMacros.FlipFlop`
                (:`A`
                  (`AudioComponent.PlayQuantized` :`self` (`self.storedSounds2`) :`InClockHandle` (`self.musicClockRef`) :`InQuantizationBoundary` _quartzquantizationboundary :`InFadeVolumeLevel` _musicvolumelevel)
                  (set `self.currentBankPlaying` 2))
                (:`B`
                  (`AudioComponent.PlayQuantized` :`self` (`self.storedSounds1`) :`InClockHandle` (`self.musicClockRef`) :`InQuantizationBoundary` _quartzquantizationboundary :`InFadeVolumeLevel` _musicvolumelevel)
                  (set `self.currentBankPlaying` 1))))))))
    (:`then_1`
      (if (== _returnvalue 0)
        (goto _label :!via `Open`)
        (else
          (`|ExecutionSequence`
            (:`then_0`
              (goto _label :!via `Close`))
            (:`then_1`
              (goto _label_2 :!via `Reset`))))))
    (:`then_2`
      (bind _distanceto (`/Game/GameReady/SarniaVRThirdPerson.findClosestSomething` (`self.firstPersonRef`)))
      (`KismetSystemLibrary.PrintText` (`|FormatText` "Clock Name: {Name} \nClock Name: {VName}(Verified) \nMod: {M} \nBars: {B} \nBeats: {Bts} \nDistance: {Val} \nCurrent Bank: {Bnk}" (`self.musicClockRef`) ClockName _returnvalue (`self.currentBar`) (`self.currentBeat`) _distanceto (`self.currentBankPlaying`)) (`self.showDebug`) false (struct :`G` 0.66 :`B` 1.0 :`A` 1.0) 1.99))))

(fn `blinkMe`
  (params (turnOff :type Boolean))
  (if (`self.blinkState`)
    (for _index (range (+ (`PrimitiveComponent.GetNumMaterials` (`self.Light`)) 1))
      (`PrimitiveComponent.SetMaterial` (`self.Light`) _index (`self.offMaterial`))
      (`self.toggleState` :!label _label)
      (`KismetSystemLibrary.PrintString` (`KismetStringLibrary.Concat_StrStr` (`KismetSystemLibrary.GetDisplayName` self) " Blinked")))
    (else
      (for _index_2 (range (+ (`PrimitiveComponent.GetNumMaterials` (`self.Light`)) 1))
        (`PrimitiveComponent.SetMaterial` (`self.Light`) _index_2 (`self.onMaterial`))
        (goto _label)))))

(fn `Calc Start Time for Next Transition`
  (params (sounBase :type "SoundBase Object Reference") (playbackPercent :type "Float (double-precision)"))
  (returns (startTimeForNextTransOut :type "Float (double-precision)") (percentOffsetOut :type "Float (double-precision)"))
  (locals (l_duration :type "Float (double-precision)" :default 0.0) (l_playBackPercent :type "Float (double-precision)") (l_timeToNextTransition :type "Float (double-precision)" :default 0.0) (l_percentOffset :type "Float (double-precision)" :default 0.0))
  (bind _output_get (set `local.l_playBackPercent` playbackPercent))
  (set `local.l_duration` (`SoundBase.Duration` sounBase))
  (bind _returnvalue (mod (+ (- (* _output_get (`local.l_playBackPercent`)) (`self.transitionTime`)) (* (`GameplayStatics.GetWorldDeltaSeconds`) 2.0)) (`local.l_duration`)))
  (bind _output_get_2 (set `local.l_timeToNextTransition` _returnvalue))
  ;[1 1 1] Calc offset for playback
  (set `local.l_percentOffset` (/ _output_get_2 _returnvalue))
  (return (`local.l_timeToNextTransition`) (`local.l_percentOffset`)))

(fn `setSounds`
  (locals (local_TrackSoundBase :type "SoundBase Object Reference") (local_oneOffSBase :type "SoundBase Object Reference"))
  (bind _track_6 (`self.Track_6`))
  (bind _onesound_0 (`self.oneSound_0`))
  (bind _onesound_1 (`self.oneSound_1`))
  (bind _soundsetarray (`self.soundSetArray`))
  (bind _track_1 (`self.Track_1`))
  (bind _track_7 (`self.Track_7`))
  (bind _track_0 (`self.Track_0`))
  (bind _oneoffsoundset (`self.oneOffSoundSet`))
  (bind _track_2 (`self.Track_2`))
  (bind _track_7_2 (`self.Track_7`))
  (bind _track_0_2 (`self.Track_0`))
  (bind _track_1_2 (`self.Track_1`))
  (bind _track_2_2 (`self.Track_2`))
  (bind _track_3 (`self.Track_3`))
  (bind _track_3_2 (`self.Track_3`))
  (bind _track_4 (`self.Track_4`))
  (bind _track_5 (`self.Track_5`))
  (bind _track_6_2 (`self.Track_6`))
  (bind _track_4_2 (`self.Track_4`))
  (bind _track_5_2 (`self.Track_5`))
  (bind _local_tracksoundbase (`local.local_TrackSoundBase`))
  (bind _local_tracksoundbase_2 (`local.local_TrackSoundBase`))
  (bind _returnvalue (`KismetArrayLibrary.Array_Length` _soundsetarray))
  ;[1 0 0.08857] Clear before use
  (`KismetArrayLibrary.Array_Clear` (`self.storedSounds1`))
  (`KismetArrayLibrary.Array_Clear` (`self.storedSounds2`))
  (`|ExecutionSequence`
    (:`then_0`
      (for (_array_element _array_index) _soundsetarray
        (set `local.local_TrackSoundBase` _array_element)
        (if (not (== _array_index _returnvalue))
          (`/Engine/EditorBlueprintResources/StandardMacros.Do N` _returnvalue :!label _label
            (:`Exit`
              (switch `int` _array_index
                (:`0`
                  ;[1 0.3965 0.02884] Group 1
                  (`AudioComponent.SetSound` _track_0_2 _local_tracksoundbase_2)
                  (`KismetArrayLibrary.Array_Add` (`self.storedSounds1`) _track_0_2)
                  ;[1 0.06871 0.9013] Group 1
                  (`AudioComponent.SetSound` _track_0 _local_tracksoundbase)
                  (`KismetArrayLibrary.Array_Add` (`self.storedSounds2`) _track_0))
                (:`1`
                  (`AudioComponent.SetSound` _track_1_2 _local_tracksoundbase_2)
                  (`KismetArrayLibrary.Array_Add` (`self.storedSounds1`) _track_1_2)
                  (`AudioComponent.SetSound` _track_1 _local_tracksoundbase)
                  (`KismetArrayLibrary.Array_Add` (`self.storedSounds2`) _track_1))
                (:`2`
                  (`AudioComponent.SetSound` _track_2_2 _local_tracksoundbase_2)
                  (`KismetArrayLibrary.Array_Add` (`self.storedSounds1`) _track_2_2)
                  (`AudioComponent.SetSound` _track_2 _local_tracksoundbase)
                  (`KismetArrayLibrary.Array_Add` (`self.storedSounds2`) _track_2))
                (:`3`
                  (`AudioComponent.SetSound` _track_3_2 _local_tracksoundbase_2)
                  (`KismetArrayLibrary.Array_Add` (`self.storedSounds1`) _track_3_2)
                  (`AudioComponent.SetSound` _track_3 _local_tracksoundbase)
                  (`KismetArrayLibrary.Array_Add` (`self.storedSounds2`) _track_3))
                (:`4`
                  (`AudioComponent.SetSound` _track_4 _local_tracksoundbase_2)
                  (`KismetArrayLibrary.Array_Add` (`self.storedSounds1`) _track_4)
                  (`AudioComponent.SetSound` _track_4_2 _local_tracksoundbase)
                  (`KismetArrayLibrary.Array_Add` (`self.storedSounds2`) _track_4_2))
                (:`5`
                  (`AudioComponent.SetSound` _track_5 _local_tracksoundbase_2)
                  (`KismetArrayLibrary.Array_Add` (`self.storedSounds1`) _track_5)
                  (`AudioComponent.SetSound` _track_5_2 _local_tracksoundbase)
                  (`KismetArrayLibrary.Array_Add` (`self.storedSounds2`) _track_5_2))
                (:`6`
                  (`AudioComponent.SetSound` _track_6_2 _local_tracksoundbase_2)
                  (`KismetArrayLibrary.Array_Add` (`self.storedSounds1`) _track_6_2)
                  (`AudioComponent.SetSound` _track_6 _local_tracksoundbase)
                  (`KismetArrayLibrary.Array_Add` (`self.storedSounds2`) _track_6))
                (:`7`
                  (`AudioComponent.SetSound` _track_7_2 _local_tracksoundbase_2)
                  (`KismetArrayLibrary.Array_Add` (`self.storedSounds1`) _track_7_2)
                  (`AudioComponent.SetSound` _track_7 _local_tracksoundbase)
                  (`KismetArrayLibrary.Array_Add` (`self.storedSounds2`) _track_7)))))))
      (goto _label :!via `Reset`))
    (:`then_1`
      ;[1 0.2892 0.1795] One off sound handling
      (for (_array_element_2 _array_index_2) _oneoffsoundset
        (set `local.local_oneOffSBase` _array_element_2)
        (if (not (== _array_index_2 (`KismetArrayLibrary.Array_Length` _oneoffsoundset)))
          (`/Engine/EditorBlueprintResources/StandardMacros.Do N` _array_index_2 :!label _label_2
            (:`Exit`
              (switch `int` _array_index_2
                (:`0`
                  (`AudioComponent.SetSound` _onesound_0 (`local.local_oneOffSBase`))
                  (`KismetArrayLibrary.Array_Add` (`self.storedOneOffSounds`) _onesound_0))
                (:`1`
                  (`AudioComponent.SetSound` _onesound_1 (`local.local_oneOffSBase`))
                  (`KismetArrayLibrary.Array_Add` (`self.storedOneOffSounds`) _onesound_1)))))))
      (goto _label_2 :!via `Reset`))))

(fn `toggleState`
  (if (`self.blinkState`)
    (set `self.blinkState` false)
    (else
      (set `self.blinkState` true))))

(fn `UserConstructionScript`)