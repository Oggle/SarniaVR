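; BP_Building_Generator is an early-stage building actor whose construction script tints a story mesh and positions a window on it.
; Colour and tiling reach the story's material through custom primitive data.
; The story's local bounds, oriented by a Y-forward flag, plus floor count and offsets set the single Window component's location.
; An unconnected nested loop would add chosen window meshes per floor, but it never runs.
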(fn `UserConstructionScript`
  (locals (local_storyWidth :type "Float (double-precision)") (local_storyHeight :type "Float (double-precision)") (local_storyDepth :type "Float (double-precision)"))
  (bind _story (`self.Story`))
  (bind (_colour_r _colour_g _colour_b) (break `LinearColor` (`self.colour`)))
  (bind (_min _max) (`StaticMeshComponent.GetLocalBounds` (`self.Story`)))
  (bind _x (.x (- _max _min)))
  (bind _y (.y (- _max _min)))
  (`|ExecutionSequence`
    (:`then_0`
      ;[0.7195 1 0] Set primitive colour and tiling from RGBA which  feeds the material
      (`PrimitiveComponent.SetCustomPrimitiveDataFloat` _story 0 0.0)
      (`PrimitiveComponent.SetCustomPrimitiveDataVector4` _story 0 (`KismetMathLibrary.MakeVector4` _colour_r _colour_g _colour_b (`self.tiling`))))
    (:`then_1`
      (`SceneComponent.K2_SetRelativeLocation` (`self.window`) (0.0 0.0 0.0) false false)
      (`|ExecutionSequence`
        (:`then_0`
          ;[0.04337 0.127 1] If Y is forward then make it the depth
          (if (`self.yForward`)
            (set `local.local_storyDepth` _y)
            (set `local.local_storyWidth` _x)
            (else
              (set `local.local_storyDepth` _x)
              (set `local.local_storyWidth` _y))))
        (:`then_1`
          (set `local.local_storyHeight` (.z (- _max _min)))
          ;[1 1 1] Produce windows all over
          (`SceneComponent.K2_SetRelativeLocation` (`self.window`) (`KismetMathLibrary.MakeVector` (/ (`local.local_storyDepth`) 2.0) (+ (/ (`local.local_storyWidth`) 2.0) (`self.window_off_wall`)) (+ (+ (/ (/ (`local.local_storyHeight`) 2.0) (`KismetMathLibrary.Conv_IntToDouble` (`self.floorCount`))) (`self.window_off_ground`)) (`self.window_center_z`))) false false))))))