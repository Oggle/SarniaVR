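; BP_Knob is a knob control actor from the buttons and switches set, with a mesh and a text label.
; The construction script places UiControlMesh by an offset transform, then sizes the label, shifts it additively by a configured location and fills it from MyLabel.
; Runtime behavior is only a placeholder: overlapping the mesh prints a fixed debug message, and the knob has no turning or value logic.
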(event `self.uiControlMesh.OnComponentBeginOverlap`
  (params (OverlappedComponent :type "PrimitiveComponent Object Reference") (OtherActor :type "Actor Object Reference") (OtherComp :type "PrimitiveComponent Object Reference") (OtherBodyIndex :type Integer) (bFromSweep :type Boolean) (SweepResult :type "HitResult Structure (by ref)"))
  (`KismetSystemLibrary.PrintString` "Hello"))

(fn `UserConstructionScript`
  (bind _showinfotxttransform_location (`KismetMathLibrary.BreakTransform` (`self.showInfoTxtTransform`)))
  (`SceneComponent.K2_SetRelativeTransform` (`self.uiControlMesh`) (`self.uiControlMeshOffsets`) false false)
  (`TextRenderComponent.SetWorldSize` (`self.showInfoTxt`) (`self.controlLabelTextSize`))
  (`SceneComponent.K2_AddRelativeLocation` (`self.showInfoTxt`) _showinfotxttransform_location false false)
  (bind _output_get (set `self.showLabelTxt` (`KismetTextLibrary.Conv_StringToText` (`self.myLabel`))))
  (`TextRenderComponent.K2_SetText` (`self.showInfoTxt`) _output_get))