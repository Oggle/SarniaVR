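; Throwable boomerang actor that is held through a grab component and flies a curved path when dropped.
; While held, Tick derives velocity from frame-to-frame transforms and switches between in-hand and throw-tracking states by movement per frame.
; Dropping engages flight, detaching it with overlap collision; Tick then rotates the velocity each frame, eases height toward the player pawn and spins the actor.
; A Begin/End state machine handles transitions, mostly with debug prints.
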(event `self.ReceiveBeginPlay`
  ;[1 0.1784 0.8721] Bind to the grab component drop
  (add `/Game/VRTemplate/Blueprints/GrabComponent.OnDropped` (`self.GrabComponent`) (delegate `dropWithVelocity`)))

(event `dropWithVelocity`
  ;[1 0.1784 0.8721] Bind to the grab component drop
  (`self.releaseMyThrow`))

(event `self.ReceiveTick`
  (params (DeltaSeconds :type "Float (single-precision)"))
  (bind (_returnvalue_location _returnvalue_rotation) (`KismetMathLibrary.BreakTransform` (`self.GetTransform`)))
  (bind (_oldtransform_location _oldtransform_rotation) (`KismetMathLibrary.BreakTransform` (`self.oldTransform`)))
  (bind (_boomerangfulcrumoffset_x _boomerangfulcrumoffset_y _boomerangfulcrumoffset_z) (`KismetMathLibrary.BreakVector` (`self.boomerangFulcrumOffset`)))
  (bind _oldtransform_location_2 (`KismetMathLibrary.BreakTransform` (`self.oldTransform`)))
  (bind _delta_seconds (`self.Delta Seconds`))
  (bind (_returnvalue_x _returnvalue_y _returnvalue_z) (`KismetMathLibrary.BreakVector` (`self.K2_GetActorLocation` (`GameplayStatics.GetPlayerPawn` 0))))
  (bind (_returnvalue_x_2 _returnvalue_y_2 _returnvalue_z_2) (`KismetMathLibrary.BreakVector` (`SceneComponent.K2_GetComponentLocation` (`self.BoRang_Standard_01`))))
  (bind _rotation (.rotation (`self.GetTransform`)))
  (bind _returnvalue (* (`KismetMathLibrary.GetPI`) -0.1))
  (set `self.Delta Seconds` DeltaSeconds)
  ;[0.7152 0.02946 1] Are We Flying
  (if (not (`self.engageFlight`))
    ;[0.5981 0 1 1 12] If We Are Held then start tracking check
    (if (`/Game/VRTemplate/Blueprints/GrabComponent.bIsHeld` (`self.GrabComponent`))
      ;[1 0 0.03209] Classic then and Now distance velocity calculation
      (bind (_nowvelocityvector _nowvwctorlength) (`self.Get My Velocity Vector` _returnvalue_location _oldtransform_location))
      (set `self.myVelocityVector` _nowvelocityvector)
      (set `self.local_vectorLength` _nowvwctorlength)
      (bind _nowrotationvelocity (`self.getRotationVelocity` _returnvalue_rotation _oldtransform_rotation))
      (set `self.boomerangLaunchRotator` _nowrotationvelocity)
      (set `self.oldTransform` (`KismetMathLibrary.MakeTransform` (+ (.location (`self.GetTransform`)) (* (`KismetMathLibrary.GetRightVector` _rotation) _boomerangfulcrumoffset_z)) (`KismetMathLibrary.MakeRotator` (.roll _rotation) (.pitch _rotation) (.yaw _rotation))))
      ;;[1 0 0.7295] Switch between in hand and tracking to throw
      (if (> (`self.local_vectorLength`) (`self.trackingVelocityThreshold`))
        (`self.setBoomerangState` "NewEnumerator3")
        (`KismetSystemLibrary.LineTraceSingle` :`Start` _oldtransform_location_2 :`End` (* (`self.myVelocityVector`) (`self.boomerangSpeed`)) :`TraceChannel` "TraceTypeQuery1" :`DrawDebugType` "ForOneFrame")
        (else
          (`self.setBoomerangState` "NewEnumerator2"))))
    (else
      ;[1 0 0.1598] Dirty Original Release Course
      (set `self.currentPathRot` _returnvalue)
      (bind _output_get (set `self.myVelocityVector` (`KismetMathLibrary.GreaterGreater_VectorRotator` (`self.myVelocityVector`) (`KismetMathLibrary.MakeRotator` 0.0 0.0 _returnvalue))))
      (`self.K2_AddActorWorldTransform` (`KismetMathLibrary.MakeTransform` (`KismetMathLibrary.MakeVector` (.x (* (`KismetMathLibrary.MakeVector` (.x _output_get) (.y _output_get) (.z _output_get)) _delta_seconds)) (.y (* (`KismetMathLibrary.MakeVector` (.x _output_get) (.y _output_get) (.z _output_get)) _delta_seconds)) (* (- (+ _returnvalue_z 42.0) _returnvalue_z_2) _delta_seconds)) (`KismetMathLibrary.MakeRotator` 0.0 0.0 (* (`self.currentPathRot`) (`self.Delta Seconds`)))))
      ;[1 0.001901 0.3054] SideSpin
      (`self.K2_AddActorLocalRotation` (`KismetMathLibrary.MakeRotator` 0.0 0.0 (* (`self.boomerangSpinSpeed`) (`self.Delta Seconds`))))
      (set `self.oldTransform` (`self.GetTransform`)))))

(fn `beginState`
  (params (thisState :type "/Game/BluePrints/BP_Weapons/Boomerang/EBoomerangState Enum" :default "NewEnumerator0"))
  (switch `/Game/BluePrints/BP_Weapons/Boomerang/EBoomerangState` thisState
    (:`NewEnumerator3`
      (`KismetSystemLibrary.PrintString` "Tracking"))
    (:`NewEnumerator4`
      (`KismetSystemLibrary.PrintString` "FLYING")
      (`self.K2_DetachFromActor` "KeepWorld" "KeepWorld" "KeepWorld")
      (`PrimitiveComponent.SetCollisionProfileName` (`self.BoRang_Standard_01`) "OverlapAllDynamic" true))))

(fn `endState`
  (params (thisState :type "/Game/BluePrints/BP_Weapons/Boomerang/EBoomerangState Enum" :default "NewEnumerator0"))
  (switch `/Game/BluePrints/BP_Weapons/Boomerang/EBoomerangState` thisState
    (:`NewEnumerator2`
      (`KismetSystemLibrary.PrintString` "LeftHand"))
    (:`NewEnumerator3`
      (`KismetSystemLibrary.PrintString` "NotTracking"))
    (:`NewEnumerator4`
      (`KismetSystemLibrary.PrintString` "Landed"))))

(fn `Get My Velocity Vector`
  (params (nowVector :type "Vector Structure") (thenVector :type "Vector Structure"))
  (returns (nowVelocityVector :type "Vector Structure") (nowVwctorLength :type "Float (double-precision)"))
  (bind _returnvalue (- nowVector thenVector))
  (return (/ _returnvalue (`self.Delta Seconds`)) (`KismetMathLibrary.VSize` _returnvalue)))

(fn `getRotationVelocity`
  (params (nowRotation :type "Rotator Structure") (thenRotation :type "Rotator Structure"))
  (returns (nowRotationVelocity :type "Rotator Structure"))
  (return (`KismetMathLibrary.MakeRotator` (- nowRotation_Roll thenRotation_Roll) (- nowRotation_Pitch thenRotation_Pitch) (- nowRotation_Yaw thenRotation_Yaw))))

(fn `releaseMyThrow`
  (set `self.engageFlight` true)
  (`self.setBoomerangState` "NewEnumerator4")
  (`KismetSystemLibrary.PrintString` "Throw Released" true true (struct :`R` 1.0 :`G` 0.756773 :`A` 1.0)))

(fn `setBoomerangState`
  (params (newState :type "/Game/BluePrints/BP_Weapons/Boomerang/EBoomerangState Enum" :default "NewEnumerator0"))
  (bind _boomerangstate (`self.boomerangState`))
  (bind _newstate (`local.newState`))
  (if (`|EnumInequality` newState _boomerangstate)
    (`self.endState` _boomerangstate)
    (set `self.boomerangState` _newstate)
    (`self.beginState` _newstate)))

(fn `UserConstructionScript`
  (set `self.boomerangState` "NewEnumerator1")
  (`SceneComponent.K2_SetRelativeRotation` (`self.BoRang_Standard_01`) (struct :`Pitch` 180.0) false false))