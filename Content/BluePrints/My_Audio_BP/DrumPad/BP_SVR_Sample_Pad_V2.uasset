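; Drum pad actor that plays a random sample and can flash an emissive material when something overlaps its trigger mesh.
; The construction script sets meshes, sound cue, scale, colour, optional material overrides and a text title from presets and instance settings.
; Overlaps pass a delta-seconds gate meant to stop retriggers, then set a random cue integer parameter to choose the sample.
; Drumstick filtering, hit velocity, haptics and kit grouping are present but unwired.
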(event `self.ReceiveBeginPlay`
  (set `self.oldGate` (`GameplayStatics.GetWorldDeltaSeconds`))
  ;[0 0.2046 1 1 14] Store original material at emissive int slot of the trigger mesh. This assumes index 0 is the body of the object.
  (set `self.oldTriggerMatterial` (`|GetArrayItem` (`MeshComponent.GetMaterials` (`self.myMesh`)) (`self.emissiveTriggerSlot`))))

(event `self.myTrigger.OnComponentBeginOverlap`
  (params (OverlappedComponent :type "PrimitiveComponent Object Reference") (OtherActor :type "Actor Object Reference") (OtherComp :type "PrimitiveComponent Object Reference") (OtherBodyIndex :type Integer) (bFromSweep :type Boolean) (SweepResult :type "HitResult Structure (by ref)"))
  ;[0.5677 0.3773 0] Testing just overlap trigger
  (`KismetSystemLibrary.PrintString` "Drum Trigger Overlap" true true (struct :`R` 0.760417 :`G` 0.033362 :`A` 1.0))
  ;[0.2571 1 0] Trying to prevent retriggers
  (if (< (`GameplayStatics.GetWorldDeltaSeconds`) (+ (`self.oldGate`) (`self.gateMin`)))
    ;[0.04928 0.4855 1] Capture Overlap Object
    (set `self.triggerByOverlapComponent` OverlappedComponent)
    (bind _output_get (set `self.triggerHitByActor` OtherActor))
    (`KismetSystemLibrary.PrintString` (`KismetStringLibrary.Conv_VectorToString` (`self.GetVelocity` _output_get)))
    (`|ExecutionSequence`
      (:`then_0`
        ;[1 0 0.02203] Firiing Correct Samples
        ;;[0.4965 0.1124 1 1 12] Sample set from use sample int to the cue hit table of switch names with a set modulus vol integer for right now
        (`AudioComponent.SetIntParameter` (`self.DP_SamplePad_Cue`) "dynSampleInt" (`KismetMathLibrary.RandomInteger` (`self.hitVolModulus`)))
        (`AudioComponent.Play` (`self.DP_SamplePad_Cue`) (`self.fineSampleOffsetStart`)))
      (:`then_1`
        ;[1 0.88 0.276] Light Up material animation
        (if (`self.lightUp`)
          ;;[1 0.125 0.125] Reset to original then set the emissive
          (`PrimitiveComponent.SetMaterial` (`self.myTrigger`) (`self.emissiveTriggerSlot`) (`self.oldTriggerMatterial`))
          (`PrimitiveComponent.SetMaterial` (`self.myTrigger`) (`self.emissiveTriggerSlot`) (`self.emmisiveMaterial`))
          ;;[0.2294 1 0] Delay then return to the original material
          (`KismetSystemLibrary.Delay` (`self.animHitDelay`))
          (`PrimitiveComponent.SetMaterial` (`self.myTrigger`) (`self.emissiveTriggerSlot`) (`self.oldTriggerMatterial`))))
      (:`then_2`
        (set `self.oldGate` (`GameplayStatics.GetWorldDeltaSeconds`))))))

(event `self.myTrigger.OnComponentEndOverlap`
  (params (OverlappedComponent :type "PrimitiveComponent Object Reference") (OtherActor :type "Actor Object Reference") (OtherComp :type "PrimitiveComponent Object Reference") (OtherBodyIndex :type Integer))
  ;[1 0.7392 0.01289] Open Hard Overlap GATE
  ;;[1 0.04418 0] using trigger as end overlap
)

(event `self.myMesh.OnComponentEndOverlap`
  (params (OverlappedComponent :type "PrimitiveComponent Object Reference") (OtherActor :type "Actor Object Reference") (OtherComp :type "PrimitiveComponent Object Reference") (OtherBodyIndex :type Integer))
  ;[1 0.7392 0.01289] Open Hard Overlap GATE
  ;;[1 0.04418 0] using trigger as end overlap
)

(fn `UserConstructionScript`
  (locals (local_myTextRenderTitle :type "TextRenderComponent Object Reference") (local_nextPolyChannel :type "AudioComponent Object Reference") (local_mySampleChannelArray :type "Array of AudioComponent Object Reference") (local_DPKitCheck :type "/Game/BluePrints/My_Audio_BP/DrumPad/BP_SVR_Sample_Pad_V2 Object Reference") (local_nearByKitArray :type "Array of Integer") (nearByDrumPadsArray :type "Array of /Game/BluePrints/My_Audio_BP/DrumPad/BP_SVR_Sample_Pad_V2 Object Reference") (local_dpKitInt :type Integer) (local_triggerTransform :type "Vector Structure"))
  (bind (_drumscale_location _drumscale_rotation _drumscale_scale) (`KismetMathLibrary.BreakTransform` (`self.drumScale`)))
  (bind _local_mytextrendertitle (`local.local_myTextRenderTitle`))
  (bind (_mydp_inst_id _mydp_inst_title _mydp_inst_note _mydp_inst_dp_soundcue) (break `/Game/BluePrints/My_Audio_BP/DrumPad/Structs/DP_Poly_Drum_Inst` (`self.myDP_Inst`)))
  (bind _mymesh (`self.myMesh`))
  (bind (_returnvalue_location _returnvalue_rotation _returnvalue_scale) (`KismetMathLibrary.BreakTransform` (`SceneComponent.GetRelativeTransform` (`self.myTrigger`))))
  (bind (_returnvalue_location_2 _returnvalue_rotation_2 _returnvalue_scale_2) (`KismetMathLibrary.BreakTransform` (`SceneComponent.GetRelativeTransform` (`self.myMesh`))))
  (bind (_r _g _b) (`KismetMathLibrary.BreakColor` (`self.primitiveColour`)))
  (bind (_id _drumstaticmesh _deftriggermesh _noshell _title _author _triggeradjust) (break `/Game/BluePrints/My_Audio_BP/DrumPad/Structs/DP_Mesh_Types` (`|GetArrayItem` (`self.DP_DrumMeshes`) (`self.useDPDrumMesh`))))
  (bind _y (.y (.scale (`self.padTitleOffset`))))
  (bind _x (.x (+ _returnvalue_scale_2 _drumscale_scale)))
  (bind _x_2 (.x (+ _returnvalue_scale _drumscale_scale)))
  ;[1 0 0.0169] CONSTRUCTION
  ;[1 0.3601 0] Array Resets
  (`KismetArrayLibrary.Array_Clear` (`local.local_nearByKitArray`))
  ;[1 0.5376 0.0904] Set Custom Shell and Skins
  (`StaticMeshComponent.SetStaticMesh` (`self.myMesh`) _drumstaticmesh)
  (`StaticMeshComponent.SetStaticMesh` (`self.myTrigger`) _deftriggermesh)
  (set `local.local_triggerTransform` _triggeradjust)
  ;[1 0.06221 0.2526] Set Drum Sound Cue for this Pad
  (`AudioComponent.SetSound` (`self.DP_SamplePad_Cue`) _mydp_inst_dp_soundcue)
  ;[0.9124 0.1697 1] Over complicated scaling of trigger and mesh, need to find a way to keep mesh below trigger at z-half zbound
  (`SceneComponent.K2_SetRelativeTransform` (`self.myMesh`) (`KismetMathLibrary.MakeTransform` _returnvalue_location_2 (struct) (`KismetMathLibrary.MakeVector` _x _x (.z (+ _returnvalue_scale_2 _drumscale_scale)))) false false)
  (`SceneComponent.K2_SetRelativeTransform` (`self.myTrigger`) (`KismetMathLibrary.MakeTransform` (`local.local_triggerTransform`) (struct) (`KismetMathLibrary.MakeVector` _x_2 _x_2 1.0)) false false)
  ;[1 0.5344 0] Establish Primitive Colour  Connection
  (`PrimitiveComponent.SetCustomPrimitiveDataFloat` _mymesh 0 0.0)
  (`PrimitiveComponent.SetCustomPrimitiveDataVector3` _mymesh 0 (`KismetMathLibrary.MakeVector` _r _g _b))
  ;[1 0.3866 0 1 14] Store transform of the trigger mesh
  (set `self.triggerMeshTransform` (`SceneComponent.GetRelativeTransform` (`self.myTrigger`)))
  (`|ExecutionSequence`
    (:`then_0`
      ;[1 0 0.2223] Override Materials
      (if (`self.overrideMaterials`)
        (`|ExecutionSequence`
          (:`then_0`
            ;[1 0.1208 0.3216] Set mesh material
            (`PrimitiveComponent.SetMaterial` (`self.myMesh`) 0 (`|GetArrayItem` (`self.meshMaterial`) (`self.useMeshMaterial`))))
          (:`then_1`
            ;[1 0 0.4547] Visible Trigger if so use material
            (if (`self.triggerMeshVisible`)
              (`PrimitiveComponent.SetMaterial` (`self.myTrigger`) 0 (`|GetArrayItem` (`self.meshMaterial`) (`self.useTriggerMaterial`)))
              (else
                (`SceneComponent.SetVisibility` (`self.myTrigger`) false false)))))))
    (:`then_1`
      ;[0.4651 1 0.1096] Show Title Of Sample
      (if (`self.showTitle`)
        (bind _returnvalue (`AddComponent|NODE_AddTextRenderComponent-0`))
        (set `local.local_myTextRenderTitle` _returnvalue)
        (if (`KismetStringLibrary.NotEqual_StrStr` (`self.userDrumTitle`))
          (`TextRenderComponent.K2_SetText` (`local.local_myTextRenderTitle`) (`KismetTextLibrary.Conv_StringToText` (`self.userDrumTitle`)))
          (else
            (`TextRenderComponent.K2_SetText` (`local.local_myTextRenderTitle`) (`KismetTextLibrary.Conv_NameToText` (`KismetStringLibrary.Conv_StringToName` (`.Title_5_B7AB38F14B84A1D75264EB88009C25FD` (break `/Game/BluePrints/My_Audio_BP/DrumPad/Structs/DP_Poly_Drum_Inst` (`self.myDP_Inst`))))))))
        (`TextRenderComponent.SetHorizontalAlignment` (`local.local_myTextRenderTitle`) "EHTA_Center")
        (`SceneComponent.K2_SetRelativeTransform` _local_mytextrendertitle (`KismetMathLibrary.MakeTransform` (.location (`self.padTitleOffset`)) (struct) (`KismetMathLibrary.MakeVector` 1.0 _y _y)) false false)
        (`SceneComponent.K2_SetWorldRotation` _local_mytextrendertitle (.rotation (`self.padTitleOffset`)) false false)))
    (:`then_2`
      ;[0.4455 1 0] notused
      (if (`self.noOverlapOthers`)
        _))))