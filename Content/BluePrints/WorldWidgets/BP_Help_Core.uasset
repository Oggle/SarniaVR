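; In-world help widget with an optionally spinning icon, whose title and body panels appear with a sound when the first player's pawn enters its collision sphere.
; The Construction Script creates the text renders and applies configurable meshes, materials, transforms, trigger radius and starting visibility, passing colours through Custom Primitive Data.
; The visibility toggle leaves the icon untouched, and nothing hides the panels on exit.
; Layout is manual, as the auto-sizing logic is disconnected.
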(event `self.ReceiveBeginPlay`)

(event `self.ReceiveTick`
  (params (DeltaSeconds :type "Float (single-precision)"))
  (set `self.Delta Seconds` DeltaSeconds)
  ;[1 0.8026 0.04144] Animate the Icon
  (if (`self.animateIcon`)
    (`SceneComponent.K2_AddWorldRotation` (`self.Iconmesh`) (`KismetMathLibrary.MakeRotator` 0.0 0.0 (`self.spinSpeed`)) false false)))

(event `self.myCollisionSphere.OnComponentBeginOverlap`
  (params (OverlappedComponent :type "PrimitiveComponent Object Reference") (OtherActor :type "Actor Object Reference") (OtherComp :type "PrimitiveComponent Object Reference") (OtherBodyIndex :type Integer) (bFromSweep :type Boolean) (SweepResult :type "HitResult Structure (by ref)"))
  ;[0.1003 1 0.9203] Check that a player hit us
  (if (== OtherActor (`GameplayStatics.GetPlayerPawn` 0))
    (`self.Set All Visibility` true true)
    (`AudioComponent.Play` (`self.CompileSuccess_Cue`) 0.0)))

(fn `getObjectDimension`
  (params (staticMeshComponent :type "StaticMeshComponent Object Reference") (useScale :type Boolean))
  (returns (meshSize :type "Vector Structure"))
  (locals (local_scaleVector :type "Vector Structure" :default (0.0 0.0 0.0)))
  (bind (_min _max) (`StaticMeshComponent.GetLocalBounds` staticMeshComponent))
  (if useScale
    (set `local.local_scaleVector` (`SceneComponent.K2_GetComponentScale` staticMeshComponent)))
  (return (* (`local.local_scaleVector`) (- _max _min))))

(fn `Set All Visibility`
  (params (setAllVisible :type Boolean) (setChildren :type Boolean))
  (set `self.weAreVisible` (`local.setAllVisible`))
  (`SceneComponent.SetVisibility` (`self.myTextTitle`) (`local.setAllVisible`) (`local.setChildren`))
  (`SceneComponent.SetVisibility` (`self.bodyText`) (`local.setAllVisible`) (`local.setChildren`))
  (`SceneComponent.SetVisibility` (`self.titleBackingMesh`) (`local.setAllVisible`) (`local.setChildren`))
  (`SceneComponent.SetVisibility` (`self.BodyBackingMesh`) (`local.setAllVisible`) (`local.setChildren`)))

(fn `UserConstructionScript`
  (locals (local_myWidget :type "UserWidget Object Reference") (local_addedWidgetDyn :type "WidgetComponent Object Reference") (local_widgetMenu :type "/Game/BluePrints/WorldWidgets/DP_Pad_Menu Object Reference") (local_DynWidget :type "/Game/BluePrints/WorldWidgets/DP_Pad_Menu Object Reference") (local_myIcon :type "/Game/BluePrints/WorldWidgets/HelpCoreIcons Structure"))
  (bind _mytexttitle (`self.myTextTitle`))
  (bind (_local_myicon_id _local_myicon_title _local_myicon_type _local_myicon_iconmesh _local_myicon_iconcolor _local_myicon_iconmaterial) (break `/Game/BluePrints/WorldWidgets/HelpCoreIcons` (`local.local_myIcon`)))
  (bind (_icontransform_location _icontransform_rotation _icontransform_scale) (`KismetMathLibrary.BreakTransform` (`self.iconTransform`)))
  (bind _bodytext (`self.bodyText`))
  (bind (_backingmeshcolour_r _backingmeshcolour_g _backingmeshcolour_b _backingmeshcolour_a) (break `LinearColor` (`self.backingMeshColour`)))
  (bind (_r _g _b _a) (`KismetMathLibrary.BreakColor` (`self.titleMeshColour`)))
  (bind (_r_2 _g_2 _b_2 _a_2) (`KismetMathLibrary.BreakColor` (`.iconColor_16_AE504C0F464DE1DD0803B281E29AA26B` (break `/Game/BluePrints/WorldWidgets/HelpCoreIcons` (`local.local_myIcon`)))))
  ;[0.331 1 0.3281] Create and set the text render for the title and the body text
  (bind _returnvalue (`AddComponent|NODE_AddTextRenderComponent-0`))
  (bind _returnvalue_2 (`AddComponent|NODE_AddTextRenderComponent-1`))
  (set `self.myTextTitle` _returnvalue)
  (set `self.bodyText` _returnvalue_2)
  ;[0 0.8423 1] Set the Icon custom static mesh
  (bind _output_get (set `local.local_myIcon` (`|GetArrayItem` (`self.myWidgetIcons`) (`self.useIconMesh`))))
  (`StaticMeshComponent.SetStaticMesh` (`self.Iconmesh`) (`.iconMesh_13_ABB396B54E45F6E190FA939AF24C9323` (break `/Game/BluePrints/WorldWidgets/HelpCoreIcons` _output_get)))
  ;[0 0.2703 1 1 14] Set the bodybacking mesh to a mesh from the array of backing meshes
  (`StaticMeshComponent.SetStaticMesh` (`self.BodyBackingMesh`) (`|GetArrayItem` (`self.backingMeshes`) (`self.useBackingMesh`)))
  (`StaticMeshComponent.SetStaticMesh` (`self.titleBackingMesh`) (`|GetArrayItem` (`self.backingMeshes`) (`self.useTitleBackingMesh`)))
  ;[0.2356 0 1 1 14] Inject 4Vec Colour and tiling data for materials that support a primitive mesh colour
  ;;[0.1476 0.269 1 1 12] Set Icon, Body, Title Mesh Primitive4vec to our custom colour
  (`PrimitiveComponent.SetCustomPrimitiveDataVector4` (`self.Iconmesh`) 0 (`KismetMathLibrary.MakeVector4` _r_2 _g_2 _b_2 _a_2))
  (`PrimitiveComponent.SetCustomPrimitiveDataVector4` (`self.BodyBackingMesh`) 0 (`KismetMathLibrary.MakeVector4` _backingmeshcolour_r _backingmeshcolour_g _backingmeshcolour_b _backingmeshcolour_a))
  (`PrimitiveComponent.SetCustomPrimitiveDataVector4` (`self.titleBackingMesh`) 0 (`KismetMathLibrary.MakeVector4` _r _g _b _a))
  ;[0.3356 1 0.05203] Set custom material
  (`PrimitiveComponent.SetMaterial` (`self.BodyBackingMesh`) 0 (`|GetArrayItem` (`self.HC_Core_Materials`) (`self.useBackingMeshMaterial`)))
  (`PrimitiveComponent.SetMaterial` (`self.titleBackingMesh`) 0 (`|GetArrayItem` (`self.HC_Core_Materials`) (`self.useTitleMeshMaterial`)))
  (`PrimitiveComponent.SetMaterial` (`self.Iconmesh`) 0 _local_myicon_iconmaterial)
  ;[1 0.09166 0.6459] Set the custom collision size
  (`SphereComponent.SetSphereRadius` (`self.myCollisionSphere`) (`self.collisionSize`) true)
  (`TextRenderComponent.K2_SetText` _mytexttitle (`self.showTitle`))
  (`TextRenderComponent.K2_SetText` _bodytext (`self.showText`))
  (`TextRenderComponent.SetWorldSize` _mytexttitle (`self.titleTextSize`))
  (`TextRenderComponent.SetWorldSize` _bodytext (`self.bodyTextSize`))
  ;;[1 0.0625 0.0625] Get text render dimensions
  (set `self.bodyTextDim` (`TextRenderComponent.GetTextWorldSize` (`self.bodyText`)))
  (set `self.titleTextDim` (`TextRenderComponent.GetTextWorldSize` (`self.myTextTitle`)))
  ;[1 0.01836 0] Totally Manual Adjustments
  (`SceneComponent.K2_SetRelativeTransform` (`self.BodyBackingMesh`) (`self.bodyTransform`) false false)
  (`SceneComponent.K2_SetRelativeTransform` (`self.titleBackingMesh`) (`self.titleTransform`) false false)
  (`SceneComponent.K2_SetRelativeTransform` (`self.Iconmesh`) (`self.iconTransform`) false false)
  (`SceneComponent.K2_SetRelativeLocation` (`self.bodyText`) (`self.bodyTextOffset`) false false)
  (`SceneComponent.K2_SetRelativeLocation` (`self.myTextTitle`) (`self.titleTextOffset`) false false)
  (`TextRenderComponent.SetHorizontalAlignment` (`self.bodyText`) "EHTA_Left")
  (`TextRenderComponent.SetHorizontalAlignment` (`self.myTextTitle`) "EHTA_Center")
  ;;[1 0.08416 0.3781] Set the icon mesh
  (`SceneComponent.K2_SetRelativeTransform` (`self.Iconmesh`) (`KismetMathLibrary.MakeTransform` _icontransform_location _icontransform_rotation _icontransform_scale) false false)
  (`self.Set All Visibility` (`self.startVisible`) true))