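; Cinematography test actor that previews a scene preset and swaps the player's camera post process on contact.
; Construction sizes the trigger sphere, applies the UseScene entry's focus, lens and post-process settings to a test camera, and labels it with floating title text.
; When the SarniaVRThirdPerson player pawn enters, it receives post-process settings from a random array entry, not necessarily UseScene.
; A gate then blocks retriggering for ReactivateDelay.
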(event `self.ReceiveActorBeginOverlap`
  (params (OtherActor :type "Actor Object Reference")))

(event `self.colSphere.OnComponentBeginOverlap`
  (params (OverlappedComponent :type "PrimitiveComponent Object Reference") (OtherActor :type "Actor Object Reference") (OtherComp :type "PrimitiveComponent Object Reference") (OtherBodyIndex :type Integer) (bFromSweep :type Boolean) (SweepResult :type "HitResult Structure (by ref)"))
  (bind _masterscenesettingsarray (`self.masterSceneSettingsArray`))
  (if (`self.gateOpen`)
    (if (== OtherActor (`GameplayStatics.GetPlayerPawn` 0))
      (bind _assarnia_vrthird_person (cast `/Game/GameReady/SarniaVRThirdPerson` OtherActor))
      (set `/Game/GameReady/SarniaVRThirdPerson.currentCameraPostProcess` (`.postProcessSettings_19_8356CE34482E18676A23A29D4FB617B9` (break `/Game/BluePrints/Cinematography/struct_CameraPostSetting` (`|GetArrayItem` _masterscenesettingsarray (`KismetMathLibrary.RandomInteger` (`KismetArrayLibrary.Array_Length` _masterscenesettingsarray))))) _assarnia_vrthird_person)
      (set `self.gateOpen` false)
      (`KismetSystemLibrary.Delay` (`self.reactivateDelay`))
      (set `self.gateOpen` true))))

(fn `UserConstructionScript`
  (locals (local_TextRender :type "TextRenderComponent Object Reference") (local_Title :type String))
  (bind _mytestcamera (`self.myTestCamera`))
  (bind (_id _title _camerafocussettings _cameralenssettings _cameraexposuresettings _postprocesssettings) (break `/Game/BluePrints/Cinematography/struct_CameraPostSetting` (`|GetArrayItem` (`self.masterSceneSettingsArray`) (`self.useScene`))))
  (`SphereComponent.SetSphereRadius` (`self.colSphere`) (`self.collisionSize`) true)
  (set `local.local_Title` _title)
  (set `CineCameraComponent.FocusSettings` _camerafocussettings _mytestcamera)
  (set `CineCameraComponent.LensSettings` _cameralenssettings _mytestcamera)
  (set `CameraComponent.PostProcessSettings` _postprocesssettings _mytestcamera)
  (bind _returnvalue (`AddComponent|NODE_AddTextRenderComponent-0` :`RelativeTransform` (`self.textTitleAdjust`)))
  (bind _output_get (set `local.local_TextRender` _returnvalue))
  (`TextRenderComponent.K2_SetText` _output_get (`KismetTextLibrary.Conv_StringToText` (`local.local_Title`)))
  (`TextRenderComponent.SetWorldSize` (`local.local_TextRender`) (`self.textTitleSize`)))