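; Power line generator Blueprint that builds a wire along a spline in the construction script.
; It divides the X distance from the first point of Wire0 to WireFinalDestination by WireRes, then appends points offset along X by that step.
; A spline mesh component is added and attached for each segment, using neighboring point locations and tangents.
; The event graph and test function are empty.
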(fn `testFunction`)

(fn `UserConstructionScript`
  (locals (local_nextPoint :type "SplinePoint Structure") (local_myPointIndex :type Integer) (local_myMeshDrawIndex :type Integer))
  (bind _local_mymeshdrawindex (`local.local_myMeshDrawIndex`))
  (bind _wire_0 (`self.wire_0`))
  (bind (_location _tangent) (`SplineComponent.GetLocationAndTangentAtSplinePoint` _wire_0 _local_mymeshdrawindex "Local"))
  (bind (_returnvalue_x _returnvalue_y _returnvalue_z) (`KismetMathLibrary.BreakVector` (`SplineComponent.GetLocationAtSplinePoint` (`self.wire_0`) (`local.local_myPointIndex`) "World")))
  (bind _returnvalue (`SplineComponent.GetLocationAtSplinePoint` (`self.wire_0`) 0 "Local"))
  (bind (_location_2 _tangent_2) (`SplineComponent.GetLocationAndTangentAtSplinePoint` _wire_0 (+ _local_mymeshdrawindex 1) "Local"))
  (`|ExecutionSequence`
    (:`then_0`
      (set `self.distanceToNextPoint` (/ (`KismetMathLibrary.Vector_Distance` _returnvalue (`KismetMathLibrary.MakeVector` (.x (`self.wireFinalDestination`)) (.y _returnvalue) (.z _returnvalue))) (`KismetMathLibrary.Conv_IntToDouble` (`self.wireRes`)))))
    (:`then_1`
      (for _index (range 2 (+ (+ (`self.wireRes`) 1) 1))
        (set `local.local_myPointIndex` _index)
        (`SplineComponent.AddSplinePoint` (`self.wire_0`) (`KismetMathLibrary.MakeVector` (+ _returnvalue_x (`self.distanceToNextPoint`)) _returnvalue_y _returnvalue_z) "World" true)))
    (:`then_2`
      (for _index_2 (range (+ (- (`SplineComponent.GetNumberOfSplinePoints` (`self.wire_0`)) 2) 1))
        (set `local.local_myMeshDrawIndex` _index_2)
        (bind _returnvalue_2 (`AddComponent|NODE_AddSplineMeshComponent-0` :`self` self))
        (`SplineMeshComponent.SetStartAndEnd` _returnvalue_2 _location _tangent _location_2 _tangent_2 true)
        (`SceneComponent.K2_AttachToComponent` _returnvalue_2 (`self.wire_0`) "None" "KeepRelative" "KeepRelative" "KeepRelative" true)))))