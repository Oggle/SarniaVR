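; Push button actor that toggles on overlap, swapping material, position and text label, calling state-change dispatchers and playing a sound.
; The construction script applies custom materials, builds labels and, in Simple Looper mode, loads a loop cue from a curated set with BPM-derived timing.
; A button can mark a LinkWith button as slave, sharing an indicator material and driving its loop audio with a computed phrase offset.
; BruteTest auto-toggles it on a repeating delay.
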(event `self.ReceiveBeginPlay`
  (`|ExecutionSequence`
    (:`then_0`
      (if (not (`self.buttonOn`))
        (`AudioComponent.Stop` (`self.tmpAudio`))))
    (:`then_1`
      (if (`self.bruteTest`)
        (`self.toggleButton` :!label _label)
        (`AudioComponent.Play` (`self.buttonStateSound`) 0.0)
        ;[1 0 0] Testing
        (`KismetSystemLibrary.Delay` 3.0)
        (goto _label)))))

(event `self.Button.OnComponentBeginOverlap`
  (params (OverlappedComponent :type "PrimitiveComponent Object Reference") (OtherActor :type "Actor Object Reference") (OtherComp :type "PrimitiveComponent Object Reference") (OtherBodyIndex :type Integer) (bFromSweep :type Boolean) (SweepResult :type "HitResult Structure (by ref)"))
  (`self.toggleButton`)
  (`KismetSystemLibrary.PrintString` "Hello")
  (`AudioComponent.Play` (`self.buttonStateSound`) 0.0))

(fn `getNextPhraseStartSec`
  (returns (nextPhraseStarting :type "Float (double-precision)"))
  (return (* (`self.noteDivision`) (/ (- (`GameplayStatics.GetWorldDeltaSeconds`) (`self.loopPlayStartDelta`)) (`self.loopPerBPMDelta`)))))

(fn `setButtonState`
  (bind _scale (.scale (`self.defButtonTransform`)))
  ;[1 0.02787 0] Toggle all on and off positions based on the custom variables and the incoming state boolean
  (if (`self.buttonOn`)
    (`SceneComponent.K2_SetRelativeTransform` (`self.Button`) (`KismetMathLibrary.MakeTransform` (.location (`self.buttonOnZ`)) (.rotation (`self.buttonOnZ`)) _scale) false false)
    (else
      (`SceneComponent.K2_SetRelativeTransform` (`self.Button`) (`KismetMathLibrary.MakeTransform` (.location (`self.buttonOffZ`)) (.rotation (`self.defButtonTransform`)) _scale) false false))))

(fn `setLinkedAudio`
  (params (doStop :type Boolean) (doPlay :type Boolean))
  (bind _linked_tmpaudio (`self.linked_tmpAudio`))
  (if (`self.validLink`)
    (`|ExecutionSequence`
      (:`then_0`
        (if doStop
          (`AudioComponent.Stop` _linked_tmpaudio)))
      (:`then_1`
        (if doPlay
          (`AudioComponent.Play` _linked_tmpaudio 0.0))))))

(fn `setPlayTimer`
  (set `self.loopPlayStartDelta` (`GameplayStatics.GetWorldDeltaSeconds`)))

(fn `toggleButton`
  (locals (NewLocalVar_0 :type "Array of Integer"))
  (`|ExecutionSequence`
    (:`then_0`
      (if (`self.buttonOn`)
        (set `self.buttonOn` false)
        (`self.buttonStateChangedOff`)
        (`self.toggleMaterial` (`self.Button`) (`self.customButtonMaterial`) (`self.buttonCustomMaterialIndex`) (`self.replaceAllButtonMatIndex`))
        (else
          (set `self.buttonOn` true)
          (`self.buttonStateChangedOn`)
          (`self.toggleMaterial` (`self.Button`) (`self.onButtonMaterial`) (`self.buttonCustomMaterialIndex`) (`self.replaceAllButtonMatIndex`))))
      (`|ExecutionSequence`
        (:`then_0`
          ;[0 0.1184 1] Label Visibility
          (if (`self.showLabel`)
            (`SceneComponent.ToggleVisibility` (`self.tr_OffText`) true)
            (`SceneComponent.ToggleVisibility` (`self.tr_onText`) true)))
        (:`then_1`
          ;[1 0.3605 0] Handle Looper
          (if (`self.simpleLooper`)
            (`self.toggleLoop`)))))
    (:`then_1`
      (`self.setButtonState`))))

(fn `toggleLoop`
  (bind _tmpaudio (`self.tmpAudio`))
  (bind _validlink (`self.validLink`))
  (bind _linked_tmpaudio (`self.linked_tmpAudio`))
  (if (`AudioComponent.IsPlaying` _tmpaudio)
    (`AudioComponent.Stop` _tmpaudio)
    (`AudioComponent.Stop` (`self.tmpAudio`))
    ;[1 0.5522 0] Synchronize Linked Stop and Playback
    (if _validlink
      (`AudioComponent.Stop` _linked_tmpaudio))
    (else
      (`AudioComponent.Play` _tmpaudio 0.0)
      (`AudioComponent.Play` (`self.tmpAudio`) 0.0)
      (if _validlink
        (bind _nextphrasestarting (`self.getNextPhraseStartSec`))
        (`AudioComponent.Play` _linked_tmpaudio _nextphrasestarting)))))

(fn `toggleMaterial`
  (params (thisMeshComponent :type "StaticMeshComponent Object Reference") (thisMaterial :type "MaterialInterface Object Reference") (thisIndex :type Integer) (replaceAll :type Boolean))
  ;[1 0 0.4728 1 14] Replace all meshComponent material\ indindices with material
  (if replaceAll
    ;[1 0.09267 0] Set all material indices with input material
    (for _index (range (+ (`PrimitiveComponent.GetNumMaterials` (`local.thisMeshComponent`)) 1))
      (`PrimitiveComponent.SetMaterial` (`local.thisMeshComponent`) _index (`local.thisMaterial`)))
    (else
      ;[1 0 0.8048] Set the single element to the material
      (`PrimitiveComponent.SetMaterial` (`local.thisMeshComponent`) (`local.thisIndex`) (`local.thisMaterial`)))))

(fn `UserConstructionScript`
  (locals (local_LoopCue :type "SoundCue Object Reference"))
  (bind _button (`self.Button`))
  (bind _showdiagnostic (`self.showDiagnostic`))
  (bind _labeloffsetvector (`self.labelOffsetVector`))
  (bind _button_2 (`self.Button`))
  (bind _buttonon (`self.buttonOn`))
  (bind _linked_tmpaudio (`self.linked_tmpAudio`))
  (bind _linkwith (`self.linkWith`))
  (bind (_min _max) (`StaticMeshComponent.GetLocalBounds` _button))
  (bind _returnvalue (`SceneComponent.K2_GetComponentToWorld` _button))
  (bind _returnvalue_2 (`KismetTextLibrary.Conv_StringToText` (`self.loopDetailLabel`)))
  (bind (_id _loopcue _bpm _instrument _samplekey) (break `/Game/BluePrints/My_Audio_BP/SimpleLooper/Struct_SimpleLoop_Single` (`|GetArrayItem` (`.cueSetArray_5_E274C0A94E284CF80E5A5DA68AB49091` (break `/Game/BluePrints/My_Audio_BP/SimpleLooper/Struct_SimpleLoopSets` (`self.myLooperSets`))) (`self.useLoopSingle`))))
  ;[0.2396 0 0.01177] Diagnostic Overide of label showing
  (if _showdiagnostic
    (set `self.showLabel` _showdiagnostic))
  ;[1 0 0.03588 1 14] Start states and sizes for the buttons
  (set `self.defButtonTransform` _returnvalue)
  ;[1 0.2983 0] Get the default size and material of the button
  (set `self.myButtonSize` (* (- _max _min) (.x (.scale _returnvalue))))
  ;;[0.3422 0.2124 1 1 14] Store default button material at the user set material index, if theres more than one material on the mesh
  (set `self.defButtonMaterial` (`PrimitiveComponent.GetMaterial` (`self.Button`) (`self.buttonCustomMaterialIndex`)))
  (`|ExecutionSequence`
    (:`then_0`
      ;;[0 0.5332 1 1 14] Valid custom button material? if so then use it
      (if (`KismetSystemLibrary.IsValid` (`self.customButtonMaterial`))
        (`self.toggleMaterial` (`self.Button`) (`self.customButtonMaterial`) (`self.buttonCustomMaterialIndex`) (`self.replaceAllButtonMatIndex`))))
    (:`then_1`
      ;;[1 0.7723 0.1455] Custom base material
      (if (`KismetSystemLibrary.IsValid` (`self.customBaseMaterial`))
        (`self.toggleMaterial` (`self.Base`) (`self.customBaseMaterial`) (`self.baseCustomMaterialIndex`) (`self.replaceAllBaseMatIndex`))))
    (:`then_2`
      ;;[0.2012 1 0] Simple Looper
      (if (`self.simpleLooper`)
        ;;;[0.2844 1 0.09399 1 12] Loop default bpm
        (set `self.defLoopBPM` _bpm)
        ;;;[0.7173 0 1 1 14] Create labels from details
        (set `self.loopDetailLabel` (`KismetStringLibrary.Concat_StrStr` (`KismetStringLibrary.Concat_StrStr` _instrument ":") _samplekey))
        ;;;[0.384 0.8076 1 1 14] Make local and public Sound Cue
        (set `local.local_LoopCue` _loopcue)
        (bind _output_get (set `self.myLoopCue` _loopcue))
        ;;;[1 0 0.07331 1 14] Set the sound cue of the component
        (`AudioComponent.SetSound` (`self.tmpAudio`) _output_get)
        ;;;[0 1 0.9218 1 12] Reach into the component cue and get the sound and then its duration
        (bind _output_get_2 (set `self.sampleDuration` (`SoundBase.Duration` (`AudioComponent.Sound` (`self.tmpAudio`)))))
        ;;;[1 0 0.3889 1 12] Duration divided by the loops default BPM from its settings
        (bind _output_get_3 (set `self.loopPerBPMDelta` (/ _output_get_2 (`self.defLoopBPM`))))
        ;;;[1 0.1242 0] For Click Track
        (set `self.bpmDelaDelta` (/ _output_get_3 (`KismetMathLibrary.Conv_IntToDouble` (`self.noteDivision`))))
        ;;;[0 0.6928 1] Volume
        (`AudioComponent.SetVolumeMultiplier` (`self.tmpAudio`) (`self.simpleLoopVol`))
        ;;;[0.603 0.02672 1] Start Playing if button on?
        (if (`self.buttonOn`)
          (if (not (`AudioComponent.IsPlaying` (`self.tmpAudio`)))
            (`AudioComponent.Play` (`self.tmpAudio`) 0.0))
          (else
            (`AudioComponent.Stop` (`self.tmpAudio`))))))
    (:`then_3`
      ;;[1 0.0546 0.3482] Using Labels? Then set them up, rient and set the text
      (if (`self.showLabel`)
        (bind _returnvalue_3 (`AddComponent|NODE_AddTextRenderComponent-0` :`RelativeTransform` (`KismetMathLibrary.MakeTransform` _labeloffsetvector)))
        (set `self.tr_onText` _returnvalue_3)
        (bind _returnvalue_4 (`AddComponent|NODE_AddTextRenderComponent-1` :`RelativeTransform` (`KismetMathLibrary.MakeTransform` _labeloffsetvector)))
        (set `self.tr_OffText` _returnvalue_4)
        (if (`self.useLoopDetailLabel`)
          (`TextRenderComponent.K2_SetText` (`self.tr_onText`) _returnvalue_2)
          (`TextRenderComponent.K2_SetText` (`self.tr_OffText`) _returnvalue_2)
          (else
            (`TextRenderComponent.K2_SetText` (`self.tr_onText`) (`self.labelOn`))
            (`TextRenderComponent.K2_SetText` (`self.tr_OffText`) (`self.labelOff`))))
        (`TextRenderComponent.SetTextRenderColor` (`self.tr_onText`) (`self.labelOnColour`))
        (`TextRenderComponent.SetTextRenderColor` (`self.tr_OffText`) (`self.labelOffColour`))
        (`TextRenderComponent.SetWorldSize` (`self.tr_onText`) (`self.labelTextSize`))
        (`TextRenderComponent.SetWorldSize` (`self.tr_OffText`) (`self.labelTextSize`))
        ;;;[0 0.7005 1] Check buttonOn for visibility
        (`SceneComponent.SetVisibility` (`self.tr_onText`) _buttonon _buttonon)
        (if (`self.buttonOn`)
          (`SceneComponent.SetVisibility` (`self.tr_OffText`) false true))))
    (:`then_4`
      ;;[1 0 0.05021] Set default mesh positions from offsets
      (`SceneComponent.K2_SetRelativeTransform` (`self.Base`) (`self.baseOffsetTransform`) false false)
      (if (`self.buttonOn`)
        (`SceneComponent.K2_SetRelativeTransform` _button_2 (`self.buttonOnZ`) false false)
        (else
          (`SceneComponent.K2_SetRelativeTransform` _button_2 (`self.buttonOffZ`) false false))))
    (:`then_5`
      ;;[0.3394 0 1] Am I a Slave?
      (if (`self.linkSlave`)
        ;;[1 0 0.9405] Setup Links to synchronize playback
        ;;;[1 0 0.4653] Replace My Material
        (bind _output_get_4 (set `self.customBaseMaterial` (`self.linkedMaterial`)))
        (`PrimitiveComponent.SetMaterial` (`self.Base`) (`self.linkedMaterialIndex`) _output_get_4)
        (else
          ;;;[1 0 0 1 12] Good Linked with Button Class
          (set `self.validLink` (`KismetSystemLibrary.IsValid` (`self.linkWith`)))
          ;;;[1 0 0.1736] Put Linked with in Slave mode
          (set `self.linked_tmpAudio` (`/Game/BluePrints/BP_Buttons_Switches/BP_Push_Button.tmpAudio` (`self.linkWith`)))
          (set `/Game/BluePrints/BP_Buttons_Switches/BP_Push_Button.linkSlave` true (`self.linkWith`))
          ;;;[1 0 0 1 14] Set my link indicator material at my custom material index
          (`PrimitiveComponent.SetMaterial` (`self.Base`) (`self.linkedMaterialIndex`) (`self.linkedMaterial`))
          ;;;;[0 0.2297 1 1 14] Set linked button custom material and custom usage
          (set `/Game/BluePrints/BP_Buttons_Switches/BP_Push_Button.linkedMaterial` (`self.linkedMaterial`) _linkwith)
          (set `/Game/BluePrints/BP_Buttons_Switches/BP_Push_Button.linkedMaterialIndex` (`self.linkedMaterialIndex`) _linkwith)
          ;;;[1 0.365 0] Sync On States and playback
          (if (`self.buttonOn`)
            (if (not (`AudioComponent.IsPlaying` _linked_tmpaudio))
              (`AudioComponent.Play` _linked_tmpaudio 0.0))))))))