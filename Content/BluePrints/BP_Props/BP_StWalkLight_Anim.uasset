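; BP_StWalkLight_Anim is a street prop, apparently a walk light, that cycles the text shown on a sign.
; On BeginPlay it sets the ShowSign1 text and render color from parallel text and color arrays at a shared index.
; The index advances and wraps at the end of the text array, and a retriggerable delay loops the sequence on a fixed interval without using Tick.
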(event `self.ReceiveBeginPlay`
  ;[0.247 0.1257 1] Set Sign content text from array
  (`TextRenderComponent.K2_SetText` (`self.showSign_1`) (`KismetTextLibrary.Conv_StringToText` (`|GetArrayItem` (`self.signTxtArray`) (`self.atSignTxt`))) :!label _label)
  ;[0.8726 0.1758 1] Set Text Render Color From Array
  (`TextRenderComponent.SetTextRenderColor` (`self.showSign_1`) (`|GetArrayItem` (`self.txtColorArray`) (`self.atSignTxt`)))
  ;[0.904 0.2572 1] Increment At Content
  (bind _output_get (set `self.atSignTxt` (+ (`self.atSignTxt`) 1)))
  ;[0.1093 0.8399 1] Reset Seq Content if no more content
  (if (>= _output_get (`KismetArrayLibrary.Array_Length` (`self.signTxtArray`)))
    (set `self.atSignTxt` 0))
  (`KismetSystemLibrary.RetriggerableDelay` 12.0)
  (goto _label))

(fn `UserConstructionScript`)