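; VR drum sample pad that plays a velocity-scaled hit when a grabbed drumstick strikes its trigger moving downward.
; The construction script builds it from preset meshes, sound cue, scale, colour, optional materials and a title.
; Overlaps pass a timed gate and stick-state check, then set the cue's sample parameter, fire haptics and briefly flash an emissive material.
; PlayMetronome plays and flashes the pad as a click; kit-grouping logic is unconnected.
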(event `self.ReceiveTick`
  (params (DeltaSeconds :type "Float (single-precision)"))
  (set `self.Delta Seconds` DeltaSeconds))

(event `self.ReceiveBeginPlay`
  ;[0 0.2046 1 1 14] Store original material at emissive int slot of the trigger mesh. This assumes index 0 is the body of the object.
  (set `self.oldTriggerMatterial` (`|GetArrayItem` (`MeshComponent.GetMaterials` (`self.myMesh`)) (`self.emissiveTriggerSlot`))))

(event `self.myTrigger.OnComponentBeginOverlap`
  (params (OverlappedComponent :type "PrimitiveComponent Object Reference") (OtherActor :type "Actor Object Reference") (OtherComp :type "PrimitiveComponent Object Reference") (OtherBodyIndex :type Integer) (bFromSweep :type Boolean) (SweepResult :type "HitResult Structure (by ref)"))
  (bind _local_overlappedstick (`self.local_overlappedStick`))
  ;[0.5677 0.3773 0] Testing just overlap trigger
  (`KismetSystemLibrary.PrintString` "DrumOverlap")
  ;[1 0.03409 0 1 14] GATE CLOSED FROM LAST HIT AND ON A TIMER FROM GATEMIN
  (if (`self.gateOpen`)
    ;[0.05254 0.7687 1 1 14] Store overlap actor at start
    (bind _output_get (set `self.triggerHitByActor` OtherActor :!label _label))
    ;[0.5193 0 1 1 14] Is this a drum stick?
    (if (== (`GameplayStatics.GetObjectClass` _output_get) "/Game/BluePrints/My_Audio_BP/grab_drumstick.grab_drumstick_C")
      ;[0.01289 0.2456 1] Make it one and set the local variable
      (bind _asgrab_drumstick (cast `/Game/BluePrints/My_Audio_BP/grab_drumstick` (`self.triggerHitByActor`)))
      (set `self.local_overlappedStick` _asgrab_drumstick)
      ;;[1 0.1344 0.1742 1 14] Is the stick still overlapped
      (if (`/Game/BluePrints/My_Audio_BP/grab_drumstick.stickOverlapped` _local_overlappedstick)
        ;[1 0.08013 0] No Good
        (`KismetSystemLibrary.PrintString` "Stick is overlapped still")
        (else
          ;[1 0.6776 0] THIS WORKS
          (bind _output_get_2 (set `self.stickOverlapVelocity` (`/Game/BluePrints/My_Audio_BP/grab_drumstick.deltaStickVelVector` _local_overlappedstick)))
          (set `self.overlapVelocityLength` (`KismetMathLibrary.VSize` _output_get_2))
          ;[0.2571 1 0] Trying to prevent retriggers
          ;;[1 0 0.03055] Check for down hit only
          (if (< (.z (`self.stickOverlapVelocity`)) 0.0)
            ;;[1 0.1048 0 1 14] If not then start the overlap sequence
            (`/Game/BluePrints/My_Audio_BP/grab_drumstick.startMyOverlap` (`self.local_overlappedStick`))
            (`KismetSystemLibrary.PrintString` "Overlap Sequence Called playing sample" true false)
            (`|ExecutionSequence`
              (:`then_0`
                ;[0.09801 0.04961 0.1615 1 12] Sample set from use sample int to the cue hit table of switch names with a set modulus vol integer for right now
                (`AudioComponent.SetIntParameter` (`self.DP_SamplePad_Cue`) "dynSampleInt" (`KismetMathLibrary.Round` (* (`self.hitVolModulus`) (/ (`self.overlapVelocityLength`) (`self.velocityInputScalar`)))))
                ;;[0.9427 0 0.4174] Firing Sample
                (`AudioComponent.Play` (`self.DP_SamplePad_Cue`) (`self.fineSampleOffsetStart`))
                (`/Game/VRTemplate/Blueprints/GrabComponent.HapticHit` (`/Game/BluePrints/My_Audio_BP/grab_drumstick.GrabComponent` (`self.local_overlappedStick`)) "/Game/VRTemplate/Haptics/PistolFireHapticEffect.PistolFireHapticEffect")
                (`KismetSystemLibrary.PrintString` "Sample n Haptic Fired" false false)
                (`KismetSystemLibrary.PrintString` (`KismetStringLibrary.Concat_StrStr` (`KismetStringLibrary.Conv_VectorToString` (`self.stickOverlapVelocity`)) (`KismetStringLibrary.Conv_DoubleToString` (`self.overlapVelocityLength`))) false)
                ;;[1 0 0.006772] Close Gate, open on gate min
                (set `self.gateOpen` false)
                (`KismetSystemLibrary.Delay` (`self.gateMin`))
                (set `self.gateOpen` true))
              (:`then_1`
                ;[0.1979 0.1742 0.05463] Light Up material animation
                (if (`self.lightUp`)
                  ;;[1 0.125 0.125] Reset to original then set the emissive
                  (bind _inputoriginalpassthru (`self.flashMaterial` (`self.myTrigger`) (`self.emissiveTriggerSlot`) (`self.oldTriggerMatterial`) (`self.emissiveTriggerSlot`) (`self.emmisiveMaterial`)))
                  ;;[0.2294 1 0] Delay then return to the original material
                  (`KismetSystemLibrary.Delay` (`self.animHitDelay`))
                  (`self.flashMaterial` (`self.myTrigger`) 0 _inputoriginalpassthru (`self.emissiveTriggerSlot`) (`self.emmisiveMaterial`) true))))))))
    (else
      ;[1 0 0.03509] Did Stick Report?
      (if (`self.stickReportedIn`)
        (goto _label)
        (else
          ;[0.2812 0 0.01198 1 12] GATECLOSED
          (set `self.stickReportedIn` false)
          (`KismetSystemLibrary.PrintString` "GateClosed") ; GATE CLOSED
        )))))

(event `self.myTrigger.OnComponentEndOverlap`
  (params (OverlappedComponent :type "PrimitiveComponent Object Reference") (OtherActor :type "Actor Object Reference") (OtherComp :type "PrimitiveComponent Object Reference") (OtherBodyIndex :type Integer))
  ;[1 0.4579 0] Clear Overlap
  (set `self.stickReportedIn` false))

(fn `flashMaterial`
  (params (targetPrimitive :type "PrimitiveComponent Object Reference") (materialIndex :type Integer) (originalMaterial :type "MaterialInterface Object Reference") (emissiveIndex :type Integer) (emissiveMaterial :type "MaterialInterface Object Reference") (flashBack :type Boolean))
  (returns (inputOriginalPassThru :type "MaterialInterface Object Reference"))
  ;[0.1979 0.1742 0.05463] Light Up material animation
  ;;[1 0.125 0.125] Reset to original then set the emissive
  (`PrimitiveComponent.SetMaterial` targetPrimitive materialIndex originalMaterial)
  ;;[0.1627 0.4062 0 1 14] Flash Back? Then stop at restoring original
  (if (not flashBack)
    ;;[1 0 0] Finish Flash Externally
    (`PrimitiveComponent.SetMaterial` targetPrimitive emissiveIndex emissiveMaterial))
  ;[1 0 0.1187 1 14] In the event we are using this with a delay, we pass the original material right through
  (return (`local.originalMaterial`)))

(fn `playMetronome`
  (bind _dp_samplepad_cue (`self.DP_SamplePad_Cue`))
  (`AudioComponent.SetIntParameter` _dp_samplepad_cue "dynSampleInt" 0)
  (`AudioComponent.Play` _dp_samplepad_cue 0.0)
  (`self.flashMaterial` (`self.myMesh`) 0 null (`self.emissiveTriggerSlot`) (`self.emmisiveMaterial`))
  (`KismetSystemLibrary.PrintString` "SPad Played Metro Click"))

(fn `UserConstructionScript`
  (locals (local_myTextRenderTitle :type "TextRenderComponent Object Reference") (local_nextPolyChannel :type "AudioComponent Object Reference") (local_mySampleChannelArray :type "Array of AudioComponent Object Reference") (local_DPKitCheck :type "/Game/BluePrints/My_Audio_BP/DrumPad/BP_SVR_Sample_Pad_V2 Object Reference") (local_nearByKitArray :type "Array of Integer") (nearByDrumPadsArray :type "Array of /Game/BluePrints/My_Audio_BP/DrumPad/BP_SVR_Sample_Pad_V2 Object Reference") (local_dpKitInt :type Integer) (local_triggerTransform :type "Vector Structure"))
  (bind (_drumscale_location _drumscale_rotation _drumscale_scale) (`KismetMathLibrary.BreakTransform` (`self.drumScale`)))
  (bind _local_mytextrendertitle (`local.local_myTextRenderTitle`))
  (bind (_mydp_inst_id _mydp_inst_title _mydp_inst_note _mydp_inst_dp_soundcue) (break `/Game/BluePrints/My_Audio_BP/DrumPad/Structs/DP_Poly_Drum_Inst` (`self.myDP_Inst`)))
  (bind _mymesh (`self.myMesh`))
  (bind (_returnvalue_location _returnvalue_rotation _returnvalue_scale) (`KismetMathLibrary.BreakTransform` (`SceneComponent.GetRelativeTransform` (`self.myTrigger`))))
  (bind (_returnvalue_location_2 _returnvalue_rotation_2 _returnvalue_scale_2) (`KismetMathLibrary.BreakTransform` (`SceneComponent.GetRelativeTransform` (`self.myMesh`))))
  (bind (_r _g _b) (`KismetMathLibrary.BreakColor` (`self.primitiveColour`)))
  (bind (_id _drumstaticmesh _deftriggermesh _noshell _title _author _triggeradjust) (break `/Game/BluePrints/My_Audio_BP/DrumPad/Structs/DP_Mesh_Types` (`|GetArrayItem` (`self.DP_DrumMeshes`) (`self.useDPDrumMesh`))))
  (bind _y (.y (.scale (`self.padTitleOffset`))))
  (bind _x (.x (+ _returnvalue_scale_2 _drumscale_scale)))
  (bind _x_2 (.x (+ _returnvalue_scale _drumscale_scale)))
  ;[1 0 0.0169] CONSTRUCTION
  ;[1 0.3601 0] Array Resets
  (`KismetArrayLibrary.Array_Clear` (`local.local_nearByKitArray`))
  ;[1 0.5376 0.0904] Set Custom Shell and Skins
  (`StaticMeshComponent.SetStaticMesh` (`self.myMesh`) _drumstaticmesh)
  (`StaticMeshComponent.SetStaticMesh` (`self.myTrigger`) _deftriggermesh)
  (set `local.local_triggerTransform` _triggeradjust)
  ;[1 0.06221 0.2526] Set Drum Sound Cue for this Pad
  (`AudioComponent.SetSound` (`self.DP_SamplePad_Cue`) _mydp_inst_dp_soundcue)
  ;[0.9124 0.1697 1] Over complicated scaling of trigger and mesh, need to find a way to keep mesh below trigger at z-half zbound
  (`SceneComponent.K2_SetRelativeTransform` (`self.myMesh`) (`KismetMathLibrary.MakeTransform` _returnvalue_location_2 (struct) (`KismetMathLibrary.MakeVector` _x _x (.z (+ _returnvalue_scale_2 _drumscale_scale)))) false false)
  (`SceneComponent.K2_SetRelativeTransform` (`self.myTrigger`) (`KismetMathLibrary.MakeTransform` (`local.local_triggerTransform`) (struct) (`KismetMathLibrary.MakeVector` _x_2 _x_2)) false false)
  ;[1 0.5344 0] Establish Primitive Colour  Connection
  (`PrimitiveComponent.SetCustomPrimitiveDataFloat` _mymesh 0 0.0)
  (`PrimitiveComponent.SetCustomPrimitiveDataVector3` _mymesh 0 (`KismetMathLibrary.MakeVector` _r _g _b))
  ;[1 0.3866 0 1 14] Store transform of the trigger mesh
  (set `self.triggerMeshTransform` (`SceneComponent.GetRelativeTransform` (`self.myTrigger`)))
  (`|ExecutionSequence`
    (:`then_0`
      ;[1 0 0.2223] Override Materials
      (if (`self.overrideMaterials`)
        (`|ExecutionSequence`
          (:`then_0`
            ;[1 0.1208 0.3216] Set mesh material
            (`PrimitiveComponent.SetMaterial` (`self.myMesh`) 0 (`|GetArrayItem` (`self.meshMaterial`) (`self.useMeshMaterial`))))
          (:`then_1`
            ;[1 0 0.4547] Visible Trigger if so use material
            (if (`self.triggerMeshVisible`)
              (`PrimitiveComponent.SetMaterial` (`self.myTrigger`) 0 (`|GetArrayItem` (`self.meshMaterial`) (`self.useTriggerMaterial`)))
              (else
                (`SceneComponent.SetVisibility` (`self.myTrigger`) false false)))))))
    (:`then_1`
      ;[0.4651 1 0.1096] Show Title Of Sample
      (if (`self.showTitle`)
        (bind _returnvalue (`AddComponent|NODE_AddTextRenderComponent-0`))
        (set `local.local_myTextRenderTitle` _returnvalue)
        (if (`KismetStringLibrary.NotEqual_StrStr` (`self.userDrumTitle`))
          (`TextRenderComponent.K2_SetText` (`local.local_myTextRenderTitle`) (`KismetTextLibrary.Conv_StringToText` (`self.userDrumTitle`)))
          (else
            (`TextRenderComponent.K2_SetText` (`local.local_myTextRenderTitle`) (`KismetTextLibrary.Conv_NameToText` (`KismetStringLibrary.Conv_StringToName` (`.Title_5_B7AB38F14B84A1D75264EB88009C25FD` (break `/Game/BluePrints/My_Audio_BP/DrumPad/Structs/DP_Poly_Drum_Inst` (`self.myDP_Inst`))))))))
        (`TextRenderComponent.SetHorizontalAlignment` (`local.local_myTextRenderTitle`) "EHTA_Center")
        (`SceneComponent.K2_SetRelativeTransform` _local_mytextrendertitle (`KismetMathLibrary.MakeTransform` (.location (`self.padTitleOffset`)) (struct) (`KismetMathLibrary.MakeVector` 1.0 _y _y)) false false)
        (`SceneComponent.K2_SetWorldRotation` _local_mytextrendertitle (.rotation (`self.padTitleOffset`)) false false)))))