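; Mini data screen prop that shows configurable text on a display component which snaps between open and closed transforms.
; The construction script sets the text and size, and calls OpenDisplay when DisplayOpen is set, which toggles it closed.
; OpenDisplay presets the state for its force flags, with open overriding closed, then flips it and applies the relative transform.
; Unconnected leftover nodes would show linked-button group and BPM info.
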(fn `openDisplay`
  (params (forceOpen :type Boolean) (forceClosed :type Boolean))
  ;[0.2865 0 0] Force open overrides close
  (if forceClosed
    (set `self.displayOpen` true))
  (if forceOpen
    ;[0.4246 0.295 1] Allow a forced state change
    (set `self.displayOpen` false))
  (`|ExecutionSequence`
    (:`then_0`
      (if (`self.displayOpen`)
        ;[1 0.1131 0.6083] If open then close it and vice versa
        (set `self.toggleTransform` (`self.closedTransForm`))
        ;;[1 0 0.00876] Toggle opeen/close boolean
        (set `self.displayOpen` false)
        (else
          (set `self.toggleTransform` (`self.openTransform`))
          (set `self.displayOpen` true))))
    (:`then_1`
      ;[1 0 0.04338] Set the position of the display to the toggle final transform
      (`SceneComponent.K2_SetRelativeTransform` (`self.displayScreen`) (`self.toggleTransform`) false false))))

(fn `UserConstructionScript`
  (bind _tmptr (`self.tmpTR`))
  (if (`self.displayOpen`)
    (`self.openDisplay` false))
  (`TextRenderComponent.K2_SetText` _tmptr (`self.myScreenData`))
  (`TextRenderComponent.SetWorldSize` _tmptr (`self.screenTxtSize`)))