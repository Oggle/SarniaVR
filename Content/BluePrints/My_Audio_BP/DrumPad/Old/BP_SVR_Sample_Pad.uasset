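; Sample drum pad actor that plays a random snare-hit variant through a sound cue when another actor overlaps its trigger.
; An array of overlapping actors blocks retriggers until end overlap.
; Hits select a free channel from six but never play it, and record velocity; the GoodHit flag gates an emissive flash, though its setter is disconnected.
; Construction configures scale, colour, materials, channel sound, volume, attenuation and an optional title.
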(event `self.ReceiveBeginPlay`
  ;[0 0.2046 1 1 14] Store original material at emissive int slot of the trigger mesh. This assumes index 0 is the body of the object.
  (set `self.oldTriggerMatterial` (`|GetArrayItem` (`MeshComponent.GetMaterials` (`self.myMesh`)) (`self.emissiveTriggerSlot`))))

(event `self.myTrigger.OnComponentHit`
  (params (HitComponent :type "PrimitiveComponent Object Reference") (OtherActor :type "Actor Object Reference") (OtherComp :type "PrimitiveComponent Object Reference") (NormalImpulse :type "Vector Structure") (Hit :type "HitResult Structure (by ref)"))
  ;[1 0 0.08905] Checking for DrumPad HITS
)

(event `self.myTrigger.OnComponentBeginOverlap`
  (params (OverlappedComponent :type "PrimitiveComponent Object Reference") (OtherActor :type "Actor Object Reference") (OtherComp :type "PrimitiveComponent Object Reference") (OtherBodyIndex :type Integer) (bFromSweep :type Boolean) (SweepResult :type "HitResult Structure (by ref)"))
  (bind _dp_samplepad_cue (`self.DP_SamplePad_Cue`))
  (bind _output (`|GetArrayItem` (`self.mySampleChannelArray`)))
  ;[1 0 0.1118] Testing just overlap
  ;[1 0.008092 0 1 14] Set the other actor overlapped and primitive for physics
  (set `self.triggerByOverlapComponent` OverlappedComponent)
  (set `self.triggerHitByActor` OtherActor)
  ;[0.07777 0.1149 0.3281 1 14] Does the down array contain this actor?
  (if (`KismetArrayLibrary.Array_Contains` (`self.objectDownArray`) (`self.triggerHitByActor`))
    (`KismetSystemLibrary.PrintString` (`KismetStringLibrary.Concat_StrStr` (`KismetSystemLibrary.GetDisplayName` (`self.triggerHitByActor`)) " Still Down"))
    (else
      (`KismetArrayLibrary.Array_Add` (`self.objectDownArray`) (`self.triggerHitByActor`))
      (`KismetSystemLibrary.PrintString` (`KismetStringLibrary.Conv_VectorToString` (`SceneComponent.GetComponentVelocity` (`self.triggerByOverlapComponent`))))
      (`|ExecutionSequence`
        (:`then_0`
          ;[0 0.923 1 1 12] Loop Through ALL Channels
          (for _array_element (`self.mySampleChannelArray`)
            ;[0.1303 1 0.3196] Polyphony Handling
            (if (not (`AudioComponent.IsPlaying` _array_element))
              ;;[0.6977 0 1 1 12] If channel not playing then mark it good, set the variable and set the found open channel variable
              (set `self.currentOpenChannel` _array_element)
              (set `self.foundOpenChannel` true)))
          (if (not (`self.foundOpenChannel`))
            (`AudioComponent.Stop` _output)
            (set `self.currentOpenChannel` _output)))
        (:`then_1`
          ;[1 0 0.02203] Firiing Random Samples
          (`AudioComponent.SetIntParameter` _dp_samplepad_cue "snareHit" (`KismetMathLibrary.RandomInteger` 3))
          (`AudioComponent.Play` _dp_samplepad_cue 0.0))
        (:`then_2`
          ;[0 1 0.08076 1 14] Get other object angular velocity for volume and sample pick purposes
          (bind _output_get (set `self.lastHitVelocity` (`KismetMathLibrary.VSize` (`self.GetVelocity` (`self.triggerHitByActor`)))))
          ;[1 0.01901 0.804] Continuing with material change
          (`KismetSystemLibrary.PrintString` (`KismetStringLibrary.Concat_StrStr` "Hit Velocity" (`KismetStringLibrary.Conv_DoubleToString` _output_get)))
          ;[1 0.1437 0.9059] Light Up material animation
          (if (`self.goodHit`)
            (`KismetSystemLibrary.PrintString` "Good Hit")
            (if (`self.lightUp`)
              ;;[1 0.125 0.125] Reset to original then set the eimissive
              (`PrimitiveComponent.SetMaterial` (`self.myTrigger`) (`self.emissiveTriggerSlot`) (`self.oldTriggerMatterial`))
              (`PrimitiveComponent.SetMaterial` (`self.myTrigger`) (`self.emissiveTriggerSlot`) (`self.emmisiveMaterial`))
              ;;[0.2294 1 0] Delay then return to the original material
              (`KismetSystemLibrary.Delay` (`self.animHitDelay`))
              (`PrimitiveComponent.SetMaterial` (`self.myTrigger`) (`self.emissiveTriggerSlot`) (`self.oldTriggerMatterial`))
              (else
                (set `self.goodHit` false)))))))))

(event `self.myTrigger.OnComponentEndOverlap`
  (params (OverlappedComponent :type "PrimitiveComponent Object Reference") (OtherActor :type "Actor Object Reference") (OtherComp :type "PrimitiveComponent Object Reference") (OtherBodyIndex :type Integer))
  (bind _objectdownarray (`self.objectDownArray`))
  ;[1 0.3506 0 1 14] Using End overlap to clear objects that have already hit us from the array
  ;[1 0.08256 0.2731 1 14] If the actor of the end overlap is in the down array then remove it
  (if (`KismetArrayLibrary.Array_Contains` (`self.objectDownArray`) OtherActor)
    (`KismetArrayLibrary.Array_Remove` _objectdownarray (`KismetArrayLibrary.Array_Find` _objectdownarray OtherActor))))

(fn `UserConstructionScript`
  (locals (local_myTextRenderTitle :type "TextRenderComponent Object Reference") (local_nextPolyChannel :type "AudioComponent Object Reference") (local_mySampleChannelArray :type "Array of AudioComponent Object Reference"))
  (bind (_drumscale_location _drumscale_rotation _drumscale_scale) (`KismetMathLibrary.BreakTransform` (`self.drumScale`)))
  (bind _local_mytextrendertitle (`local.local_myTextRenderTitle`))
  (bind _mysamplechannelarray (`self.mySampleChannelArray`))
  (bind _local_mytextrendertitle_2 (`local.local_myTextRenderTitle`))
  (bind _mymesh (`self.myMesh`))
  (bind (_returnvalue_location _returnvalue_rotation _returnvalue_scale) (`KismetMathLibrary.BreakTransform` (`SceneComponent.GetRelativeTransform` (`self.myTrigger`))))
  (bind (_returnvalue_location_2 _returnvalue_rotation_2 _returnvalue_scale_2) (`KismetMathLibrary.BreakTransform` (`SceneComponent.GetRelativeTransform` (`self.myMesh`))))
  (bind (_r _g _b) (`KismetMathLibrary.BreakColor` (`self.primitiveColour`)))
  (bind _x (.x (+ _returnvalue_scale_2 _drumscale_scale)))
  (bind _x_2 (.x (+ _returnvalue_scale _drumscale_scale)))
  ;[1 0 0.0169] CONSTRUCTION
  (for _array_element (`AudioComponent.InstanceParameters` (`self.DP_SamplePad_Cue`))
    (`KismetSystemLibrary.PrintString` (`KismetStringLibrary.Concat_StrStr` "Cue Parameter :" (`KismetStringLibrary.Conv_NameToString` (break `AudioComponentParam` _array_element)))))
  ;[0 0.2273 1] Setting up the polyphony array
  (`KismetArrayLibrary.Array_Clear` (`self.mySampleChannelArray`))
  (`KismetArrayLibrary.Array_Add` _mysamplechannelarray (`self.mySampleChan1`))
  (`KismetArrayLibrary.Array_Add` _mysamplechannelarray (`self.mySampleChan2`))
  (`KismetArrayLibrary.Array_Add` _mysamplechannelarray (`self.mySampleChan3`))
  (`KismetArrayLibrary.Array_Add` _mysamplechannelarray (`self.mySampleChan4`))
  (`KismetArrayLibrary.Array_Add` _mysamplechannelarray (`self.mySampleChan5`))
  (`KismetArrayLibrary.Array_Add` _mysamplechannelarray (`self.mySampleChan6`))
  ;[0.9124 0.1697 1] Over complicated scaling of trigger and mesh, need to find a way to keep mesh below trigger at z-half zbound
  (`SceneComponent.K2_SetRelativeTransform` (`self.myMesh`) (`KismetMathLibrary.MakeTransform` _returnvalue_location_2 (struct) (`KismetMathLibrary.MakeVector` _x _x (.z (+ _returnvalue_scale_2 _drumscale_scale)))) false false)
  (`SceneComponent.K2_SetRelativeTransform` (`self.myTrigger`) (`KismetMathLibrary.MakeTransform` (0.0 0.0 0.0) (struct) (`KismetMathLibrary.MakeVector` _x_2 _x_2 (.z (+ _returnvalue_scale _drumscale_scale)))) false false)
  ;[0.04365 0.474 1] Set Pad Volume all channels
  (for _array_element_2 (`self.mySampleChannelArray`)
    (`AudioComponent.SetVolumeMultiplier` _array_element_2 (`self.defVol`)))
  ;[1 0.5344 0] Establish Primitive Colour  Connection
  (`PrimitiveComponent.SetCustomPrimitiveDataFloat` _mymesh 0 0.0)
  (`PrimitiveComponent.SetCustomPrimitiveDataVector3` _mymesh 0 (`KismetMathLibrary.MakeVector` _r _g _b))
  ;[0.1419 0 1] Load sound from table based on int
  (for _array_element_3 (`self.mySampleChannelArray`)
    (`AudioComponent.SetSound` _array_element_3 (`|GetArrayItem` (`self.padSoundSamples`) (`self.useSample`)))
    ;;[1 0 0.0641 1 12] Set Custom Attenuation
    (set `AudioComponent.AttenuationSettings` (`self.dp_Attenuation`) _array_element_3))
  ;[1 0.3866 0 1 14] Store transform of the trigger mesh
  (set `self.triggerMeshTransform` (`SceneComponent.GetRelativeTransform` (`self.myTrigger`)))
  (`|ExecutionSequence`
    (:`then_0`
      ;[1 0 0.2223] Override Materials
      (if (`self.overrideMaterials`)
        (`|ExecutionSequence`
          (:`then_0`
            ;[1 0.1208 0.3216] Set mesh material
            (`PrimitiveComponent.SetMaterial` (`self.myMesh`) 0 (`|GetArrayItem` (`self.meshMaterial`) (`self.useMeshMaterial`))))
          (:`then_1`
            ;[1 0 0.4547] Visible Trigger if so use material
            (if (`self.triggerMeshVisible`)
              (`PrimitiveComponent.SetMaterial` (`self.myTrigger`) 0 (`|GetArrayItem` (`self.meshMaterial`) (`self.useTriggerMaterial`)))
              (else
                (`SceneComponent.SetVisibility` (`self.myTrigger`) false false)))))))
    (:`then_1`
      ;[0.4651 1 0.1096] Show Title Of Sample
      (if (`self.showTitle`)
        (bind _returnvalue (`AddComponent|NODE_AddTextRenderComponent-0`))
        (set `local.local_myTextRenderTitle` _returnvalue)
        (if (`KismetStringLibrary.NotEqual_StrStr` (`self.userDrumTitle`))
          (`TextRenderComponent.K2_SetText` _local_mytextrendertitle_2 (`KismetTextLibrary.Conv_StringToText` (`self.userDrumTitle`)))
          (else
            (`TextRenderComponent.K2_SetText` _local_mytextrendertitle_2 (`KismetTextLibrary.Conv_StringToText` (`KismetSystemLibrary.GetObjectName` (`|GetArrayItem` (`self.padSoundSamples`) (`self.useSample`)))))))
        (`TextRenderComponent.SetHorizontalAlignment` (`local.local_myTextRenderTitle`) "EHTA_Center")
        (`SceneComponent.K2_SetRelativeTransform` _local_mytextrendertitle (`KismetMathLibrary.MakeTransform` (.location (`self.padTitleOffset`)) (struct) (.scale (`self.padTitleOffset`))) false false)
        (`SceneComponent.K2_SetWorldRotation` _local_mytextrendertitle (struct :`Yaw` -90.0) false false)))))