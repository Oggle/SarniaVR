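; Ping pong ball actor that returns to its start location when it strays too far from its table or falls too low.
; The construction script caches the start location and passes the ball colour to the mesh as custom primitive data.
; Tick checks distance to the referenced table top and world Z against limits, setting a reset flag that moves the ball back.
; The component hit event is an empty stub.
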(event `self.ReceiveTick`
  (params (DeltaSeconds :type "Float (single-precision)"))
  (bind _returnvalue (`self.K2_GetActorLocation` self))
  (set `self.Delta Seconds` DeltaSeconds)
  (`|ExecutionSequence`
    (:`then_0`
      ;[0.461 0 1] Too far from table
      (if (> (`KismetMathLibrary.Vector_Distance` _returnvalue (`SceneComponent.K2_GetComponentLocation` (`/Game/BluePrints/BP_PingPong/BP_PingPong_Game.V1_PPTPlayTopFull` (`self.myPPTable`)))) (`self.ballResetDistance`))
        (set `self.resetBall` true)))
    (:`then_1`
      ;[1 0 0.3905] Too Far Below Table
      (if (< (.z _returnvalue) (`self.ballResetZOffset`))
        (set `self.resetBall` true)))
    (:`then_2`
      ;[0.5213 1 0.06244] Reset Ball
      (if (`self.resetBall`)
        (`self.K2_SetActorLocation` (`self.ballOriginLocation`))
        (set `self.resetBall` false)))))

(event `self.PingPong_Exp_Set_V1_PPTBall_V1.OnComponentHit`
  (params (HitComponent :type "PrimitiveComponent Object Reference") (OtherActor :type "Actor Object Reference") (OtherComp :type "PrimitiveComponent Object Reference") (NormalImpulse :type "Vector Structure") (Hit :type "HitResult Structure (by ref)")))

(fn `UserConstructionScript`
  (locals (local_ballOrigLocation :type "Vector Structure" :default (0.0 0.0 0.0)))
  (bind (_ballcolourdef_r _ballcolourdef_g _ballcolourdef_b _ballcolourdef_a) (break `LinearColor` (`self.ballColourDef`)))
  (set `self.ballOriginLocation` (`self.K2_GetActorLocation` self))
  (`PrimitiveComponent.SetCustomPrimitiveDataVector4` (`self.PingPong_Exp_Set_V1_PPTBall_V1`) 0 (`KismetMathLibrary.MakeVector4` _ballcolourdef_r _ballcolourdef_g _ballcolourdef_b _ballcolourdef_a)))