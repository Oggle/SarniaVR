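; Spline-driven road/track generator actor that builds deformed mesh segments along the Road spline in the Construction Script.
; It stores the point count, resizes RoadDataArray to match, then adds one spline mesh per pair of consecutive points, leaving the loop unclosed.
; Per-point data drives each segment's width, thickness and bank roll at both ends.
; An older even-length/stretch builder remains disconnected.
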(fn `buildTrackElement`
  (params (loopIndex :type Integer) (trackElementMesh :type "StaticMesh Object Reference"))
  (locals (local_currentLoopIndex :type Integer) (local_nextLoopIndex :type Integer) (local_TrackElementMesh :type "StaticMesh Object Reference") (local_startLocation :type "Vector Structure") (local_startTangent :type "Vector Structure") (local_endLocation :type "Vector Structure") (local_endTangent :type "Vector Structure") (local_CurrentSplineMesh :type "SplineMeshComponent Object Reference") (local_startRoll :type "Float (double-precision)") (local_trackWidth :type "Float (double-precision)") (local_trackThickness :type "Float (double-precision)") (local_startScale :type "Vector2D Structure") (local_endRoll :type "Float (double-precision)") (local_endScale :type "Vector2D Structure"))
  (bind _local_currentsplinemesh (`local.local_CurrentSplineMesh`))
  (bind _local_currentsplinemesh_2 (`local.local_CurrentSplineMesh`))
  (bind (_location _tangent) (`SplineComponent.GetLocationAndTangentAtSplinePoint` (`self.Road`) (`local.local_nextLoopIndex`) "Local"))
  (bind (_location_2 _tangent_2) (`SplineComponent.GetLocationAndTangentAtSplinePoint` (`self.Road`) (`local.local_currentLoopIndex`) "Local"))
  (bind (_output_leftguardrail _output_rightguardrail _output_trackbank _output_trackwidth _output_trackthickness) (break `/Game/BluePrints/RoadSplines/Data/RoadData` (`|GetArrayItem` (`self.RoadDataArray`) (`local.local_nextLoopIndex`))))
  (bind (_output_leftguardrail_2 _output_rightguardrail_2 _output_trackbank_2 _output_trackwidth_2 _output_trackthickness_2) (break `/Game/BluePrints/RoadSplines/Data/RoadData` (`|GetArrayItem` (`self.RoadDataArray`) (`local.local_currentLoopIndex`))))
  (bind _output_get (set `local.local_currentLoopIndex` loopIndex))
  (set `local.local_nextLoopIndex` (mod (+ _output_get 1) (`self.numberOfSplinePoints`)))
  (set `local.local_TrackElementMesh` trackElementMesh)
  (`|ExecutionSequence`
    (:`then_0`
      (set `local.local_startLocation` _location_2)
      (set `local.local_startTangent` _tangent_2)
      (set `local.local_endLocation` _location)
      (set `local.local_endTangent` _tangent)
      (set `local.local_startScale` (`KismetMathLibrary.MakeVector2D` _output_trackwidth_2 _output_trackthickness_2))
      (set `local.local_startRoll` _output_trackbank_2)
      (set `local.local_endScale` (`KismetMathLibrary.MakeVector2D` _output_trackwidth _output_trackthickness))
      (set `local.local_endRoll` _output_trackbank))
    (:`then_1`
      (bind _returnvalue (`AddComponent|NODE_AddSplineMeshComponent-3`))
      (bind _output_get_2 (set `local.local_CurrentSplineMesh` _returnvalue))
      (`StaticMeshComponent.SetStaticMesh` _output_get_2 (`local.local_TrackElementMesh`))
      (`SplineMeshComponent.SetStartAndEnd` (`local.local_CurrentSplineMesh`) (`local.local_startLocation`) (`local.local_startTangent`) (`local.local_endLocation`) (`local.local_endTangent`) true)
      (`SplineMeshComponent.SetStartRoll` _local_currentsplinemesh (`local.local_startRoll`) true)
      (`SplineMeshComponent.SetEndRoll` _local_currentsplinemesh (`local.local_endRoll`) true)
      (`SplineMeshComponent.SetStartScale` _local_currentsplinemesh_2 (`local.local_startScale`) true)
      (`SplineMeshComponent.SetEndScale` _local_currentsplinemesh_2 (`local.local_endScale`) true))))

(fn `UserConstructionScript`
  (bind _roaddataarray (`self.RoadDataArray`))
  ;[0.8325 1 0.2617] From Video Task List
  (`|ExecutionSequence`
    (:`then_0`
      (set `self.numberOfSplinePoints` (`SplineComponent.GetNumberOfSplinePoints` (`self.Road`))))
    (:`then_1`
      (`/Engine/EditorBlueprintResources/StandardMacros.CompareInt` (`KismetArrayLibrary.Array_Length` (`self.RoadDataArray`)) (`self.numberOfSplinePoints`) :!label _label
        (:`>`
          (`KismetArrayLibrary.Array_Remove` _roaddataarray (`KismetArrayLibrary.Array_LastIndex` _roaddataarray))
          (goto _label))
        (:`<`
          (`KismetArrayLibrary.Array_Add` (`self.RoadDataArray`))
          (goto _label))))
    (:`then_2`
      (for _index (range (+ (- (`self.numberOfSplinePoints`) 2) 1))
        (`self.buildTrackElement` _index (`self.Track Element Mesh`))))
    (:`then_3`)))