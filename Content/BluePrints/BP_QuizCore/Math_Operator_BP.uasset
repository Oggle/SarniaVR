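; Math operator actor for the quiz game that homes toward the player and destroys itself on contact.
; The construction script picks its mesh and material from arrays by the selected operator and material, then applies a configurable relative transform.
; Tick moves the actor along the vector from its mesh to the player pawn, scaled by a speed factor, so it slows as it nears.
; Overlapping the player only prints a debug message before destruction.
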(event `self.ReceiveTick`
  (params (DeltaSeconds :type "Float (single-precision)"))
  (bind _output_get (set `self.Delta Seconds` DeltaSeconds))
  (`self.K2_AddActorWorldOffset` (* (* (- (`self.K2_GetActorLocation` (`GameplayStatics.GetPlayerPawn` 0)) (`SceneComponent.K2_GetComponentLocation` (`self.opMesh`))) (`self.towardPlayerDeltaScalar`)) _output_get)))

(event `self.ReceiveActorBeginOverlap`
  (params (OtherActor :type "Actor Object Reference"))
  (if (== OtherActor (`GameplayStatics.GetPlayerPawn` 0))
    (`KismetSystemLibrary.PrintString` "Hit Player")
    (`self.K2_DestroyActor` self)))

(fn `UserConstructionScript`
  (`StaticMeshComponent.SetStaticMesh` (`self.opMesh`) (`|GetArrayItem` (`self.operatorMeshArray`) (`self.myOperator`)))
  (`PrimitiveComponent.SetMaterial` (`self.opMesh`) 0 (`|GetArrayItem` (`self.opMaterials`) (`self.myOptMaterial`)))
  (`SceneComponent.K2_SetRelativeTransform` (`self.opMesh`) (`self.opMeshTransform`) false false))