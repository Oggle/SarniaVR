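; Grabbable key actor that moves and rotates a drum sample pad it touches.
; Overlapping a BP_SVR_Sample_Pad_V2 stores the key mesh's starting transform and enables moving until the GrabComponent reports a drop.
; While moving, Tick adds the key's offset from that start, scaled by delta time, to the pad's world transform each frame, so displacement acts like a joystick-style velocity, with yaw halved for softer turning.
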(event `self.GrabComponent.OnDropped`
  ;[1 0.2032 0.07339] Dropped Key End Overlap
  (set `self.moveDrum` false))

(event `self.ReceiveActorBeginOverlap`
  (params (OtherActor :type "Actor Object Reference"))
  ;[1 0.02322 0.1429] EVENT OVERLAP : Check who it is and prepare start transforms for a drum move
  (bind _output_get (set `self.Other Actor` OtherActor))
  (if (== (`GameplayStatics.GetObjectClass` _output_get) "/Game/BluePrints/My_Audio_BP/DrumPad/BP_SVR_Sample_Pad_V2.BP_SVR_Sample_Pad_V2_C")
    (set `self.otherActorTransform` (`self.GetTransform` (`self.Other Actor`)))
    (set `self.controlTransform` (struct))
    (set `self.keyStartTransform` (`SceneComponent.K2_GetComponentToWorld` (`self.StaticMesh`)))
    (set `self.moveDrum` true)
    (`KismetSystemLibrary.PrintString` "DrumPadFound")))

(event `self.ReceiveTick`
  (params (DeltaSeconds :type "Float (single-precision)"))
  (bind _mydeltaseconds (`self.myDeltaSeconds`))
  ;[1 0.01036 0.02031] EVENT TICK : Can We Move
  (set `self.myDeltaSeconds` DeltaSeconds)
  (if (`self.moveDrum`)
    ;[0.124 1 0.9602] Subtract Current Location From Old Start overlap location and transfer changes to the drum
    ;;[1 0 0.01354] Apply Changes to control transform then pass to other actor
    (bind _output_get (set `self.controlTransform` (`KismetMathLibrary.MakeTransform` (* (- (.location (`self.GetTransform`)) (.location (`self.keyStartTransform`))) _mydeltaseconds) (* (`KismetMathLibrary.MakeRotator` (- (.roll (.rotation (`self.GetTransform`))) (.roll (.rotation (`self.keyStartTransform`)))) (- (.pitch (.rotation (`self.GetTransform`))) (.pitch (.rotation (`self.keyStartTransform`)))) (/ (- (.yaw (.rotation (`self.GetTransform`))) (.yaw (.rotation (`self.keyStartTransform`)))) 2.0)) _mydeltaseconds))))
    (`self.K2_AddActorWorldTransform` (`self.Other Actor`) (`KismetMathLibrary.MakeTransform` (.location _output_get) (.rotation _output_get)) false false)))

(fn `UserConstructionScript`)