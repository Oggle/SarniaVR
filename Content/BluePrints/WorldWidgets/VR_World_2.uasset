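; VR world-widget Blueprint pairing an icon mesh with a menu widget, apparently work in progress with placeholder text.
; Its construction script adds a widget component and constructs a DP_Pad_Menu, but never assigns it to that component.
; An indexed MyWidgetIcons entry supplies the icon's mesh, material and color, the latter passed through Custom Primitive Data.
; Start-visibility logic and widget-class lookup are disconnected, and the event graph is empty.
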(fn `UserConstructionScript`
  (locals (local_myWidget :type "UserWidget Object Reference") (local_addedWidgetDyn :type "WidgetComponent Object Reference") (local_widgetMenu :type "/Game/BluePrints/WorldWidgets/DP_Pad_Menu Object Reference") (local_DynWidget :type "/Game/BluePrints/WorldWidgets/DP_Pad_Menu Object Reference") (local_myIcon :type "/Game/BluePrints/WorldWidgets/widgetIcons Structure"))
  (bind (_local_myicon_id _local_myicon_title _local_myicon_type _local_myicon_iconmesh _local_myicon_iconcolor _local_myicon_iconmaterial) (break `/Game/BluePrints/WorldWidgets/widgetIcons` (`local.local_myIcon`)))
  ;[0.1143 1 0.9801] Add Widget Component
  (bind _returnvalue (`AddComponent|NODE_AddWidgetComponent-1`))
  (bind _returnvalue_2 (`|GenericCreateObject` "/Game/BluePrints/WorldWidgets/DP_Pad_Menu.DP_Pad_Menu_C" _returnvalue (`self.showText`)))
  (set `/Game/BluePrints/WorldWidgets/DP_Pad_Menu.myShowText` "sdggdgzfghfadgge" _returnvalue_2)
  (bind _output_get (set `local.local_DynWidget` _returnvalue_2))
  (set `/Game/BluePrints/WorldWidgets/DP_Pad_Menu.myShowText` "Fuckoff" _output_get)
  ;[0 0.8423 1] Set the custom static mesh
  (bind _output_get_2 (set `local.local_myIcon` (`|GetArrayItem` (`self.myWidgetIcons`) (`self.useMesh`))))
  (bind (_id _title _type _iconmesh _iconcolor) (break `/Game/BluePrints/WorldWidgets/widgetIcons` _output_get_2))
  (`StaticMeshComponent.SetStaticMesh` (`self.Iconmesh`) _iconmesh)
  (bind (_r _g _b _a) (`KismetMathLibrary.BreakColor` _iconcolor))
  ;[0.2356 0 1 1 14] Inject 4Vec Colour and tiling data for materials that support a primitive mesh colour
  (`PrimitiveComponent.SetCustomPrimitiveDataVector4` (`self.Iconmesh`) 0 (`KismetMathLibrary.MakeVector4` _r _g _b _a))
  ;[0.3356 1 0.05203] Set custom material
  (`PrimitiveComponent.SetMaterial` (`self.Iconmesh`) 0 _local_myicon_iconmaterial))