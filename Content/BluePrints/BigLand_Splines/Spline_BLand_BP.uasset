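; Spline road Blueprint that builds a track in the construction script, with one spline mesh per segment between Road spline points.
; RoadDataArray is resized to the point count and supplies each segment's mesh, bank roll and width scale, blended toward the next point.
; Tangents are clamped, and custom primitive data carries colour for dynamic materials.
; Toggles control collision, point-number labels and a one-shot copy of the default mesh to all entries.
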(fn `copyDefaultMeshToAll`
  (params (thisStaticMesh :type "StaticMesh Object Reference"))
  (locals (local_tempRoadData :type "/Game/BluePrints/RoadSplines/Data/RoadData Structure") (local_roadArrayIndex :type Integer))
  (for (_array_element _array_index) (`self.RoadDataArray`)
    (set `local.local_roadArrayIndex` _array_index)
    (bind (_leftguardrail _rightguardrail _trackbank _trackwidth _trackthickness) (break `/Game/BluePrints/RoadSplines/Data/RoadData` _array_element))
    (bind _output_get (set `local.local_tempRoadData` (make `/Game/BluePrints/RoadSplines/Data/RoadData` _leftguardrail _rightguardrail _trackbank _trackwidth _trackthickness (`local.thisStaticMesh`))))
    (`KismetArrayLibrary.Array_Set` (`self.RoadDataArray`) (`local.local_roadArrayIndex`) (make `/Game/BluePrints/RoadSplines/Data/RoadData` (break `/Game/BluePrints/RoadSplines/Data/RoadData` _output_get) (`.RightGuardRail_22_7A09DE3242EDB49D4BDE1D8FF31FF632` (break `/Game/BluePrints/RoadSplines/Data/RoadData` _output_get)) (`.TrackBank_23_1862C6CD423F930A72BD8BB1D4291D26` (break `/Game/BluePrints/RoadSplines/Data/RoadData` _output_get)) (`.TrackWidth_24_E2D385CD4B9D92ADE74ECFB078427BD7` (break `/Game/BluePrints/RoadSplines/Data/RoadData` _output_get)) (`.TrackThickness_25_02C1AD924D571EED691E6BAAD93B0297` (break `/Game/BluePrints/RoadSplines/Data/RoadData` _output_get)) (`.TrackType_28_9DD777BD46716FB6B95771A328938E60` (break `/Game/BluePrints/RoadSplines/Data/RoadData` _output_get)))))
  (`KismetSystemLibrary.PrintString` "Default Track Applied"))

(fn `getMeshTransform`
  (locals (local_thisActor :type "StaticMesh Object Reference") (local_actor_transform :type "Transform Structure")))

(fn `UserConstructionScript`
  (locals (mySplineMesh :type "SplineMeshComponent Object Reference") (myArrayIndex :type Integer) (local_TrackElementMesh :type "StaticMesh Object Reference" :default "StaticMesh'/Game/BluePrints/RoadSplines/Meshes/Pier_Open_3x5m.Pier_Open_3x5m'") (local_CurrentSplineMesh :type "SplineMeshComponent Object Reference") (local_arrayMesh :type "StaticMesh Object Reference") (local_meshFromArray :type "StaticMesh Object Reference"))
  (bind _roaddataarray (`self.RoadDataArray`))
  (bind _road (`self.Road`))
  (bind _maxtangent (`self.maxTangent`))
  (bind _mintangent (`self.minTangent`))
  (bind (_myprimitivecolour_r _myprimitivecolour_g _myprimitivecolour_b) (break `LinearColor` (`self.myPrimitiveColour`)))
  (bind _myarrayindex (`local.myArrayIndex`))
  (bind (_location _tangent) (`SplineComponent.GetLocationAndTangentAtSplinePoint` _road _myarrayindex "Local"))
  (bind (_output_leftguardrail _output_rightguardrail _output_trackbank _output_trackwidth _output_trackthickness _output_tracktype) (break `/Game/BluePrints/RoadSplines/Data/RoadData` (`|GetArrayItem` (`self.RoadDataArray`) (`local.myArrayIndex`))))
  (bind (_output_leftguardrail_2 _output_rightguardrail_2 _output_trackbank_2 _output_trackwidth_2) (break `/Game/BluePrints/RoadSplines/Data/RoadData` (`|GetArrayItem` (`self.RoadDataArray`) (`local.myArrayIndex`))))
  (bind (_location_2 _tangent_2) (`SplineComponent.GetLocationAndTangentAtSplinePoint` _road (+ _myarrayindex 1) "Local"))
  (bind (_output_leftguardrail_3 _output_rightguardrail_3 _output_trackbank_3 _output_trackwidth_3) (break `/Game/BluePrints/RoadSplines/Data/RoadData` (`|GetArrayItem` (`self.RoadDataArray`) (+ (`local.myArrayIndex`) 1))))
  (`|ExecutionSequence`
    (:`then_0`
      ;[0.3747 0.9801 1] Get Number of Spline Points
      (set `self.numberOfSplinePoints` (`SplineComponent.GetNumberOfSplinePoints` (`self.Road`))))
    (:`then_1`
      (`/Engine/EditorBlueprintResources/StandardMacros.CompareInt` (`KismetArrayLibrary.Array_Length` (`self.RoadDataArray`)) (`self.numberOfSplinePoints`) :!label _label
        (:`>`
          (`KismetArrayLibrary.Array_Remove` _roaddataarray (`KismetArrayLibrary.Array_LastIndex` _roaddataarray))
          (goto _label))
        (:`<`
          (`KismetArrayLibrary.Array_Add` (`self.RoadDataArray`))
          (goto _label))))
    (:`then_2`
      ;[1 0.8767 0.027] Set the Default Mesh From Set
      (set `local.local_TrackElementMesh` (`|GetArrayItem` (`self.roadMeshSet`) (`self.choseSet`)))
      ;[1 0.1123 0 1 10] Make Room in Road Data Array for Custom transformations
      (for _index (range (+ (- (`self.numberOfSplinePoints`) 2) 1))
        (set `local.myArrayIndex` _index)
        ;[1 0.02034 0.05018] Add a spline Mesh Component
        (bind _returnvalue (`AddComponent|NODE_AddSplineMeshComponent-0`))
        (bind _output_get (set `local.mySplineMesh` _returnvalue))
        (if (`self.collisionOn`)
          (`PrimitiveComponent.SetCollisionEnabled` _output_get "QueryAndPhysics")
          (`PrimitiveComponent.SetCollisionEnabled` (`local.mySplineMesh`) "QueryAndPhysics")
          (else
            (`PrimitiveComponent.SetCollisionEnabled` (`local.mySplineMesh`) "NoCollision")))
        ;[0.2026 0.5578 1] Assign User mesh to spline mesh
        (if (`self.copyToAll`)
          (`self.copyDefaultMeshToAll` (`self.Default Element Mesh`))
          (set `self.copyToAll` false))
        (bind _output_get_2 (set `local.local_meshFromArray` _output_tracktype))
        (`StaticMeshComponent.SetStaticMesh` (`local.mySplineMesh`) _output_get_2)
        ;[1 0.01415 0.6478] Get mesh size for non stretch operations
        (bind _output_get_3 (set `local.local_arrayMesh` _output_tracktype))
        (bind (_returnvalue_min _returnvalue_max) (break `Box` (`StaticMesh.GetBoundingBox` _output_get_3)))
        (set `self.staticMeshTransform` (`KismetMathLibrary.MakeTransform` (0.0 0.0 0.0) (struct) (- _returnvalue_max _returnvalue_min)))
        ;[0.02805 0.03625 0.1615] For Dynamic material colouring from primitive data
        (`PrimitiveComponent.SetCustomPrimitiveDataFloat` (`local.mySplineMesh`) 4 1.0)
        (`PrimitiveComponent.SetCustomPrimitiveDataVector3` (`local.mySplineMesh`) 0 (`KismetMathLibrary.MakeVector` _myprimitivecolour_r _myprimitivecolour_g _myprimitivecolour_b))
        ;[1 0.9359 0.09279 1 14] Set Start and End Spline Mesh Positions and Tangents for Each based on the start of the next position as the end for this one
        (`SplineMeshComponent.SetStartAndEnd` (`local.mySplineMesh`) _location (`KismetMathLibrary.ClampVectorSize` _tangent _mintangent _maxtangent) _location_2 (`KismetMathLibrary.ClampVectorSize` _tangent_2 _mintangent _maxtangent) true)
        ;[0.2722 0.8901 1] Start Roll n Scale
        (`SplineMeshComponent.SetStartRoll` (`local.mySplineMesh`) _output_trackbank_2 true)
        ;[1 0.2904 0.7663] End Roll n Scale
        (`SplineMeshComponent.SetEndRoll` (`local.mySplineMesh`) _output_trackbank_3 true)
        (`SplineMeshComponent.SetStartScale` (`local.mySplineMesh`) (`KismetMathLibrary.MakeVector2D` _output_trackwidth_2 1.0) true)
        (`SplineMeshComponent.SetEndScale` (`local.mySplineMesh`) (`KismetMathLibrary.MakeVector2D` _output_trackwidth_3 1.0) true)
        ;[1 0.298 0.1277] Draw Point Numbers
        (if (`self.showNumbers`)
          (for _index_2 (range (`SplineComponent.GetNumberOfSplinePoints` (`self.Road`)))
            (bind _returnvalue_2 (`AddComponent|NODE_AddTextRenderComponent-0` :`RelativeTransform` (`KismetMathLibrary.MakeTransform` (`SplineComponent.GetLocationAtSplinePoint` (`self.Road`) _index_2 "Local") (struct) (5.0 5.0 5.0))))
            (`TextRenderComponent.K2_SetText` _returnvalue_2 (`KismetTextLibrary.Conv_IntToText` _index_2))))))))