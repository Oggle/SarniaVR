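; A sit spot actor that seats the player in the drumming activity when their pawn enters its SitSetter sphere.
; On overlap it sets the SarniaVRThirdPerson pawn's ActivityMode and snaps it to the sphere's XY and rotation, keeping its Z.
; The construction script applies configurable sphere radius and location offset.
; InUse blocks re-triggering once seated; the end-overlap reset is disconnected, so it is never cleared here.
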(event `self.sitSetter.OnComponentBeginOverlap`
  (params (OverlappedComponent :type "PrimitiveComponent Object Reference") (OtherActor :type "Actor Object Reference") (OtherComp :type "PrimitiveComponent Object Reference") (OtherBodyIndex :type Integer) (bFromSweep :type Boolean) (SweepResult :type "HitResult Structure (by ref)"))
  (bind _returnvalue (`GameplayStatics.GetPlayerPawn` 0))
  (bind _local_otheractor (`self.local_otherActor`))
  (bind (_returnvalue_x _returnvalue_y _returnvalue_z) (`KismetMathLibrary.BreakVector` (`self.K2_GetActorLocation` _local_otheractor)))
  (bind _returnvalue_2 (`SceneComponent.K2_GetComponentToWorld` (`self.sitSetter`)))
  (if (not (`self.inUse`))
    (set `self.local_otherActor` OtherActor)
    (`KismetSystemLibrary.PrintString` "SIT")
    (if (== (`self.local_otherActor`) _returnvalue)
      (bind _assarnia_vrthird_person (cast `/Game/GameReady/SarniaVRThirdPerson` _returnvalue))
      (if (!= (`/Game/GameReady/SarniaVRThirdPerson.activityMode` _assarnia_vrthird_person) 1)
        ;[0.04598 0.07154 1] Drumming Activity
        (set `/Game/GameReady/SarniaVRThirdPerson.activityMode` 1 _assarnia_vrthird_person)
        (`self.K2_SetActorLocationAndRotation` _local_otheractor (`KismetMathLibrary.MakeVector` (.x (.location _returnvalue_2)) (.y (.location _returnvalue_2)) _returnvalue_z) (.rotation _returnvalue_2) false false)
        (set `self.inUse` true)))))

(event `self.sitSetter.OnComponentEndOverlap`
  (params (OverlappedComponent :type "PrimitiveComponent Object Reference") (OtherActor :type "Actor Object Reference") (OtherComp :type "PrimitiveComponent Object Reference") (OtherBodyIndex :type Integer)))

(fn `UserConstructionScript`
  (bind _sitsetteroffset_location (`KismetMathLibrary.BreakTransform` (`self.sitSetterOffset`)))
  (`SphereComponent.SetSphereRadius` (`self.sitSetter`) (`self.sitSetRadius`) true)
  (`SceneComponent.K2_AddLocalTransform` (`self.sitSetter`) (`KismetMathLibrary.MakeTransform` _sitsetteroffset_location) false false))