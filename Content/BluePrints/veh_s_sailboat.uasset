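; Sailboat vehicle Blueprint that, when CanDrive is set, starts one slow eased glide of its Bus component at BeginPlay.
; A single MoveComponentTo runs over a very long duration, using the actor's world X and Y as the component's relative target.
; An unconnected waypoint-array direction calculation remains in the graph, and overlap, tick and construction logic are empty.
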(event `self.ReceiveBeginPlay`
  (bind (_returnvalue_x _returnvalue_y) (`KismetMathLibrary.BreakVector` (`self.K2_GetActorLocation`)))
  (if (`self.canDrive`)
    (`KismetSystemLibrary.MoveComponentTo` (`self.Bus`) (`KismetMathLibrary.MakeVector` _returnvalue_x _returnvalue_y) (struct) true true 2000.0)))

(fn `UserConstructionScript`)