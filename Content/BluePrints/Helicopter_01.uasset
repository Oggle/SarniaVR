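; Helicopter actor that, while CanFly is set, spins its rotors and flies toward a destination.
; Tick adds local yaw to the main and tail rotors from one shared RotorSpeed, scaled by delta time.
; It also calls a latent MoveComponentTo every frame, moving the root over a long fixed duration to the DestLoc entry at AtDest while keeping current altitude.
; Nothing in this Blueprint sets CanFly or advances AtDest.
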(event `self.ReceiveTick`
  (params (DeltaSeconds :type "Float (single-precision)"))
  (bind (_returnvalue_x _returnvalue_y _returnvalue_z) (`KismetMathLibrary.BreakVector` (`self.K2_GetActorLocation`)))
  (bind _returnvalue (* DeltaSeconds (`self.rotorSpeed`)))
  ;[1 0.1519 0] Event Tick Rotate
  (if (`self.canFly`)
    (`SceneComponent.K2_AddLocalRotation` (`self.HeliRotor`) (`KismetMathLibrary.MakeRotator` 0.0 0.0 _returnvalue) false false)
    (`SceneComponent.K2_AddLocalRotation` (`self.HeliTailRotor`) (`KismetMathLibrary.MakeRotator` 0.0 0.0 _returnvalue) false false)
    (`KismetSystemLibrary.MoveComponentTo` (`self.DefaultSceneRoot`) (`KismetMathLibrary.MakeVector` (.x (`|GetArrayItem` (`self.destLoc`) (`self.atDest`))) (.y (`|GetArrayItem` (`self.destLoc`) (`self.atDest`))) _returnvalue_z) (struct) false false 120.0)))

(fn `UserConstructionScript`)