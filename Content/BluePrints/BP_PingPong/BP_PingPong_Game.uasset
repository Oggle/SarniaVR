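; BP_PingPong_Game is a ping pong table Blueprint that appears to be an early draft of ball bounce detection.
; The construction script shows or hides the half tabletop and its children from RaiseHalf.
; Hit events on the half and full tops print debug bounce messages.
; The full top prints only for actors absent from BallsOnTableArray, and its Add runs only for those already present, with no item wired.
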(event `self.V1_PPTPlayTopHalf.OnComponentHit`
  (params (HitComponent :type "PrimitiveComponent Object Reference") (OtherActor :type "Actor Object Reference") (OtherComp :type "PrimitiveComponent Object Reference") (NormalImpulse :type "Vector Structure") (Hit :type "HitResult Structure (by ref)"))
  (`KismetSystemLibrary.PrintString` "Ball Bounced on Half"))

(event `self.V1_PPTPlayTopFull.OnComponentHit`
  (params (HitComponent :type "PrimitiveComponent Object Reference") (OtherActor :type "Actor Object Reference") (OtherComp :type "PrimitiveComponent Object Reference") (NormalImpulse :type "Vector Structure") (Hit :type "HitResult Structure (by ref)"))
  (bind _ballsontablearray (`self.ballsOnTableArray`))
  (if (`KismetArrayLibrary.Array_Contains` _ballsontablearray OtherActor)
    (`KismetArrayLibrary.Array_Add` _ballsontablearray)
    (else
      (`KismetSystemLibrary.PrintString` "Ball Bounced on Full"))))

(fn `UserConstructionScript`
  (`SceneComponent.SetVisibility` (`self.V1_PPTPlayTopHalf`) (`self.raiseHalf`) true))