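; Construction-script block generator that places static meshes along a guide spline, using a per-point mesh chosen in RoadDataArray.
; BuildRoadDataArray resizes the array to match the spline point count.
; Each segment's length is divided by the mesh's forward bounds (X or Y) to fill it with evenly stepped, collision-free copies, or position one mesh at the point.
; Only location follows the spline; the CollisonOn branch is unconnected.
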(fn `UserConstructionScript`
  (locals (local_dynamicDistance :type "Float (double-precision)") (local_myIndex :type Integer) (local_myMeshSize :type "Vector Structure") (local_copyFillIndex :type Integer))
  (bind _roaddataarray (`self.RoadDataArray`))
  (bind _guidespline (`self.guideSpline`))
  (bind _local_myindex (`local.local_myIndex`))
  (bind (_min _max) (`StaticMeshComponent.GetLocalBounds` (`self.myStaticMesh`)))
  (bind _returnvalue (`KismetMathLibrary.FTrunc` (/ (- (`SplineComponent.GetDistanceAlongSplineAtSplinePoint` _guidespline (+ _local_myindex 1)) (`SplineComponent.GetDistanceAlongSplineAtSplinePoint` _guidespline _local_myindex)) (`self.meshForwardSize`))))
  (`|ExecutionSequence`
    (:`then_0`
      ;[0.3747 0.9801 1] Get Number of Spline Points
      (set `self.numberOfSplinePoints` (`SplineComponent.GetNumberOfSplinePoints` (`self.guideSpline`))))
    (:`then_1`
      (`/Engine/EditorBlueprintResources/StandardMacros.CompareInt` (`KismetArrayLibrary.Array_Length` (`self.RoadDataArray`)) (`self.numberOfSplinePoints`) :!label _label
        (:`>`
          (`KismetArrayLibrary.Array_Remove` _roaddataarray (`KismetArrayLibrary.Array_LastIndex` _roaddataarray))
          (goto _label))
        (:`<`
          (`KismetArrayLibrary.Array_Add` (`self.RoadDataArray`))
          (goto _label))))
    (:`then_2`
      ;[1 0 0.4067] Loop Through Spline Points
      (for _index (range (+ (- (`self.numberOfSplinePoints`) 2) 1))
        ;[1 0.666 0.03035] Use roaddata array to get then set spline point mesh and index variable
        (set `local.local_myIndex` _index)
        (bind (_output_leftguardrail _output_rightguardrail _output_trackbank _output_trackwidth _output_trackthickness _output_tracktype) (break `/Game/BluePrints/RoadSplines/Data/RoadData` (`|GetArrayItem` (`self.RoadDataArray`) _index)))
        (set `self.placedMesh` _output_tracktype)
        (bind _returnvalue_2 (`AddComponent|NODE_AddStaticMeshComponent-0` :`RelativeTransform` (`self.transformOffset`)))
        (bind _output_get (set `self.myStaticMesh` _returnvalue_2))
        (`StaticMeshComponent.SetStaticMesh` _output_get _output_tracktype)
        (bind _output_get_2 (set `local.local_myMeshSize` (- _max _min)))
        ;[1 0.4803 0.03552] If X is not forward
        (if (`self.yForward`)
          (set `self.meshForwardSize` (.y _output_get_2))
          (else
            (set `self.meshForwardSize` (.x _output_get_2))))
        ;[0.00642 1 0 1 14] Subtract current distance from next distance by the depth of mesh to calc the number of meshes we can insert or possible scale
        ;;[1 0 0] Can We Fit More
        (if (> _returnvalue 1)
          (for _index_2 (range (+ _returnvalue 1))
            ;;[0.2573 0.1697 1] Add copy of the mesh just placed
            (set `local.local_copyFillIndex` _index_2)
            (bind _returnvalue_3 (`AddComponent|NODE_AddStaticMeshComponent-1` :`RelativeTransform` (`self.transformOffset`)))
            ;;;[0.08854 0.02466 0.02995 1 14] Set static mesh to chosen mesh
            (bind _output_get_3 (set `self.myStaticMesh` _returnvalue_3))
            (`StaticMeshComponent.SetStaticMesh` _output_get_3 (`self.placedMesh`))
            (`PrimitiveComponent.SetCollisionEnabled` _output_get_3 "NoCollision")
            (`SceneComponent.K2_SetWorldLocation` (`self.myStaticMesh`) (`SplineComponent.GetLocationAtDistanceAlongSpline` (`self.guideSpline`) (+ (`SplineComponent.GetDistanceAlongSplineAtSplinePoint` (`self.guideSpline`) (`local.local_myIndex`)) (* (`local.local_copyFillIndex`) (`self.meshForwardSize`))) "World") false false))
          (else
            ;[1 0 0.01364] Set Final Position
            (`SceneComponent.K2_SetWorldLocation` (`self.myStaticMesh`) (`SplineComponent.GetLocationAtSplinePoint` (`self.guideSpline`) (`local.local_myIndex`) "World") false false)))))))