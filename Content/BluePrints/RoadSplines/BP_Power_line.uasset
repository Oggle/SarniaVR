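; Power line actor that defines a wire toward a next pole along a spline component named Road.
; The construction script adds a spline mesh for each existing spline point, using world-space locations and tangents of that point and the next.
; On BeginPlay, DrawWire appends three points: the spline origin, the offset to NextPoleVector (commented as a sagging midpoint) and NextPoleVector itself, without creating meshes for them.
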(event `self.ReceiveBeginPlay`
  (`self.drawWire` (`self.nextPoleVector`)))

(fn `drawWire`
  (params (thisVector :type "Vector Structure (by ref)"))
  (locals (local_NextPoleConnect :type "Vector Structure"))
  (bind _returnvalue (`SceneComponent.K2_GetComponentLocation` (`self.Road`)))
  (set `local.local_NextPoleConnect` thisVector)
  ;[0.441 0.7525 1] Create 1st Point in wire spline, not sure if I need it
  (`SplineComponent.AddSplinePoint` (`self.Road`) _returnvalue "World" true)
  ;[0.2568 1 0.01696] Add Point Half Way and down a little.
  (`SplineComponent.AddSplinePoint` (`self.Road`) (- (`local.local_NextPoleConnect`) _returnvalue) "World" true)
  ;[0.6094 0.103 0] Create final spline wire point at the next poles wire connect
  (`SplineComponent.AddSplinePoint` (`self.Road`) (`local.local_NextPoleConnect`) "World" true)
  (`KismetSystemLibrary.PrintString` "Wire Drawn" false))

(fn `UserConstructionScript`
  (bind _road (`self.Road`))
  (for _index (range (`SplineComponent.GetNumberOfSplinePoints` (`self.Road`)))
    (bind _returnvalue (`AddComponent|NODE_AddSplineMeshComponent-0`))
    (bind (_location _tangent) (`SplineComponent.GetLocationAndTangentAtSplinePoint` _road _index "World"))
    (bind (_location_2 _tangent_2) (`SplineComponent.GetLocationAndTangentAtSplinePoint` _road (+ _index 1) "World"))
    (`SplineMeshComponent.SetStartAndEnd` _returnvalue _location _tangent _location_2 _tangent_2 true)
    (`SceneComponent.K2_AttachToComponent` _returnvalue null "None" "KeepRelative" "KeepRelative" "KeepRelative" true)))