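; Bus vehicle Pawn, apparently an early movement prototype, that prints a debug message on BeginPlay.
; Every Tick it stores delta time and feeds a constant diagonal world vector, including an upward component, into FloatingPawnMovement, so it moves without player input.
; An AddMovementInput call and nodes for tires, top speed, forward vector and location are left unconnected.
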(event `self.ReceiveBeginPlay`
  (`KismetSystemLibrary.PrintString` "Bus Pawn Alive"))

(event `self.ReceiveTick`
  (params (DeltaSeconds :type "Float (single-precision)"))
  (bind _output_get (set `self.myDeltaSeconds` DeltaSeconds))
  (`PawnMovementComponent.AddInputVector` (`self.FloatingPawnMovement`) (1.0 1.0 1.0) false))

(fn `UserConstructionScript`)