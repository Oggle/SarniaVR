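; Spline-driven sidewalk actor (1m variant) that builds deformed mesh segments along its Road spline in the construction script.
; Each pair of neighboring points gets a SplineMeshComponent with the ScaleBy transform, local-space positions and tangents from the spline, attached to the root.
; When EvenTangent is set, one segment gets zero tangents and the flag then clears itself, so later segments keep spline tangents.
; Event graph is empty.
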(fn `UserConstructionScript`
  (locals (local_startTangent :type "Vector Structure") (local_endTangent :type "Vector Structure") (local_startPos :type "Vector Structure") (local_endPos :type "Vector Structure") (local_splineMeshComp :type "SplineMeshComponent Object Reference") (local_myArrayIndex :type Integer))
  (bind _road (`self.Road`))
  (bind (_location _tangent) (`SplineComponent.GetLocationAndTangentAtSplinePoint` _road (`local.local_myArrayIndex`) "Local"))
  (bind (_location_2 _tangent_2) (`SplineComponent.GetLocationAndTangentAtSplinePoint` _road (+ (`local.local_myArrayIndex`) 1) "Local"))
  (for _index (range (+ (- (`SplineComponent.GetNumberOfSplinePoints` (`self.Road`)) 2) 1))
    (set `local.local_myArrayIndex` _index)
    (bind _returnvalue (`AddComponent|NODE_AddSplineMeshComponent-0` :`RelativeTransform` (`self.scaleBy`)))
    (set `local.local_splineMeshComp` _returnvalue)
    (bind _output_get (set `local.local_startPos` _location))
    (set `local.local_endPos` _location_2)
    (set `local.local_startTangent` _tangent)
    (set `local.local_endTangent` _tangent_2)
    (if (`self.evenTangent`)
      (set `local.local_startTangent` (0.0 0.0 0.0))
      (set `local.local_endTangent` (0.0 0.0 0.0))
      (set `self.evenTangent` false))
    (`SplineMeshComponent.SetStartAndEnd` (`local.local_splineMeshComp`) (`local.local_startPos`) (`local.local_startTangent`) (`local.local_endPos`) (`local.local_endTangent`) true)
    (`SceneComponent.K2_AttachToComponent` (`local.local_splineMeshComp`) (`self.DefaultSceneRoot`) "None" "KeepRelative" "KeepRelative" "KeepRelative" true)))