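; Exterior vehicle prop that picks a chassis from a struct array, optionally randomized once, and drives along world Y at the Accel rate.
; The construction script sets the body mesh and tints it through custom primitive data, avoiding dynamic materials.
; Per-chassis data positions and scales the four wheels when a front offset is set.
; Toggles control the title text and remove the headlights.
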(event `self.ReceiveTick`
  (params (DeltaSeconds :type "Float (single-precision)"))
  (`self.K2_AddActorWorldOffset` (`KismetMathLibrary.MakeVector` 0.0 (* DeltaSeconds (`self.accel`)))))

(fn `UserConstructionScript`
  (locals (local_totalChassis :type Integer) (local_finalWheelOffset :type "Float (double-precision)") (local_tireScaleOffset :type "Float (double-precision)" :default 1.0) (local_wheelFrameOffset :type "Float (double-precision)") (local_myTitle :type Name))
  (bind (_myprimitivecolor_r _myprimitivecolor_g _myprimitivecolor_b) (break `LinearColor` (`self.myPrimitiveColor`)))
  (bind _local_tirescaleoffset (`local.local_tireScaleOffset`))
  (bind _veh_textrender (`self.veh_textRender`))
  (bind _output_veh_mesh (break `/Game/GameReady/ext_prop/ext_veh_struct` (`|GetArrayItem` (`self.myVehicleStruct`) (`self.atBody`))))
  (bind (_output_veh_mesh_2 _output_veh_title _output_veh_wheeloffset_front _output_veh_wheelframeoffset _output_veh_wheelscaleoffset) (break `/Game/GameReady/ext_prop/ext_veh_struct` (`|GetArrayItem` (`self.myVehicleStruct`) (`self.atBody`))))
  ;[0.7438 0.2276 1] Inject Primitive Colour
  ;;[0.8183 1 0.008445] Get Total User Chassis
  (bind _output_get (set `local.local_totalChassis` (`KismetArrayLibrary.Array_Length` (`self.myVehicleStruct`))))
  ;;[0.6757 0.07181 1] Randomize Body
  (if (`self.makeRandom`)
    (set `self.atBody` (`KismetMathLibrary.RandomInteger` (`local.local_totalChassis`)))
    (set `self.makeRandom` false))
  ;;[1 0.8628 0.2543] Set the custom chassis mesh
  (`StaticMeshComponent.SetStaticMesh` (`self.Body`) _output_veh_mesh)
  ;;[0.2111 0.07339 1] Inject Color
  (`PrimitiveComponent.SetCustomPrimitiveDataFloat` (`self.Body`) 4 1.0)
  (`PrimitiveComponent.SetCustomPrimitiveDataVector3` (`self.Body`) 0 (`KismetMathLibrary.MakeVector` _myprimitivecolor_r _myprimitivecolor_g _myprimitivecolor_b))
  ;;[1 0.0904 0.2911] Offset Tires
  ;;;[1 0 0.1562] Localize Struct Variables
  (set `local.local_tireScaleOffset` _output_veh_wheelscaleoffset)
  (set `local.local_wheelFrameOffset` _output_veh_wheelframeoffset)
  (set `local.local_myTitle` _output_veh_title)
  (bind _output_get_2 (set `local.local_finalWheelOffset` _output_veh_wheeloffset_front))
  (if (> _output_get_2 0.0)
    (`SceneComponent.K2_SetRelativeLocation` (`self.Veh_Sedan_01_Blue_Wheel_FL`) (`KismetMathLibrary.MakeVector` 0.0 (+ (`local.local_finalWheelOffset`) (`local.local_wheelFrameOffset`))) false false)
    (`SceneComponent.K2_SetRelativeLocation` (`self.Veh_Sedan_01_Blue_Wheel_FR`) (`KismetMathLibrary.MakeVector` 0.0 (+ (`local.local_finalWheelOffset`) (`local.local_wheelFrameOffset`))) false false)
    (`SceneComponent.K2_SetRelativeLocation` (`self.Veh_Sedan_01_Blue_Wheel_RL`) (`KismetMathLibrary.MakeVector` 0.0 (+ (* (`local.local_finalWheelOffset`) -1.0) (`local.local_wheelFrameOffset`))) false false)
    (`SceneComponent.K2_SetRelativeLocation` (`self.Veh_Sedan_01_Blue_Wheel_RR`) (`KismetMathLibrary.MakeVector` 0.0 (+ (* (`local.local_finalWheelOffset`) -1.0) (`local.local_wheelFrameOffset`))) false false)
    ;;;[0.6839 1 0.0478] Apply Tire Scale Per Vehicle
    (`SceneComponent.SetRelativeScale3D` (`self.Veh_Sedan_01_Blue_Wheel_RR`) (`KismetMathLibrary.MakeVector` _local_tirescaleoffset _local_tirescaleoffset _local_tirescaleoffset))
    (`SceneComponent.SetRelativeScale3D` (`self.Veh_Sedan_01_Blue_Wheel_RL`) (`KismetMathLibrary.MakeVector` _local_tirescaleoffset _local_tirescaleoffset _local_tirescaleoffset))
    (`SceneComponent.SetRelativeScale3D` (`self.Veh_Sedan_01_Blue_Wheel_FR`) (`KismetMathLibrary.MakeVector` _local_tirescaleoffset _local_tirescaleoffset _local_tirescaleoffset))
    (`SceneComponent.SetRelativeScale3D` (`self.Veh_Sedan_01_Blue_Wheel_FL`) (`KismetMathLibrary.MakeVector` _local_tirescaleoffset _local_tirescaleoffset _local_tirescaleoffset)))
  ;;;[0.1455 0.8701 1] Show Title Of Car
  (if (`self.showTitle`)
    (`TextRenderComponent.K2_SetText` _veh_textrender (`KismetTextLibrary.Conv_NameToText` (`local.local_myTitle`)))
    (else
      (`SceneComponent.SetVisibility` _veh_textrender false true)))
  (if (not (`self.lightsOn`))
    (`ActorComponent.K2_DestroyComponent` (`self.headLight_left`))
    (`ActorComponent.K2_DestroyComponent` (`self.headLight_right`))))