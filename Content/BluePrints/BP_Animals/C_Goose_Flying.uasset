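; Flying goose actor that plays a looping crow flight animation on its Bird component after a random startup delay.
; It slowly eases its root toward an indexed DestLoc location with MoveComponentTo, then increments the index.
; Only when the index exceeds the array length does it reset to zero, wait randomly, turn the root with LookAt, and repeat the move.
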(event `self.ReceiveBeginPlay`
  (bind _output (`|GetArrayItem` (`self.destLoc`) (`self.atDestArray`)))
  (bind (_returnvalue_location _returnvalue_rotation) (`KismetMathLibrary.BreakTransform` (`KismetAnimationLibrary.K2_LookAt` (`SceneComponent.K2_GetComponentToWorld` (`self.DefaultSceneRoot`)) _output _output)))
  (`KismetSystemLibrary.Delay` (* (`KismetMathLibrary.RandomFloat`) 8.0))
  (`SkeletalMeshComponent.PlayAnimation` (`self.Bird`) "/Game/AnimalVarietyPack/Crow/Animations/ANIM_Crow_Fly.ANIM_Crow_Fly" true)
  (`KismetSystemLibrary.MoveComponentTo` (`self.DefaultSceneRoot`) (`|GetArrayItem` (`self.destLoc`) (`self.atDestArray`)) (`KismetMathLibrary.MakeRotator` 0.0 0.0 (`self.rotOffset`)) true true 200.0 :!label _label)
  (`/Engine/EditorBlueprintResources/StandardMacros.IncrementInt` (`self.atDestArray`)
    (:`  `
      (if (> (`self.atDestArray`) (`KismetArrayLibrary.Array_Length` (`self.destLoc`)))
        (set `self.atDestArray` 0)
        (`KismetSystemLibrary.Delay` (* (`KismetMathLibrary.RandomFloat`) (`self.delayBaseTime`)))
        (`SceneComponent.K2_SetWorldRotation` (`self.DefaultSceneRoot`) _returnvalue_rotation false false)
        (goto _label)))))

(fn `UserConstructionScript`)