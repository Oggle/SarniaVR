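; Floating bus pawn that drives itself between the level's BP_BusStop actors, using FloatingPawnMovement.
; BeginPlay gathers stop locations; Tick feeds forward input and, when turning is enabled, yaws the actor toward the current goal.
; Overlapping an actor not yet in route history halts the bus, advances the goal, classifies it as ahead or turn, and resumes after a delay.
; Ground-trace ride height, tire steering and road-spline lookup are present but unconnected.
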(event `self.ReceiveTick`
  (params (DeltaSeconds :type "Float (single-precision)"))
  (bind _sarnia_bus_01 (`self.Sarnia_Bus_01`))
  (bind (_returnvalue_x _returnvalue_y) (`KismetMathLibrary.BreakVector` (+ (`self.busForwardVector`) (`self.myDeltaXDrive`))))
  (bind _returnvalue (`SceneComponent.K2_GetComponentLocation` _sarnia_bus_01))
  (bind (_returnvalue_roll _returnvalue_pitch _returnvalue_yaw) (`KismetMathLibrary.BreakRotator` (`KismetMathLibrary.FindLookAtRotation` _returnvalue (`self.destGoal`))))
  ;[1 0 0.02652] Event Tick
  (set `self.myDeltaSeconds` DeltaSeconds)
  (bind _newdeltadrivepower (`self.getDeltaDrivePower`))
  (set `self.myDeltaXDrive` _newdeltadrivepower)
  (bind _output_get (set `self.atLocation` _returnvalue))
  (set `self.busForwardVector` (`SceneComponent.GetForwardVector` _sarnia_bus_01))
  (if (== _output_get (`self.destGoal`) :`ErrorTolerance` 0.5)
    (switch `int` 0
      (:`0`
        _)
      (:`1`
        (set `self.canTurn` true :!label _label))
      (:`2`
        (goto _label))))
  (if (`self.canDrive`)
    ;;[0.487 0.7506 1] Move All Input Vector w Rotate
    (if (`self.canTurn`)
      (`self.K2_AddActorWorldRotation` (`KismetMathLibrary.MakeRotator` 0.0 0.0 (* (* (`self.myDeltaSeconds`) (- _returnvalue_yaw (.yaw (`SceneComponent.K2_GetComponentRotation` _sarnia_bus_01)))) (`self.myTurnRadius`)))) ; Rotate All
      (`PawnMovementComponent.AddInputVector` (`self.busFloatingPawnMovement`) (`KismetMathLibrary.MakeVector` _returnvalue_x _returnvalue_y) false)
      (else
        ;;[0.487 0.7506 1] Just Move Forward
        (`PawnMovementComponent.AddInputVector` (`self.busFloatingPawnMovement`) (`KismetMathLibrary.MakeVector` _returnvalue_x) false)))))

(event `self.ReceiveActorBeginOverlap`
  (params (OtherActor :type "Actor Object Reference"))
  ;[1 0.1253 0.02567] Overlap Detect Next Stop
  (`KismetSystemLibrary.PrintString` "Hit stop" true true (struct :`G` 0.66 :`B` 1.0 :`A` 1.0) (`self.printScreenTime`))
  (if (not (`self.routeHistoryBeen` OtherActor))
    (`self.atStop`)
    (`self.nextStop` OtherActor)
    (`KismetSystemLibrary.Delay` 8.0)
    (bind _canleave (`self.leaveStop`))
    (if _canleave
      (if (> (`|GetArrayItem` (`self.destGoalType`) (`self.atGoalArray`)) 0)
        (set `self.canTurn` true))
      (set `self.canDrive` true)
      (set `self.drivePower` 0.25))))

(event `self.ReceiveBeginPlay`
  ;[1 0.009454 0] Begin Play Get Stops Next Stop Drive
  (`self.getStops`)
  (`self.nextStop` null)
  (set `self.canDrive` true))

(event `self.FR_Tire.OnComponentBeginOverlap`
  (params (OverlappedComponent :type "PrimitiveComponent Object Reference") (OtherActor :type "Actor Object Reference") (OtherComp :type "PrimitiveComponent Object Reference") (OtherBodyIndex :type Integer) (bFromSweep :type Boolean) (SweepResult :type "HitResult Structure (by ref)"))
  ;[0.1557 0.9702 1] Tire Overlaps
  (`KismetSystemLibrary.PrintString` "FR Overlap"))

(event `self.FL_Tire.OnComponentBeginOverlap`
  (params (OverlappedComponent :type "PrimitiveComponent Object Reference") (OtherActor :type "Actor Object Reference") (OtherComp :type "PrimitiveComponent Object Reference") (OtherBodyIndex :type Integer) (bFromSweep :type Boolean) (SweepResult :type "HitResult Structure (by ref)"))
  ;[0.1557 0.9702 1] Tire Overlaps
  (`KismetSystemLibrary.PrintString` "FL Overlap"))

(fn `atStop`
  (`KismetSystemLibrary.PrintString` "Arrived At Stop" true true (struct :`G` 0.66 :`B` 1.0 :`A` 1.0) (`self.printScreenTime`))
  (set `self.drivePower` 0.0)
  (set `self.canDrive` false))

(fn `getDeltaDrivePower`
  (returns (newDeltaDrivePower :type "Float (double-precision)"))
  ;[1 0.09874 0] Drive Power, should be hp..
  (return (* (* (`self.drivePower`) (`self.myDeltaSeconds`)) (`self.topSpeed`))))

(fn `getLeftRightDegree`
  (params (vectorA :type "Vector Structure") (vectorB :type "Vector Structure"))
  (returns (myRadians :type "Float (double-precision)"))
  (return (`KismetMathLibrary.Dot_VectorVector` (`KismetMathLibrary.GetForwardVector` (`KismetMathLibrary.MakeRotator` (.x vectorA) (.y vectorA))) (`KismetMathLibrary.GetForwardVector` (`KismetMathLibrary.MakeRotator` (.x vectorB) (.y vectorB))))))

(fn `getStops`
  (bind _printscreentime (`self.printScreenTime`))
  (bind _returnvalue (`KismetArrayLibrary.Array_Length` (`self.allBusStops`)))
  ;[0.09912 0.06801 1] Get all stops on level, fill array
  (bind _outactors (`GameplayStatics.GetAllActorsOfClass` "/Game/BluePrints/BP_BusStop.BP_BusStop_C"))
  (bind _output_get (set `self.allBusStops` _outactors))
  (if (> _returnvalue 0)
    (`KismetSystemLibrary.PrintString` (`KismetStringLibrary.Concat_StrStr` (`KismetStringLibrary.Conv_IntToString` _returnvalue) " Stops Found") true true (struct :`G` 0.66 :`B` 1.0 :`A` 1.0) _printscreentime)
    (for _array_element _output_get
      (`KismetArrayLibrary.Array_Add` (`self.destArrays`) (`self.K2_GetActorLocation` _array_element)))
    (`KismetSystemLibrary.PrintString` "Bus Got Routes" true true (struct :`G` 0.66 :`B` 1.0 :`A` 1.0) (`self.printScreenTime`))
    (else
      (`KismetSystemLibrary.PrintString` "No Stops" true true (struct :`G` 0.66 :`B` 1.0 :`A` 1.0) _printscreentime))))

(fn `leaveStop`
  (returns (canLeave :type Boolean))
  (`KismetSystemLibrary.PrintString` "Leaving Stop" true true (struct :`G` 0.66 :`B` 1.0 :`A` 1.0) (`self.printScreenTime`))
  (return true))

(fn `moveBus`
  (locals (newPawnY :type "Float (double-precision)"))
  (bind _returnvalue (`SceneComponent.K2_GetComponentLocation` (`self.Sarnia_Bus_01`)))
  (bind _returnvalue_2 (`KismetMathLibrary.FindLookAtRotation` _returnvalue (`self.destLocation`)))
  (bind _x (.x (+ _returnvalue (* (`KismetMathLibrary.GetForwardVector` _returnvalue_2) (`self.myDeltaSeconds`)))))
  ;[0.09912 0.06801 1] Calculate forward Vector
  (set `self.turnZ` _returnvalue_2)
  (if (`self.canTurn`)
    (set `self.deltaBusVector` (`KismetMathLibrary.MakeVector` _x (.y (+ _returnvalue (* (`KismetMathLibrary.GetForwardVector` _returnvalue_2) (`self.myDeltaSeconds`)))) (.z (+ _returnvalue (* (`KismetMathLibrary.GetForwardVector` _returnvalue_2) (`self.myDeltaSeconds`))))))
    (else
      (set `self.deltaBusVector` (`KismetMathLibrary.MakeVector` _x))))
  ;[1 0 0.02473] Move Pawn Float
  (`PawnMovementComponent.AddInputVector` (`self.busFloatingPawnMovement`) (`self.deltaBusVector`) false))

(fn `nextStop`
  (params (newStopActor :type "Actor Object Reference"))
  (bind _printscreentime (`self.printScreenTime`))
  (bind _returnvalue (`KismetMathLibrary.Dot_VectorVector` (`KismetMathLibrary.GetForwardVector` (`KismetMathLibrary.MakeRotator` (.x (`self.busForwardVector`)) (.y (`self.busForwardVector`)))) (`KismetMathLibrary.GetForwardVector` (`KismetMathLibrary.MakeRotator` (.x (`self.destLocation`)) (.y (`self.destLocation`))))))
  (bind _returnvalue_2 (`KismetMathLibrary.RadiansToDegrees` _returnvalue))
  ;[0.3032 0.08999 1 1 14] Update route history and increment stop destination integer
  (if (`KismetSystemLibrary.IsValid` newStopActor)
    (`self.routeHistoryAdd` newStopActor))
  (bind _result (`/Engine/EditorBlueprintResources/StandardMacros.IncrementInt` (`self.atLocArray`))
    (:`  `
      ;[0.3191 0.6674 1] Get our Actor current location
      (set `self.atLocation` (`self.K2_GetActorLocation`))
      (set `self.busForwardVector` (`SceneComponent.GetForwardVector` (`self.Sarnia_Bus_01`)))
      ;[0.4638 1 0.9302] Detect end of route array destinations and reset
      (if (>= _result (`KismetArrayLibrary.Array_Length` (`self.destArrays`)))
        (set `self.atLocArray` 0))
      ;[0.3934 1 0.3188] Update destination to next stop, set this to goal as well
      (bind _output_get (set `self.destLocation` (`|GetArrayItem` (`self.destArrays`) (`self.atLocArray`))))
      (`KismetSystemLibrary.PrintString` (`KismetStringLibrary.Conv_VectorToString` _output_get) true true (struct :`G` 0.66 :`B` 1.0 :`A` 1.0) (`self.printScreenTime`))
      (set `self.destGoal` _output_get)
      ;[0.3591 1 0.5123] Calc Left Right by Lookat Vectors
      (`KismetSystemLibrary.PrintString` (`KismetStringLibrary.Concat_StrStr` "Goingt To Stop " (`KismetStringLibrary.Conv_IntToString` (`self.atLocArray`))) true true (struct :`G` 0.66 :`B` 1.0 :`A` 1.0) _printscreentime)
      (`KismetSystemLibrary.PrintString` (`KismetStringLibrary.Conv_DoubleToString` _returnvalue_2) true true (struct :`R` 0.796875 :`G` 0.003423 :`B` 0.637764 :`A` 1.0) _printscreentime)
      ;;[1 0.02034 0.1601 1 12] Forward Degree Difference from Destination
      (set `self.DestDegreeDif` _returnvalue_2)
      (bind _output_get_2 (set `self.DestDotDif` _returnvalue))
      (`KismetSystemLibrary.PrintString` (`KismetStringLibrary.Concat_StrStr` (`KismetStringLibrary.Conv_DoubleToString` _output_get_2) "Dot") false true (struct :`R` 1.0 :`G` 0.109751 :`B` 0.050025 :`A` 1.0) (`self.printScreenTime`))
      ;;[1 0.1876 0.8532] If our next stop is ahead or a turn
      (if (>= (`KismetMathLibrary.Abs` (`self.DestDegreeDif`)) 35.0)
        (if (> (`self.DestDotDif`) 0.0)
          ;;;[0.5625 0.5295 0.000214] find turn if we need one
          (`KismetArrayLibrary.Array_Add` (`self.destGoalType`) 1)
          (else
            (`KismetArrayLibrary.Array_Add` (`self.destGoalType`) 2)))
        (`KismetSystemLibrary.PrintString` (`KismetStringLibrary.Concat_StrStr` "Turn Right By " (`KismetStringLibrary.Conv_DoubleToString` (`self.DestDegreeDif`))) true true (struct :`G` 0.66 :`B` 1.0 :`A` 1.0) (`self.printScreenTime`))
        (else
          ;;;[1 0.4837 0.3229] Stop Ahead
          (`KismetArrayLibrary.Array_Add` (`self.destGoalType`))
          (`KismetSystemLibrary.PrintString` "Stop Ahead" true true (struct :`G` 0.66 :`B` 1.0 :`A` 1.0) (`self.printScreenTime`)))))))

(fn `routeHistoryAdd`
  (params (stopActor :type "Actor Object Reference"))
  (bind _returnvalue (`KismetArrayLibrary.Array_Add` (`self.stopAtors`) stopActor))
  (`KismetSystemLibrary.PrintString` (`KismetStringLibrary.Concat_StrStr` (`KismetStringLibrary.Concat_StrStr` "Added Stop" (`KismetStringLibrary.Conv_IntToString` _returnvalue)) (`KismetStringLibrary.Concat_StrStr` "History Length" (`KismetStringLibrary.Conv_IntToString` (`KismetArrayLibrary.Array_Length` (`self.stopAtors`))))) true true (struct :`G` 0.66 :`B` 1.0 :`A` 1.0) (`self.printScreenTime`)))

(fn `routeHistoryBeen`
  (params (thisStop :type "Actor Object Reference"))
  (returns (haveBeen :type Boolean))
  (return (`KismetArrayLibrary.Array_Contains` (`self.stopAtors`) thisStop)))

(fn `UserConstructionScript`
  (bind _mytiresarray (`self.myTiresArray`))
  (bind _sarnia_bus_01 (`self.Sarnia_Bus_01`))
  (bind _fr_tire (`self.FR_Tire`))
  (bind (_min _max) (`StaticMeshComponent.GetLocalBounds` _sarnia_bus_01))
  (bind (_min_2 _max_2) (`StaticMeshComponent.GetLocalBounds` _fr_tire))
  (bind (_returnvalue_x _returnvalue_y _returnvalue_z) (`KismetMathLibrary.BreakVector` (* (`SceneComponent.K2_GetComponentScale` _fr_tire) (- _max_2 _min_2))))
  (`KismetArrayLibrary.Array_Clear` _mytiresarray)
  (`KismetArrayLibrary.Array_Add` _mytiresarray (`self.FL_Tire`))
  (`KismetArrayLibrary.Array_Add` _mytiresarray (`self.FR_Tire`))
  (`KismetArrayLibrary.Array_Add` _mytiresarray (`self.BL_Tire`))
  (`KismetArrayLibrary.Array_Add` _mytiresarray (`self.BR_Tire`))
  ;[1 1 1] Half Tire H Variable
  (bind _output_get (set `self.tireHeight` _returnvalue_z))
  (set `self.tireHalf` (/ _output_get 2.0))
  (set `self.busSize` (* (`SceneComponent.K2_GetComponentScale` _sarnia_bus_01) (- _max _min))))