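; BP_HouseFly is a housefly actor with procedurally flapping wings and configurable part colours.
; A looping BeginPlay delay, randomised up to FlapInterval, toggles UpWing and applies opposite relative roll rotations to the two solid wing meshes.
; The construction script writes body, eye, wing and vein colours into Custom Primitive Data through a shared helper.
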(event `self.ReceiveBeginPlay`
  (`KismetSystemLibrary.Delay` (* (`KismetMathLibrary.RandomFloat`) (`self.flapInterval`)) :!label _label)
  (if (`self.upWing`)
    (`/Engine/EditorBlueprintResources/StandardMacros.NegateFloat` (`self.flapScale`)
      (:`  `
        (set `self.upWing` false)))
    (else
      (set `self.upWing` true)))
  (`SceneComponent.K2_AddRelativeRotation` (`self.wingLeftSolid`) (`KismetMathLibrary.MakeRotator` (`self.flapScale`)) false false)
  (`SceneComponent.K2_AddRelativeRotation` (`self.wingRightSolid`) (`KismetMathLibrary.MakeRotator` (* (`self.flapScale`) -1.0)) false false)
  (goto _label))

(event `self.ReceiveTick`
  (params (DeltaSeconds :type "Float (single-precision)"))
  (set `self.Delta Seconds` DeltaSeconds))

(fn `Set Primitive CVec 4`
  (params (thisMeshPrimitive :type "PrimitiveComponent Object Reference") (thisRGBA :type "LinearColor Structure") (startDataIndex :type Integer))
  (bind (_r _g _b _a) (break `LinearColor` thisRGBA))
  (`PrimitiveComponent.SetCustomPrimitiveDataVector4` thisMeshPrimitive startDataIndex (`KismetMathLibrary.MakeVector4` _r _g _b _a)))

(fn `UserConstructionScript`
  ;[1 0 0.08366] Set all colour primitives
  (`self.Set Primitive CVec 4` (`self.wingRightSolid`) (`self.wingSolidColour`))
  (`self.Set Primitive CVec 4` (`self.wingLeftSolid`) (`self.wingSolidColour`))
  (`self.Set Primitive CVec 4` (`self.Body`) (`self.bodyPrimitiveColour`))
  (`self.Set Primitive CVec 4` (`self.leftVien`) (`self.wingVienColour`))
  (`self.Set Primitive CVec 4` (`self.rightVien`) (`self.wingVienColour`))
  (`self.Set Primitive CVec 4` (`self.Eye`) (`self.eyeBaseColour`)))