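; BP_Walkman_Pawn is a Walkman prop with a door and a removable cassette, currently running a looping demo sequence.
; The construction script captures the body, open-door and cassette-out transforms from the components.
; Helper functions snap the door or cassette between stored transforms, with open, close and play also setting WalkmanState and printing status.
; BeginPlay repeatedly inserts, closes, opens and ejects with delays, never calling play.
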(event `self.ReceiveBeginPlay`
  ;[0.4121 1 0.08369] Functions Sketch
  (`KismetSystemLibrary.RetriggerableDelay` 5.0 :!label _label)
  (`self.wm_insertCassette`)
  (`KismetSystemLibrary.Delay` 2.0)
  (`self.wm_close`)
  (`KismetSystemLibrary.Delay` 3.0)
  (`self.wm_open`)
  (`KismetSystemLibrary.Delay` 3.0)
  (`self.wm_ejectCassette`)
  (goto _label))

(fn `UserConstructionScript`
  ;[1 0.05899 0] Capture Edits as Default Transforms
  (set `self.wManBodyDefaultTransform` (`SceneComponent.GetRelativeTransform` (`self.Sony_Walkman_Walkman_Body`)))
  (set `self.wManDoorDefaultTransform` (`SceneComponent.GetRelativeTransform` (`self.Sony_Walkman_WalkmanDoor`)))
  (set `self.wManCassetteOutTransform` (`SceneComponent.GetRelativeTransform` (`self.Cassette_Tape_01`))))

(fn `wm_close`
  (`SceneComponent.K2_SetRelativeTransform` (`self.Sony_Walkman_WalkmanDoor`) (`self.wManDoorClosedTransform`) false false)
  (set `self.walkmanState` 1)
  (`KismetSystemLibrary.PrintString` "Walkman Closed"))

(fn `wm_ejectCassette`
  (`SceneComponent.K2_SetRelativeTransform` (`self.Cassette_Tape_01`) (`self.wManCassetteOutTransform`) false false))

(fn `wm_insertCassette`
  (`SceneComponent.K2_SetRelativeTransform` (`self.Cassette_Tape_01`) (`KismetMathLibrary.MakeTransform` (`KismetMathLibrary.MakeVector` (.x (.location (`self.wManCassetteInTransform`))) (.y (.location (`self.wManCassetteInTransform`))) (.z (.location (`self.wManCassetteInTransform`)))) (.rotation (`self.wManCassetteInTransform`))) false false))

(fn `wm_open`
  (`SceneComponent.K2_SetRelativeTransform` (`self.Sony_Walkman_WalkmanDoor`) (`self.wManDoorDefaultTransform`) false false)
  (set `self.walkmanState` 0)
  (`KismetSystemLibrary.PrintString` "Walkman Open"))

(fn `wm_play`
  (set `self.walkmanState` 3)
  (`KismetSystemLibrary.PrintString` "Walkman Playing"))