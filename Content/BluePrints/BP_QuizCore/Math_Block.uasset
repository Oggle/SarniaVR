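; Math_Block is a physics block for the quiz core that displays a random integer and can launch itself on BeginPlay.
; Its construction script rolls the number, applies mesh and text offsets, and adds text components per ShowNumberOnSides entry, though side rotations transform MyNumberTR instead of the new components.
; Each hit applies an impulse with Z scaled by the number and, when CanSpawn is true, toggles that delayed gate without spawning anything.
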(event `self.ReceiveBeginPlay`
  (if (`self.launchOnStart`)
    (`PrimitiveComponent.AddImpulse` (`self.backingMesh`) (`KismetMathLibrary.MakeVector` (.x (`self.launchVector`)) (.y (`self.launchVector`)) (.z (`self.launchVector`))) "None" true)))

(event `self.backingMesh.OnComponentHit`
  (params (HitComponent :type "PrimitiveComponent Object Reference") (OtherActor :type "Actor Object Reference") (OtherComp :type "PrimitiveComponent Object Reference") (NormalImpulse :type "Vector Structure") (Hit :type "HitResult Structure (by ref)"))
  ;[0.234 1 0.4255] Creates random motion from their random number
  (`PrimitiveComponent.AddImpulse` (`self.backingMesh`) (`KismetMathLibrary.MakeVector` (.x (`self.launchVector`)) (.y (`self.launchVector`)) (* (`KismetMathLibrary.Conv_IntToDouble` (`self.myRandomInt`)) 4.2)) "None" true)
  (if (`self.canSpawn`)
    (`|ExecutionSequence`
      (:`then_0`)
      (:`then_1`
        ;[0.651 0 1 1 14] Close spawn gate, delay and then open it. This can be scaled for difficulty
        (set `self.canSpawn` false)
        (`KismetSystemLibrary.Delay` (`self.newSpawnDelay`))
        (set `self.canSpawn` true)))))

(fn `UserConstructionScript`
  (locals (mySideTextTR :type "TextRenderComponent Object Reference") (mySidesTRIndex :type Integer) (finalTRSideTransform :type "Transform Structure"))
  (bind _mysidetexttr (`local.mySideTextTR`))
  (bind (_numtextoffsettransform_location _numtextoffsettransform_rotation _numtextoffsettransform_scale) (`KismetMathLibrary.BreakTransform` (`self.numTextOffsetTransform`)))
  (bind (_numtextoffsettransform_location_2 _numtextoffsettransform_rotation_2 _numtextoffsettransform_scale_2) (`KismetMathLibrary.BreakTransform` (`self.numTextOffsetTransform`)))
  (bind (_min _max) (`StaticMeshComponent.GetLocalBounds` (`self.backingMesh`)))
  (`|ExecutionSequence`
    (:`then_0`
      (bind _custombackingmesh (`self.customBackingMesh`)
        (:`then`
          (set `self.backingMesh` _custombackingmesh))
        (:`else`)))
    (:`then_1`
      ;[0.4725 0.9201 1] Set a Random Number
      (bind _output_get (set `self.myRandomInt` (`KismetMathLibrary.RandomIntegerInRange` 0 (`self.randomIntRange`))))
      ;[1 0.3326 0.9534] Set and Customize Text
      (bind _output_get_2 (set `self.myDisplayTxt` (`KismetTextLibrary.Conv_IntToText` _output_get)))
      (`TextRenderComponent.K2_SetText` (`self.myNumberTR`) _output_get_2)
      (`TextRenderComponent.SetWorldSize` (`self.myNumberTR`) (`self.textSize`))
      (`SceneComponent.K2_AddLocalTransform` (`self.backingMesh`) (`self.backingMeshOffset`) false false)
      (`SceneComponent.K2_AddLocalTransform` (`self.myNumberTR`) (`self.numTextOffsetTransform`) false false)
      ;[0.5 0.3388 0] Store full and half size dimension vecotr for the backing mesh for ease of use
      (bind _output_get_3 (set `self.backingMeshFinalSize` (* (- _max _min) (.scale (`self.backingMeshOffset`)))))
      (bind _output_get_4 (set `self.backingMeshFinalHalf` (/ _output_get_3 2)))
      (`KismetSystemLibrary.PrintString` (`KismetStringLibrary.Concat_StrStr` "Back MeshX :" (`KismetStringLibrary.Conv_DoubleToString` (.x _output_get_4)))))
    (:`then_2`
      (for (_ _array_index) (`self.showNumberOnSides`)
        (set `local.mySidesTRIndex` _array_index)
        (bind _returnvalue (`AddComponent|NODE_AddTextRenderComponent-0` :`bManualAttachment` true))
        (set `local.mySideTextTR` _returnvalue)
        ;[1 0.01702 0.4611] Switching TopBot
        (if (> (`local.mySidesTRIndex`) 3)
          ;[1 0.5553 0.1941] For TopBot
          (set `local.finalTRSideTransform` (`KismetMathLibrary.MakeTransform` _numtextoffsettransform_location_2 (* (`self.topBotRotator`) (`local.mySidesTRIndex`)) _numtextoffsettransform_scale_2))
          (else
            ;[0 0.9902 1] For around the sides
            (set `local.finalTRSideTransform` (`KismetMathLibrary.MakeTransform` _numtextoffsettransform_location (* (`self.sideRotator`) (`local.mySidesTRIndex`)) _numtextoffsettransform_scale))))
        (`SceneComponent.K2_AddLocalTransform` (`self.myNumberTR`) (`local.finalTRSideTransform`) false false)
        ;[1 0.1289 0.7259] Set the texts for each dynamic text side
        (`TextRenderComponent.K2_SetText` _mysidetexttr (`self.myDisplayTxt`))
        (`TextRenderComponent.SetWorldSize` _mysidetexttr (`self.textSize`))
        (`SceneComponent.K2_AttachToComponent` (`local.mySideTextTR`) (`self.backingMesh`) "None" "KeepRelative" "KeepRelative" "KeepRelative" false)))))