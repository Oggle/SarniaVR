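; Rotating orb that displays the statistics in SarniaStatDB as floating text around a centre sphere.
; The construction script numbers each entry by array index and adds two text renders for it: title and period total below.
; Each pair sits at SphereTextOffset in a random direction, so the layout reshuffles whenever construction reruns.
; Tick spins the whole actor in yaw at OrbitSpeed; the computed sphere size is only printed for debugging.
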(event `self.ReceiveTick`
  (params (DeltaSeconds :type "Float (single-precision)"))
  (`self.K2_AddActorWorldRotation` self (`KismetMathLibrary.MakeRotator` 0.0 0.0 (* DeltaSeconds (`self.orbitSpeed`))) false false))

(fn `UserConstructionScript`
  (locals (local_uniqueIndex :type Integer) (local_sphereSize :type "Transform Structure") (local_myShowTextRender :type "TextRenderComponent Object Reference") (local_myShowStatRender :type "TextRenderComponent Object Reference"))
  (bind _local_myshowtextrender (`local.local_myShowTextRender`))
  (bind _local_myshowstatrender (`local.local_myShowStatRender`))
  (bind _sarniastatdb (`self.sarniaStatDB`))
  (bind _local_uniqueindex (`local.local_uniqueIndex`))
  (bind (_local_spheresize_location _local_spheresize_rotation _local_spheresize_scale) (`KismetMathLibrary.BreakTransform` (`local.local_sphereSize`)))
  (bind _centersphere (`self.centerSphere`))
  (bind (_min _max) (`StaticMeshComponent.GetLocalBounds` _centersphere))
  (bind _returnvalue_location (`KismetMathLibrary.BreakTransform` (`SceneComponent.GetRelativeTransform` (`self.centerSphere`))))
  (bind (_output_uid _output_stat_title _output_stat_category _output_stat_metric _output_stat_period _output_stat_start_value _output_stat_period_total) (break `/Game/BluePrints/StatisticBP/Struct_Sarnia_Stat` (`|GetArrayItem` (`self.sarniaStatDB`) (`local.local_uniqueIndex`))))
  (bind (_uid _stat_title _stat_category _stat_metric _stat_period _stat_start_value _stat_period_total _stat_record_high _stat_record_low _stat_visible) (break `/Game/BluePrints/StatisticBP/Struct_Sarnia_Stat` (`|GetArrayItem` _sarniastatdb (`local.local_uniqueIndex`))))
  ;[1 0.88 0] Get the number of stats
  (bind _output_get (set `self.totalStats` (`KismetArrayLibrary.Array_Length` (`self.sarniaStatDB`))))
  ;[0.7318 1 0 1 12] Check for stats
  (if (> _output_get 0)
    (for _index (range _output_get)
      (`|ExecutionSequence`
        (:`then_0`
          ;[1 0 0.5379] Set unique ids from index order within the array itself.. this is sloppy, but sortable and central
          (set `local.local_uniqueIndex` _index)
          (`KismetArrayLibrary.Array_Set` _sarniastatdb _local_uniqueindex (make `/Game/BluePrints/StatisticBP/Struct_Sarnia_Stat` _local_uniqueindex _stat_title _stat_category _stat_metric _stat_period _stat_start_value _stat_period_total _stat_record_high _stat_record_low _stat_visible)))
        (:`then_1`
          ;[1 0.5969 0] Try to project the text outside the sphere diameter and rotate it.
          (set `local.local_sphereSize` (`KismetMathLibrary.MakeTransform` (0.0 0.0 0.0) (struct) (* (.scale (`SceneComponent.GetRelativeTransform` _centersphere)) (- _max _min))))
          (`KismetSystemLibrary.PrintString` (`KismetStringLibrary.Conv_VectorToString` _local_spheresize_scale)))
        (:`then_2`
          (`|ExecutionSequence`
            (:`then_0`
              ;[1 0.1824 0.7886] Add title
              (bind _returnvalue (`AddComponent|NODE_AddTextRenderComponent-0` :`RelativeTransform` (`KismetMathLibrary.MakeTransform` (+ _returnvalue_location (* (`KismetMathLibrary.GetForwardVector` (`KismetMathLibrary.RandomRotator` false)) (`self.sphereTextOffset`))))))
              (bind _output_get_2 (set `local.local_myShowTextRender` _returnvalue))
              ;[0 0.8583 1] Set the text for the statistic from the array
              (`TextRenderComponent.K2_SetText` _output_get_2 (`KismetTextLibrary.Conv_StringToText` _output_stat_title))
              ;[1 0 0.1621] Set Size and Alignment and colour
              (`TextRenderComponent.SetWorldSize` _local_myshowtextrender (`self.statTitleWorldScale`))
              (`TextRenderComponent.SetHorizontalAlignment` _local_myshowtextrender "EHTA_Center")
              (`TextRenderComponent.SetTextRenderColor` _local_myshowtextrender (`self.titleColour`)))
            (:`then_1`
              ;[1 0.7923 0.05673] Add Number stat
              (bind _returnvalue_2 (`AddComponent|NODE_AddTextRenderComponent-1` :`RelativeTransform` (`KismetMathLibrary.MakeTransform` (`KismetMathLibrary.MakeVector` (.x (.location (`SceneComponent.GetRelativeTransform` (`local.local_myShowTextRender`)))) (.y (.location (`SceneComponent.GetRelativeTransform` (`local.local_myShowTextRender`)))) (- (.z (.location (`SceneComponent.GetRelativeTransform` (`local.local_myShowTextRender`)))) (`self.statTextOffsetZ`))) (.rotation (`SceneComponent.GetRelativeTransform` (`local.local_myShowTextRender`))))))
              (bind _output_get_3 (set `local.local_myShowStatRender` _returnvalue_2))
              (`TextRenderComponent.K2_SetText` _output_get_3 (`KismetTextLibrary.Conv_DoubleToText` _output_stat_period_total "HalfToEven"))
              ;;[1 0.04638 0.146] Set Custom Stat Colour
              (`TextRenderComponent.SetTextRenderColor` _output_get_3 (`self.statColour`))
              ;[1 0.6249 0.2389] Set stat text and size and alignment
              (`TextRenderComponent.SetWorldSize` _local_myshowstatrender (`self.statTitleWorldScale`))
              (`TextRenderComponent.SetHorizontalAlignment` _local_myshowstatrender "EHTA_Center"))))
        (:`then_3`)))
    (else
      (`KismetSystemLibrary.PrintString` "No Stats"))))