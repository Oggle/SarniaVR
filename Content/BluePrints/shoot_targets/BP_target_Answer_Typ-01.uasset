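; Shootable answer target that displays a configurable label and text, set on its text components by the construction script.
; BeginPlay switches off the correct-spark and incorrect-smoke effects, and actor overlap only prints the overlapping actor's name.
; Unconnected logic branches on IsCorrect to print the result, start playback and show the matching effect for a set duration, but nothing currently triggers it.
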(event `self.ReceiveBeginPlay`
  ;[0.2965 0.1402 1] Disable special FX
  (`ActorComponent.SetActive` (`self.correctSparks`) false false)
  (`ActorComponent.SetActive` (`self.incorrectSmoke`) false false))

(event `self.ReceiveActorBeginOverlap`
  (params (OtherActor :type "Actor Object Reference"))
  (`KismetSystemLibrary.PrintString` (`KismetSystemLibrary.GetDisplayName` OtherActor)))

(fn `UserConstructionScript`
  (`TextRenderComponent.K2_SetText` (`self.target_Label`) (`KismetTextLibrary.Conv_StringToText` (`self.myLabel`)))
  (`TextRenderComponent.K2_SetText` (`self.target_ShowText`) (`KismetTextLibrary.Conv_StringToText` (`self.myShowText`))))