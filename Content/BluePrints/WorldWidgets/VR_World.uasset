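; World-placed note actor that shows an optionally spinning icon and reveals a widget when the player pawn enters its collision sphere.
; The construction script creates the widget component with a DP_Pad_Menu, picks icon mesh, material and colour from an indexed list, and sizes the sphere.
; Icon colour reaches the material through custom primitive data.
; Widget text is a hardcoded placeholder, as the ShowText assignment is unconnected.
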(event `self.ReceiveBeginPlay`)

(event `self.ReceiveTick`
  (params (DeltaSeconds :type "Float (single-precision)"))
  (set `self.Delta Seconds` DeltaSeconds)
  ;[1 0.8026 0.04144] Animate the Icon
  (if (`self.animateIcon`)
    (`SceneComponent.K2_AddWorldRotation` (`self.Iconmesh`) (`KismetMathLibrary.MakeRotator` 0.0 0.0 (`self.spinSpeed`)) false false)))

(event `self.myCollisionSphere.OnComponentBeginOverlap`
  (params (OverlappedComponent :type "PrimitiveComponent Object Reference") (OtherActor :type "Actor Object Reference") (OtherComp :type "PrimitiveComponent Object Reference") (OtherBodyIndex :type Integer) (bFromSweep :type Boolean) (SweepResult :type "HitResult Structure (by ref)"))
  (bind _mywidgetcomponent (`self.myWidgetComponent`))
  ;[0.1003 1 0.9203] Check that a player hit us
  (if (== OtherActor (`GameplayStatics.GetPlayerPawn` 0))
    (set `self.hasBeenOpened` true)
    ;[1 0.01891 0] We've been run into
    (`ActorComponent.SetActive` _mywidgetcomponent true false)
    (`SceneComponent.SetVisibility` _mywidgetcomponent true true)
    (`KismetSystemLibrary.PrintString` "Note Hit")))

(fn `UserConstructionScript`
  (locals (local_myWidget :type "UserWidget Object Reference") (local_addedWidgetDyn :type "WidgetComponent Object Reference") (local_widgetMenu :type "/Game/BluePrints/WorldWidgets/DP_Pad_Menu Object Reference") (local_DynWidget :type "/Game/BluePrints/WorldWidgets/DP_Pad_Menu Object Reference") (local_myIcon :type "/Game/BluePrints/WorldWidgets/HelpCoreIcons Structure"))
  (bind (_local_myicon_id _local_myicon_title _local_myicon_type _local_myicon_iconmesh _local_myicon_iconcolor _local_myicon_iconmaterial) (break `/Game/BluePrints/WorldWidgets/HelpCoreIcons` (`local.local_myIcon`)))
  (bind (_r _g _b _a) (`KismetMathLibrary.BreakColor` (`.iconColor_16_AE504C0F464DE1DD0803B281E29AA26B` (break `/Game/BluePrints/WorldWidgets/HelpCoreIcons` (`local.local_myIcon`)))))
  ;[0.1143 1 0.9801] Add Widget Component
  (bind _returnvalue (`AddComponent|NODE_AddWidgetComponent-1`))
  (set `self.myWidgetComponent` _returnvalue)
  ;[1 0.3051 0.8826] Contruct the DP Blueprint
  (bind _returnvalue_2 (`|GenericCreateObject` "/Game/BluePrints/WorldWidgets/DP_Pad_Menu.DP_Pad_Menu_C" (`self.myWidgetComponent`) "DefShowTextDesigner"))
  (bind _output_get (set `local.local_DynWidget` _returnvalue_2))
  ;[0.7961 0 1 1 12] Set global variable for widget Of Component
  (set `self.dynamicDPWidget` _output_get)
  ;[1 0.8855 0] Calculate Correct world scaling
  (`WidgetComponent.SetWidget` (`self.myWidgetComponent`) _output_get)
  ;[0 0.8423 1] Set the custom static mesh
  (bind _output_get_2 (set `local.local_myIcon` (`|GetArrayItem` (`self.myWidgetIcons`) (`self.useMesh`))))
  (`StaticMeshComponent.SetStaticMesh` (`self.Iconmesh`) (`.iconMesh_13_ABB396B54E45F6E190FA939AF24C9323` (break `/Game/BluePrints/WorldWidgets/HelpCoreIcons` _output_get_2)))
  (`SceneComponent.K2_SetRelativeTransform` (`self.Iconmesh`) (`self.iconTransform`) false false)
  ;[0.2356 0 1 1 14] Inject 4Vec Colour and tiling data for materials that support a primitive mesh colour
  (`PrimitiveComponent.SetCustomPrimitiveDataVector4` (`self.Iconmesh`) 0 (`KismetMathLibrary.MakeVector4` _r _g _b _a))
  ;[0.3356 1 0.05203] Set custom material
  (`PrimitiveComponent.SetMaterial` (`self.Iconmesh`) 0 _local_myicon_iconmaterial)
  ;[1 0.09166 0.6459] Set the custom collision size
  (`SphereComponent.SetSphereRadius` (`self.myCollisionSphere`) (`self.collisionSize`) true)
  (set `/Game/BluePrints/WorldWidgets/DP_Pad_Menu.myShowText` "Here is hoping" (`self.dynamicDPWidget`)))