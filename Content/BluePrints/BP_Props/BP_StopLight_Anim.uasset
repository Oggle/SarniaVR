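; BP_StopLight_Anim is an animated stop light prop that cycles through three bulbs, showing one at a time.
; The construction script gathers the three light components into an array and stores the count.
; From BeginPlay, a self-repeating delay loop shows the current bulb, hides the others, then advances and wraps the index at a fixed interval.
; Unconnected construction-script nodes for setting bulb colours through Custom Primitive Data never run.
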(event `self.ReceiveBeginPlay`
  ;[0.247 0.1257 1] Setup Bulb Sequence
  (for _index (range (`self.totalBulbs`)) :!label _label
    (if (== (`self.atSignTxt`) _index)
      (bind _output (`|GetArrayItem` (`self.myLightBulbs`) _index))
      (`SceneComponent.SetVisibility` _output true true)
      (else
        (`SceneComponent.SetVisibility` _output false true))))
  ;[0.904 0.2572 1] Increment At Content
  (bind _output_get (set `self.atSignTxt` (+ (`self.atSignTxt`) 1)))
  ;[0.1093 0.8399 1] Reset Seq Content if no more content
  (if (>= _output_get (`KismetArrayLibrary.Array_Length` (`self.myLightBulbs`)))
    (set `self.atSignTxt` 0))
  (`KismetSystemLibrary.RetriggerableDelay` 12.0)
  (goto _label))

(fn `UserConstructionScript`
  (`KismetArrayLibrary.Array_Clear` (`self.myLightBulbs`))
  (`KismetArrayLibrary.Array_Add` (`self.myLightBulbs`) (`self.light_1`))
  (`KismetArrayLibrary.Array_Add` (`self.myLightBulbs`) (`self.light_2`))
  (`KismetArrayLibrary.Array_Add` (`self.myLightBulbs`) (`self.light_3`))
  (set `self.totalBulbs` (`KismetArrayLibrary.Array_Length` (`self.myLightBulbs`))))