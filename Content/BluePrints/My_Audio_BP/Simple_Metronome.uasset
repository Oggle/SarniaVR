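; Metronome actor that uses a Quartz clock to play one of two sample tracks in musical time and show the beat.
; StartQuartz creates the clock from tempo and time-signature settings, queues quantized playback and resumes the clock once queued.
; Subscribed beat events blink the mesh material, update the beat text and trigger the last overlapped BP_SVR_Sample_Pad_V2.
; Overlap-driven buttons alternate tracks or stop playback, with optional auto-start on BeginPlay.
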(event `self.ReceiveBeginPlay`
  (if (`self.startNow`)
    (`self.StartQuartz`)
    (else
      (`AudioComponent.Stop` (`self.TrackA`))
      (`AudioComponent.Stop` (`self.TrackB`)))))

(event `playNewTrack`
  ;[1 0 0.02017 1 14] Play My Single Audio Sample in a Quantized Environment
  (`AudioComponent.PlayQuantized` (`self.NextTrackAC`) (`self.musicClockRef`) (make `QuartzQuantizationBoundary` "SixteenthNote" 1.0 "TransportRelative") (`|CreateDelegate` :!event `queStatus`) 0.0 0.0 (`self.soundVolume`) "Linear" :!label _label)
  ;[1 0 0.6873] Subscribe to the Beat and call the blink me event
  (`QuartzClockHandle.SubscribeToQuantizationEvent` (`self.musicClockRef`) (`self.subscribeToBeat`) (`|CreateDelegate` :!event `blinkMe`)))

(event `StartQuartz`
  ;[1 0 0.2228] Custom Event bindable
  ;[0.03203 0.02007 0.1562 1 14] Tutorial 2 Quart Based with musical timing
  ;;[1 0.06871 0.9013] Quartz initialize and settings
  (bind _returnvalue (`QuartzSubsystem.CreateNewClock` (subsystem `QuartzSubsystem`) (`self.bpmClockName`) (make `QuartzClockSettings` (make `QuartzTimeSignature` (`self.QTBeat`) (`self.QTBeatType`))) true true))
  (bind _output_get (set `self.musicClockRef` _returnvalue))
  ;;[1 0.1706 0.52] Set beats per minute and insert sound
  (`QuartzClockHandle.SetBeatsPerMinute` :`self` _output_get :`BeatsPerMinute` (`self.beatsPerMin`))
  (goto _label))

(event `blinkMe`
  (params (ClockName :type Name) (QuantizationType :type "EQuartzCommandQuantization Enum" :default "Bar") (NumBars :type Integer) (Beat :type Integer) (BeatFraction :type "Float (double-precision)"))
  ;[1 0 0.1024] Show the click on the beat you subscribed too.
  (`PrimitiveComponent.SetMaterial` (`self.staticShowMesh`) (`self.onMatIndex`) (`self.onMaterial`))
  (`TextRenderComponent.K2_SetText` (`self.watchBeat`) (`KismetTextLibrary.Conv_IntToText` Beat))
  (`KismetSystemLibrary.Delay` (`self.blinkDelay`))
  (`PrimitiveComponent.SetMaterial` (`self.staticShowMesh`) (`self.onMatIndex`) (`self.offMaterial`))
  (if (`self.onPad`)
    (bind _asbp_svr_sample_pad_v2 (cast `/Game/BluePrints/My_Audio_BP/DrumPad/BP_SVR_Sample_Pad_V2` (`self.overlapActor`)))
    (`/Game/BluePrints/My_Audio_BP/DrumPad/BP_SVR_Sample_Pad_V2.playMetronome` _asbp_svr_sample_pad_v2)))

(event `queStatus`
  (params (EventType :type "EQuartzCommandDelegateSubType Enum" :default "CommandOnFailedToQueue") (Name :type Name))
  ;[0.03203 0.02007 0.1562 1 14] Tutorial 2 Quart Based with musical timing
  ;;[0.4098 0.5521 0.0123] Que Status Deligate supporting quartz events
  (switch `EQuartzCommandDelegateSubType` EventType
    (:`CommandOnQueued`
      (`QuartzClockHandle.ResumeClock` (`self.musicClockRef`)))))

(event `self.staticShowMesh.OnComponentBeginOverlap`
  (params (OverlappedComponent :type "PrimitiveComponent Object Reference") (OtherActor :type "Actor Object Reference") (OtherComp :type "PrimitiveComponent Object Reference") (OtherBodyIndex :type Integer) (bFromSweep :type Boolean) (SweepResult :type "HitResult Structure (by ref)"))
  ;[0 0.4747 1] Button Functions
  ;;[1 0.6106 0] Overlap with our Root Mesh
  ;;;[1 0.1692 0.586] Checking for a Sample Pad
  (if (== (`GameplayStatics.GetObjectClass` OtherActor) "/Game/BluePrints/My_Audio_BP/DrumPad/BP_SVR_Sample_Pad_V2.BP_SVR_Sample_Pad_V2_C")
    ;;;[1 0 0.3853] Make sure its not our exisiting pad
    (set `self.overlapActor` OtherActor)
    (if (!= (`self.overlapActor`) (`self.oldOverlap`))
      ;;;;[0.2754 1 0 1 12] Replace pad reference and toggle onPad Boolean
      (set `self.oldOverlap` (`self.overlapActor`))
      (set `self.onPad` true))))

(event `self.nextButton.OnComponentBeginOverlap`
  (params (OverlappedComponent :type "PrimitiveComponent Object Reference") (OtherActor :type "Actor Object Reference") (OtherComp :type "PrimitiveComponent Object Reference") (OtherBodyIndex :type Integer) (bFromSweep :type Boolean) (SweepResult :type "HitResult Structure (by ref)"))
  ;[0 0.4747 1] Button Functions
  ;;[0.4377 1 0.1352] Next Track Button
)

(event `self.nextButton.OnComponentEndOverlap`
  (params (OverlappedComponent :type "PrimitiveComponent Object Reference") (OtherActor :type "Actor Object Reference") (OtherComp :type "PrimitiveComponent Object Reference") (OtherBodyIndex :type Integer))
  ;[0 0.4747 1] Button Functions
  ;;[0.4377 1 0.1352] Next Track Button
  (if (`self.toggleTrack`)
    (set `self.NextTrackAC` (`self.TrackA`))
    (set `self.toggleTrack` false)
    (else
      (set `self.NextTrackAC` (`self.TrackB`))
      (set `self.toggleTrack` true)))
  (`self.StartQuartz`)
  (set `self.togglePlay` true)
  (`KismetSystemLibrary.PrintString` "NextTrack"))

(event `self.stopButton.OnComponentBeginOverlap`
  (params (OverlappedComponent :type "PrimitiveComponent Object Reference") (OtherActor :type "Actor Object Reference") (OtherComp :type "PrimitiveComponent Object Reference") (OtherBodyIndex :type Integer) (bFromSweep :type Boolean) (SweepResult :type "HitResult Structure (by ref)"))
  ;[0 0.4747 1] Button Functions
  ;;[1 0.04934 0.00954] Stop Button
)

(event `self.stopButton.OnComponentEndOverlap`
  (params (OverlappedComponent :type "PrimitiveComponent Object Reference") (OtherActor :type "Actor Object Reference") (OtherComp :type "PrimitiveComponent Object Reference") (OtherBodyIndex :type Integer))
  ;[0 0.4747 1] Button Functions
  ;;[1 0.04934 0.00954] Stop Button
  (`AudioComponent.Stop` (`self.NextTrackAC`))
  (`AudioComponent.Stop` (`self.TrackA`))
  (`AudioComponent.Stop` (`self.TrackB`))
  (set `self.togglePlay` false)
  (`KismetSystemLibrary.PrintString` "StopTrack"))

(fn `UserConstructionScript`
  (locals (meshShowOldMaterials :type "Array of MaterialInterface Object Reference"))
  (bind _trackb (`self.TrackB`))
  (bind _watchbeat (`self.watchBeat`))
  ;[0 0.01735 0.2604] Fill Track A and B Components with Samples
  (`AudioComponent.SetSound` (`self.TrackA`) (`self.trackA_Sample`))
  (`AudioComponent.SetSound` _trackb (`self.trackB_Sample`))
  (set `self.NextTrackAC` _trackb)
  ;[0.2011 0.7042 1] Material and Text Default sizes and materials
  (set `local.meshShowOldMaterials` (`MeshComponent.GetMaterials` (`self.staticShowMesh`)))
  (`PrimitiveComponent.SetMaterial` (`self.staticShowMesh`) (`self.onMatIndex`) (`self.offMaterial`))
  (`TextRenderComponent.SetWorldSize` _watchbeat (`self.labelSize`))
  (`TextRenderComponent.SetTextRenderColor` _watchbeat (`self.labelColour`)))