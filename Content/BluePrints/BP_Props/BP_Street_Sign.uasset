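; BP_Street_Sign is a street sign prop that shows a choice of sign shapes.
; The Construction Script gathers five shape components (triangle, round rectangle, small square, hexagon, large rectangle) into MySignShapes.
; It then loops over the SignShape boolean array and shows or hides the component at each matching index.
; The Event Graph holds only unused default events, so nothing in it runs during play.
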(fn `UserConstructionScript`
  (locals (mySignShapes :type "Array of StaticMeshComponent Object Reference"))
  (bind _mysignshapes (`local.mySignShapes`))
  (`KismetArrayLibrary.Array_Add` _mysignshapes (`self.SS_Triangle`))
  (`KismetArrayLibrary.Array_Add` _mysignshapes (`self.SS_Round_Rec`))
  (`KismetArrayLibrary.Array_Add` _mysignshapes (`self.SS_Smal_Square`))
  (`KismetArrayLibrary.Array_Add` _mysignshapes (`self.SS_Hexagon`))
  (`KismetArrayLibrary.Array_Add` _mysignshapes (`self.SS_Large_Rec`))
  (for (_array_element _array_index) (`self.signShape`)
    (if _array_element
      (bind _output (`|GetArrayItem` (`local.mySignShapes`) _array_index))
      (`SceneComponent.SetVisibility` _output true false)
      (else
        (`SceneComponent.SetVisibility` _output false false)))))