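; Quiz core actor that presents a question and its answer options in the world on BeginPlay, if enabled.
; It renders the question as a text component on itself and spawns one answer target per array entry in front of the player, turned to face them.
; A StaggerZ flag picks the layout: answers stepped along world X and Z, or spread along world Y at a base height offset.
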(event `self.ReceiveBeginPlay`
  (bind _returnvalue (`GameplayStatics.GetPlayerPawn` 0))
  (bind _qtextrendercomponent (`self.qTextRenderComponent`))
  (bind _myquestionindex (`self.myQuestionIndex`))
  (bind _returnvalue_2 (* (`self.myQuestionIndex`) (`self.answerDistanceMin`)))
  (bind _rotation (.rotation (`self.playerTransform`)))
  ;[0.3115 1 0.06522] Begin the question sequence?
  (if (`self.beginQuestions`)
    (`|ExecutionSequence`
      (:`then_0`
        ;[0.5224 1 0.1643] Find Our Location
        (set `self.myLocation` (`self.K2_GetActorLocation`))
        ;[0.4422 0.1643 1] Store Player Transform
        (set `self.playerTransform` (`self.GetTransform` _returnvalue))
        (set `self.playerBoxExtent` (`.BoxExtent` (`self.GetActorBounds` _returnvalue false false))))
      (:`then_1`
        ;[0 1 0.9058] Add the Question Text
        (bind _returnvalue_3 (`AddComponent|NODE_AddTextRenderComponent-0` :`RelativeTransform` (`KismetMathLibrary.MakeTransform` (0.0 0.0 0.0) (struct :`Yaw` 180.0))))
        (set `self.qTextRenderComponent` _returnvalue_3)
        (`TextRenderComponent.K2_SetText` _qtextrendercomponent (`KismetTextLibrary.Conv_StringToText` (`self.Question`)))
        (`TextRenderComponent.SetWorldSize` _qtextrendercomponent (`self.questionDisplaySize`)))
      (:`then_2`
        ;[0.1107 0.9203 1] Loop Through the answers
        (for _index (range (`self.answerNumTotal`))
          (set `self.myQuestionIndex` _index)
          (bind _output_get (set `self.startShowQVector` (+ (.location (`self.playerTransform`)) (* (`KismetMathLibrary.GetForwardVector` _rotation) 500.0))))
          (bind _returnvalue_4 (`|SpawnActorFromClass` "/Game/BluePrints/BP_QuizCore/BP_target_Answer_Typ-01.BP_target_Answer_Typ-01_C" (`KismetMathLibrary.MakeTransform` _output_get (`KismetMathLibrary.MakeRotator` (.roll _rotation) (.pitch _rotation) (- (.yaw _rotation) 180.0)) (.scale (`self.playerTransform`))) "Undefined" "OverrideRootScale" null (`KismetStringLibrary.Concat_StrStr` "Option " (`KismetStringLibrary.Conv_IntToString` _myquestionindex)) (`|GetArrayItem` (`self.answerArray`) _myquestionindex) false null))
          ;[1 0 0.08657] Advance the answers in the air away from the player
          (bind _output_get_2 (set `self.myShootTarget` _returnvalue_4))
          ;;[0.173 0 1] Styles of display
          (if (`self.staggerZ`)
            (`self.K2_AddActorWorldOffset` _output_get_2 (`KismetMathLibrary.MakeVector` _returnvalue_2 0.0 (+ (`self.showAnswerBaseHeight`) _returnvalue_2)) false false)
            (else
              (`self.K2_AddActorWorldOffset` (`self.myShootTarget`) (`KismetMathLibrary.MakeVector` 0.0 (* (`self.myQuestionIndex`) (`self.answerDistanceMin`)) (`self.showAnswerBaseHeight`)) false false))))))))

(fn `UserConstructionScript`
  (locals (local_myQuestionTxt :type String) (local_myQuestionTitle :type String))
  (set `local.local_myQuestionTxt` (`self.Question`))
  (set `local.local_myQuestionTitle` (`self.Title`))
  (set `self.answerNumTotal` (`KismetArrayLibrary.Array_Length` (`self.answerArray`))))