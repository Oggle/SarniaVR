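; Bus vehicle prototype that builds a route from the BP_BusStop actors in the level and picks destinations along it.
; BeginPlay gathers stop locations; overlapping any actor not yet in the route history records it and advances the destination index, wrapping at the end.
; Tick computes a steering difference but applies only zero torque to one tire.
; Movement, turning, ground-snap and wheel-spin logic is disconnected, and debug prints run throughout.
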(event `self.ReceiveActorBeginOverlap`
  (params (OtherActor :type "Actor Object Reference"))
  (`KismetSystemLibrary.PrintString` "Hit Something")
  (if (not (`self.routeHistoryBeen` OtherActor))
    (`self.nextStop` OtherActor)))

(event `self.ReceiveBeginPlay`
  (`self.getStops`)
  (`self.nextStop` null)
  (set `self.canDrive` true))

(event `self.ReceiveTick`
  (params (DeltaSeconds :type "Float (single-precision)"))
  ;[1 1 1] Current Location
  (set `self.atLocation` (`self.K2_GetActorLocation`))
  (set `self.myDeltaSeconds` DeltaSeconds)
  (set `self.turnZ` (- (`SceneComponent.GetForwardVector` (`self.Bus`)) (`KismetMathLibrary.GetForwardVector` (`KismetMathLibrary.FindLookAtRotation` (`self.atLocation`) (`self.destLocation`)))))
  (if (`self.canDrive`)
    (`PrimitiveComponent.AddTorqueInDegrees` (`self.fl_tire`) (0.0 0.0 0.0) "None" false)))

(fn `getStops`
  (bind _returnvalue (`KismetArrayLibrary.Array_Length` (`self.allBusStops`)))
  (bind _outactors (`GameplayStatics.GetAllActorsOfClass` "/Game/GameReady/BP_BusStop.BP_BusStop_C"))
  (bind _output_get (set `self.allBusStops` _outactors))
  (if (> _returnvalue 0)
    (bind _output_get_2 (set `self.outDiagString` (`KismetStringLibrary.Concat_StrStr` (`KismetStringLibrary.Conv_IntToString` _returnvalue) " Stops Found")))
    (`KismetSystemLibrary.PrintString` _output_get_2)
    (for (_array_element _array_index) _output_get
      (`KismetArrayLibrary.Array_Insert` (`self.destArrays`) (`self.K2_GetActorLocation` _array_element) _array_index))
    (`KismetSystemLibrary.PrintString` "Bus Got Routes")
    (else
      (`KismetSystemLibrary.PrintString` "No Stops"))))

(fn `nextStop`
  (params (newStopActor :type "Actor Object Reference"))
  (bind _returnvalue (`KismetMathLibrary.Dot_VectorVector` (`KismetMathLibrary.GetForwardVector` (`KismetMathLibrary.MakeRotator` (.x (`self.atLocation`)) (.y (`self.atLocation`)))) (`KismetMathLibrary.GetForwardVector` (`KismetMathLibrary.MakeRotator` (.x (`self.destLocation`)) (.y (`self.destLocation`))))))
  (`self.routeHistoryAdd` newStopActor)
  (bind _result (`/Engine/EditorBlueprintResources/StandardMacros.IncrementInt` (`self.atLocArray`))
    (:`  `
      (set `self.atLocation` (`self.K2_GetActorLocation`))
      (if (>= _result (`KismetArrayLibrary.Array_Length` (`self.destArrays`)))
        (set `self.atLocArray` 0))
      (set `self.destLocation` (`|GetArrayItem` (`self.destArrays`) (`self.atLocArray`)))
      (`KismetSystemLibrary.PrintString` (`KismetStringLibrary.Concat_StrStr` "Goingt To Stop " (`KismetStringLibrary.Conv_IntToString` (`self.atLocArray`))) true true (struct :`G` 0.66 :`B` 1.0 :`A` 1.0) 5.0)
      (`KismetSystemLibrary.PrintString` (`KismetStringLibrary.Concat_StrStr` (`KismetStringLibrary.Conv_DoubleToString` _returnvalue) "Dot") true true (struct :`R` 1.0 :`G` 0.109751 :`B` 0.050025 :`A` 1.0) 15.0)
      (if (> _returnvalue 0.0)
        (`KismetSystemLibrary.PrintString` "Stop To Our Right")
        (else
          (`KismetSystemLibrary.PrintString` "Stop To Our Left")))
      (`KismetSystemLibrary.PrintString` (`KismetStringLibrary.Conv_DoubleToString` (`KismetMathLibrary.RadiansToDegrees` _returnvalue)) true true (struct :`R` 0.614583 :`B` 0.565375 :`A` 1.0) 15.0))))

(fn `routeHistoryAdd`
  (params (stopActor :type "Actor Object Reference"))
  (bind _returnvalue (`KismetArrayLibrary.Array_Add` (`self.stopAtors`) stopActor))
  (`KismetSystemLibrary.PrintString` (`KismetStringLibrary.Concat_StrStr` (`KismetStringLibrary.Concat_StrStr` "Added Stop" (`KismetStringLibrary.Conv_IntToString` _returnvalue)) (`KismetStringLibrary.Concat_StrStr` "History Length" (`KismetStringLibrary.Conv_IntToString` (`KismetArrayLibrary.Array_Length` (`self.stopAtors`)))))))

(fn `routeHistoryBeen`
  (params (thisStop :type "Actor Object Reference"))
  (returns (haveBeen :type Boolean))
  (return (`KismetArrayLibrary.Array_Contains` (`self.stopAtors`) thisStop)))

(fn `UserConstructionScript`)