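; Test Blueprint for a timer-driven gate that prints whether it was open or closed on each Tick.
; BeginPlay stores the world delta seconds in LastGateDelta; an open gate closes on the next Tick.
; A closed gate compares LastGateDelta plus GateMin against LastGateDelta itself, so no elapsed time is measured and any clearly positive GateMin reopens it immediately, alternating every frame.
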(event `self.ReceiveBeginPlay`
  (set `self.lastGateDelta` (`GameplayStatics.GetWorldDeltaSeconds`)))

(event `self.ReceiveActorBeginOverlap`
  (params (OtherActor :type "Actor Object Reference")))

(event `self.ReceiveTick`
  (params (DeltaSeconds :type "Float (single-precision)"))
  (set `self.Delta Seconds` DeltaSeconds)
  (if (`self.gateOpen`)
    (set `self.lastGateDelta` (`self.lastGateDelta`))
    (set `self.gateOpen` false)
    (`KismetSystemLibrary.PrintString` "Gate Was Open")
    (else
      (set `self.gateOpen` (> (+ (`self.lastGateDelta`) (`self.gateMin`)) (`self.lastGateDelta`)))
      (`KismetSystemLibrary.PrintString` "Gate Was Closed"))))

(fn `UserConstructionScript`)