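; Prototype self-driving car pawn that follows "rs_12" road splines using cheated movement rather than wheel physics.
; Each tick a downward trace finds the road actor, samples its spline two input keys ahead and passes that to DriveVehicle.
; DriveVehicle rotates tires and body and feeds FloatingPawnMovement, printing debug values.
; The construction script lays out tires, axes and suspension from chassis size; random auto-drive, gravity, suspension and spline-based steering logic are unconnected.
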(event `self.ReceiveBeginPlay`
  (`KismetSystemLibrary.PrintString` (`KismetStringLibrary.Conv_RotatorToString` (`SceneComponent.K2_GetComponentRotation` (`self.tire_fl`))) true true (struct :`G` 0.66 :`B` 1.0 :`A` 1.0) 30.0)
  (`KismetSystemLibrary.PrintString` (`KismetStringLibrary.Conv_RotatorToString` (`SceneComponent.K2_GetComponentRotation` (`self.tire_fr`))) true true (struct :`G` 0.66 :`B` 1.0 :`A` 1.0) 30.0))

(event `self.ReceiveTick`
  (params (DeltaSeconds :type "Float (single-precision)"))
  (bind _returnvalue (`SceneComponent.K2_GetComponentLocation` (`self.body`)))
  ;[1 0 0] EVENT TICK
  (set `self.myDeltaSeconds` DeltaSeconds)
  ;[1 0.9434 0] Get Bus Location Trace Down
  (bind (_outhit _returnvalue_2) (`KismetSystemLibrary.LineTraceSingle` :`Start` _returnvalue :`End` (`KismetMathLibrary.MakeVector` (.x _returnvalue) (.y _returnvalue) (- (.z _returnvalue) (`self.lineTraceZDepth`))) :`TraceChannel` "TraceTypeQuery1" :`bTraceComplex` true :`DrawDebugType` "ForDuration" :`DrawTime` 1.0))
  (if _returnvalue_2
    (bind (_bblockinghit _binitialoverlap _time _distance _location _impactpoint _normal _impactnormal _physmat _hitactor) (`GameplayStatics.BreakHitResult` _outhit))
    (if _bblockinghit
      (bind _returnvalue_3 (`KismetSystemLibrary.GetObjectName` _hitactor))
      (if (`KismetStringLibrary.Contains` _returnvalue_3 "rs_12" true)
        (bind (_nextsplinevector _nextsplinedirvector _splinerotator) (`self.getNextSplineLocation` (`KismetStringLibrary.GetSubstring` _returnvalue_3 0 5) _hitactor))
        (`self.driveVehicle` _nextsplinevector _nextsplinedirvector _splinerotator)))))

(fn `driveVehicle`
  (params (toHere :type "Vector Structure") (nextSplineDirection :type "Vector Structure") (nextSplineRotator :type "Rotator Structure"))
  (locals (finalVector :type "Vector Structure"))
  (bind (_tiresizevector_x _tiresizevector_y _tiresizevector_z) (`KismetMathLibrary.BreakVector` (`self.tireSizeVector`)))
  (bind _returnvalue (`SceneComponent.GetForwardVector` (`self.body`)))
  (bind _returnvalue_2 (`SceneComponent.GetForwardVector` (`self.body`)))
  (bind (_x _y) (`KismetMathLibrary.BreakRotIntoAxes` (`SceneComponent.K2_GetComponentRotation` (`self.tire_fr`))))
  (bind (_x_2 _y_2) (`KismetMathLibrary.BreakRotIntoAxes` (`SceneComponent.K2_GetComponentRotation` (`self.tire_fl`))))
  (bind _returnvalue_3 (`KismetMathLibrary.GetForwardVector` (`KismetMathLibrary.MakeRotFromXY` (- _x_2 _x) (- _y_2 _y))))
  (bind _returnvalue_x (`KismetMathLibrary.BreakVector` (+ _returnvalue (* (* (- _returnvalue (`local.finalVector`)) (`self.engineCurrentPower`)) (`GameplayStatics.GetWorldDeltaSeconds`)))))
  ;[0.8879 0.288 1 1 14] Use input vector or bus forward
  (set `local.finalVector` (`KismetMathLibrary.GetForwardVector` (`KismetMathLibrary.FindLookAtRotation` (`SceneComponent.K2_GetComponentLocation` (`self.body`)) toHere)))
  ;[0.1308 0.3481 1] Set Tire Spin Z
  (set `self.newTireRot` (/ 2.0 _tiresizevector_z))
  ;[1 0.3506 0] Drive Tires
  (`KismetSystemLibrary.PrintString` (`KismetStringLibrary.Conv_DoubleToString` _returnvalue_x))
  (`SceneComponent.K2_AddLocalRotation` (`self.tire_fr`) (`KismetMathLibrary.MakeRotator` _returnvalue_x) false false)
  (`SceneComponent.K2_AddLocalRotation` (`self.tire_fl`) (`KismetMathLibrary.MakeRotator` _returnvalue_x) false false)
  (`SceneComponent.K2_AddLocalRotation` (`self.tire_bl`) (struct :`Roll` 2.0) false false)
  (`SceneComponent.K2_AddLocalRotation` (`self.tire_br`) (struct :`Roll` -2.0) false false)
  ;[1 0.04918 0] Cheat a forward velocity delta
  ;;[0.2397 1 0 1 14] Calc Engine Power Add to final look at vector
  (bind _newenginepower (`self.getEnginePower`))
  (set `self.engineCurrentPower` _newenginepower)
  (`SceneComponent.K2_AddWorldRotation` (`self.body`) (`KismetMathLibrary.MakeRotator` 0.0 0.0 (.z (+ _returnvalue_3 (* (* _returnvalue_3 (`self.engineCurrentPower`)) (`GameplayStatics.GetWorldDeltaSeconds`))))) false false)
  (`PawnMovementComponent.AddInputVector` (`self.FloatingPawnMovement`) (- (- (`self.GetActorForwardVector`) (`SceneComponent.GetForwardVector` (`self.body`))) (`local.finalVector`)) false)
  (`KismetSystemLibrary.PrintString` (`KismetStringLibrary.Conv_DoubleToString` (* (.z (+ _returnvalue_2 (* (- _returnvalue_2 (`local.finalVector`)) (`self.engineCurrentPower`)))) (`self.turmRadiusScalar`))))
  (`KismetSystemLibrary.PrintString` (`KismetStringLibrary.Conv_VectorToString` (`local.toHere`)))
  (`KismetSystemLibrary.PrintString` (`KismetStringLibrary.Conv_VectorToString` (`local.nextSplineDirection`)) true true (struct :`R` 1.0 :`B` 0.227856 :`A` 1.0))
  (`KismetSystemLibrary.PrintString` (`KismetStringLibrary.Conv_RotatorToString` (`SceneComponent.K2_GetComponentRotation` (`self.body`))) true true (struct :`R` 0.988786 :`G` 1.0 :`A` 1.0)))

(fn `getEnginePower`
  (returns (newEnginePower :type "Float (double-precision)"))
  (bind _enginecurrentgear (`self.engineCurrentGear`))
  (return (+ (/ (`self.engineHP`) _enginecurrentgear) (* _enginecurrentgear 2.0))))

(fn `getNextSplineLocation`
  (params (thisSplineName :type String) (thisSplineActor :type "Actor Object Reference"))
  (returns (nextSplineVector :type "Vector Structure") (nextSplineDirVector :type "Vector Structure") (splineRotator :type "Rotator Structure"))
  (bind _rs_object (`self.RS_Object`))
  ;[0.02107 0.1667 0.1467 1 14] Substring Switch Cast to RS Spline and Get Road
  (`KismetSystemLibrary.PrintString` "Is Road SPline" false)
  (switch `string` thisSplineName
    (:`rs_12`
      (bind _asrs_actor_12p_1front_wide (cast `/Game/BluePrints/RoadSplines/RS_Actor_12p1FrontWide` thisSplineActor))
      (bind _output_get (set `self.RS_Object` (`/Game/BluePrints/RoadSplines/RS_Actor_12p1FrontWide.Road` _asrs_actor_12p_1front_wide)))
      (bind _returnvalue (+ (`SplineComponent.FindInputKeyClosestToWorldLocation` _output_get (`SceneComponent.K2_GetComponentLocation` (`self.body`))) 2.0))
      (bind _returnvalue_2 (`SplineComponent.GetLocationAtSplineInputKey` _rs_object _returnvalue "World"))
      ;[0.09582 0.07643 0.3594] Find spline points closest to bus
      (`KismetSystemLibrary.PrintString` (`KismetStringLibrary.Concat_StrStr` "Next Point At" (`KismetStringLibrary.Conv_VectorToString` _returnvalue_2)) false)
      (return _returnvalue_2 (`SplineComponent.GetDirectionAtSplineInputKey` _rs_object _returnvalue "World") (`SplineComponent.GetRotationAtSplineInputKey` _rs_object _returnvalue "World")))))

(fn `UserConstructionScript`
  (bind (_chassisusersize_location _chassisusersize_rotation _chassisusersize_scale) (`KismetMathLibrary.BreakTransform` (`self.chassisUserSize`)))
  (bind _body (`self.body`))
  (bind _tire_fr (`self.tire_fr`))
  (bind _tires_array (`self.tires_array`))
  (bind (_min _max) (`StaticMeshComponent.GetLocalBounds` _tire_fr))
  (bind (_returnvalue_x _returnvalue_y) (`KismetMathLibrary.BreakVector` (/ (`self.chassis_size`) 2)))
  (bind _returnvalue_location (`KismetMathLibrary.BreakTransform` (`SceneComponent.GetRelativeTransform` (`self.tire_br`))))
  (bind (_returnvalue_x_2 _returnvalue_y_2) (`KismetMathLibrary.BreakVector` (/ (`self.chassis_size`) 2)))
  (bind _returnvalue_location_2 (`KismetMathLibrary.BreakTransform` (`SceneComponent.GetRelativeTransform` (`self.tire_fr`))))
  (bind _returnvalue (`SceneComponent.GetRelativeTransform` _body))
  (bind _returnvalue_location_3 (`KismetMathLibrary.BreakTransform` (`SceneComponent.GetRelativeTransform` (`self.tire_fl`))))
  (bind _returnvalue_location_4 (`KismetMathLibrary.BreakTransform` (`SceneComponent.GetRelativeTransform` (`self.tire_bl`))))
  (bind (_returnvalue_x_3 _returnvalue_y_3 _returnvalue_z) (`KismetMathLibrary.BreakVector` (/ (`self.tireSizeVector`) 2)))
  (bind (_returnvalue_x_4 _returnvalue_y_4 _returnvalue_z_2) (`KismetMathLibrary.BreakVector` (/ (`self.tireSizeVector`) 2)))
  (bind _returnvalue_2 (`SceneComponent.GetRelativeTransform` _body))
  (bind _returnvalue_3 (- (.x (.location _returnvalue_2)) _returnvalue_x_2))
  ;[1 0.09154 0] Clear Construction Arrays
  (`KismetArrayLibrary.Array_Clear` (`self.lineTraceTargetEnds`))
  (`KismetArrayLibrary.Array_Clear` (`self.lineTraceTargetStarts`))
  (`KismetArrayLibrary.Array_Clear` (`self.tireStartTransforms`))
  (`KismetArrayLibrary.Array_Clear` (`self.tires_array`))
  (set `self.chassis_size` _chassisusersize_scale)
  (set `self.tireSizeVector` (* (- _max _min) (`SceneComponent.K2_GetComponentScale` _tire_fr)))
  ;[0.1335 0.6074 1] Add tires to Array
  (`KismetArrayLibrary.Array_Add` _tires_array (`self.tire_fl`))
  (`KismetArrayLibrary.Array_Add` _tires_array (`self.tire_fr`))
  (`KismetArrayLibrary.Array_Add` _tires_array (`self.tire_bl`))
  (`KismetArrayLibrary.Array_Add` _tires_array (`self.tire_br`))
  ;[1 0.3091 0.09807] Tire Base Z Rotation
  (if (`self.tire_y_forward`)
    ;[1 0.6684 0.269] If X not Forward
    (bind _output_get (set `self.tire_rot_z` 90.0))
    (`/Engine/EditorBlueprintResources/StandardMacros.NegateFloat` _output_get
      (:`  `
        (`SceneComponent.K2_SetWorldTransform` (`self.tire_fl`) (`KismetMathLibrary.MakeTransform` (`KismetMathLibrary.MakeVector` (+ (.x (.location _returnvalue_2)) _returnvalue_x_2) (- (.y (.location _returnvalue_2)) _returnvalue_y_2) (- (.z (.location _returnvalue_2)) (+ _returnvalue_z (`self.wheel_z_offset`)))) (`KismetMathLibrary.MakeRotator` 0.0 0.0 (`self.tire_rot_z`))) false false) ; Setting World Position
        (`SceneComponent.K2_SetWorldTransform` (`self.tire_bl`) (`KismetMathLibrary.MakeTransform` (`KismetMathLibrary.MakeVector` _returnvalue_3 (- (.y (.location _returnvalue_2)) _returnvalue_y_2) (- (.z (.location _returnvalue_2)) (+ _returnvalue_z (`self.wheel_z_offset`)))) (`KismetMathLibrary.MakeRotator` _returnvalue_3 0.0 (`self.tire_rot_z`))) false false) ; Setting World Position
        (`SceneComponent.K2_SetWorldTransform` (`self.tire_fr`) (`KismetMathLibrary.MakeTransform` (`KismetMathLibrary.MakeVector` (+ (.x (.location _returnvalue_2)) _returnvalue_x_2) (+ (.y (.location _returnvalue_2)) _returnvalue_y_2) (- (.z (.location _returnvalue_2)) (+ (`self.wheel_z_offset`) _returnvalue_z))) (`KismetMathLibrary.MakeRotator` 0.0 0.0 (* (`self.tire_rot_z`) -1.0))) false false) ; Setting World Position
        (`SceneComponent.K2_SetWorldTransform` (`self.tire_br`) (`KismetMathLibrary.MakeTransform` (`KismetMathLibrary.MakeVector` (- (.x (.location _returnvalue)) _returnvalue_x) (+ (.y (.location _returnvalue)) _returnvalue_y) (- (.z (.location _returnvalue)) (+ (`self.wheel_z_offset`) _returnvalue_z_2))) (`KismetMathLibrary.MakeRotator` 0.0 0.0 (* (`self.tire_rot_z`) -1.0))) false false) ; Setting World Position
        ;[0.9062 0.1827 0] Set Tire Start Positions
        (for _array_element (`self.tires_array`)
          (`KismetArrayLibrary.Array_Add` (`self.tireStartTransforms`) (`SceneComponent.GetRelativeTransform` _array_element)))
        ;[0.9067 1 0] Prepare line trace cycle variables
        (for _array_element_2 (`self.tireStartTransforms`)
          (bind _location (.location _array_element_2))
          (`KismetArrayLibrary.Array_Add` (`self.lineTraceTargetStarts`) _location)
          (`KismetArrayLibrary.Array_Add` (`self.lineTraceTargetEnds`) (`KismetMathLibrary.MakeVector` (.x _location) (.y _location) (- (.z _location) (`self.lineTraceZDepth`))))
          ;[1 0.008451 0] Set Axis and suspecsion to wheel positions
          (`SceneComponent.K2_SetRelativeLocation` (`self.fr_axis`) _returnvalue_location_2 false false)
          (`SceneComponent.K2_SetRelativeLocation` (`self.fr_sus`) _returnvalue_location_2 false false)
          (`SceneComponent.K2_SetRelativeLocation` (`self.fl_axis`) _returnvalue_location_3 false false)
          (`SceneComponent.K2_SetRelativeLocation` (`self.fl_sus`) _returnvalue_location_3 false false)
          (`SceneComponent.K2_SetRelativeLocation` (`self.bl_axis`) _returnvalue_location_4 false false)
          (`SceneComponent.K2_SetRelativeLocation` (`self.bl_sus`) _returnvalue_location_4 false false)
          (`SceneComponent.K2_SetRelativeLocation` (`self.br_axis`) _returnvalue_location false false)
          (`SceneComponent.K2_SetRelativeLocation` (`self.br_sus`) _returnvalue_location false false))))))